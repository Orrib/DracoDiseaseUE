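; BP_BlessedAltar_Cursed is a cursed altar variant that adds two eye-fire effects to the behavior inherited from its parent altar Blueprint.
; Both fires start off at BeginPlay and follow the show/hide state of the widget UI while the altar is inactive.
; Activating the altar switches the fires off, with each override calling the parent implementation first.
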(event EventBeginPlay
  (|CallParentFunction)
  (Components|Activation|SetActive (Variables|Default|GetEye%20Fire) false false))

(event Collision|EventActorBeginOverlap
  (params (OtherActor :type Actor%20Object%20Reference))
  (|CallParentFunction OtherActor) ; This node is disabled and will not be called.\nDrag off pins to build functionality.
)

(event EventTick
  (params (DeltaSeconds :type Float%20%28single-precision%29))
  (|CallParentFunction DeltaSeconds) ; This node is disabled and will not be called.\nDrag off pins to build functionality.
)

(event EventShow/HideWidgetUI
  (params (Show? :type Boolean))
  (|CallParentFunction Show?)
  (if (not (Variables|Default|GetAltar%20Active))
    (Components|Activation|SetActive (Variables|Default|GetEye%20Fire) Show? false)))

(event EventSetAltarActive
  (params (Active? :type Boolean))
  (|CallParentFunction Active?)
  (if Active?
    (Components|Activation|SetActive (Variables|Default|GetEye%20Fire%202) false false)))

(fn ConstructionScript
  (|CallParentFunction))