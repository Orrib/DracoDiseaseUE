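; Dragon fire barrier that starts hidden and, once enabled, blocks the player with a wall of blue fire.
; The player's first trigger overlap turns on the invisible wall and fire volume, then a timeline sweeps a fire effect between two points, igniting four ground fires in sequence.
; Tick damages and launches players inside the fire away from an origin with distance-scaled knockback when grounded; overlapping bushes take fire damage.
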(event OnComponentBeginOverlap(Trigger)
  (params (OverlappedComponent :type Primitive%20Component%20Object%20Reference) (OtherActor :type Actor%20Object%20Reference) (OtherComp :type Primitive%20Component%20Object%20Reference) (OtherBodyIndex :type Integer) (bFromSweep :type Boolean) (SweepResult :type Hit%20Result%20Structure%20%28by%20ref%29))
  (bind _fire_blue (Variables|Default|GetFire_blue))
  (if (Actor|ActorHasTag OtherActor "player")
    (Utilities|FlowControl|DoOnce false
      (:Completed
        (Collision|SetCollisionEnabled (Variables|Default|GetInvisible%20Wall) "QueryAndPhysics")
        (Components|Timeline|SetPlayRate (Variables|Default|GetTimeline) (Math|Float|Power 1.3 -1.0))
        (Components|Activation|SetActive _fire_blue true false)
        (bind _move_dragon_fire (Timeline|Timeline PlayFromStart)
          (:Update
            (Transformation|SetWorldLocation _fire_blue (Math|Vector|Lerp(Vector) (Transformation|GetWorldLocation (Variables|Default|GetDragon%20Fire%20Start%20pos)) (Transformation|GetWorldLocation (Variables|Default|GetDragon%20Fire%20End%20pos)) _move_dragon_fire) false false))
          (:Finished
            (Components|Activation|SetActive _fire_blue false false))
          (:Trigger%20a%20ground%20fire
            (Utilities|FlowControl|MultiGate false false -1
              (:Out%200
                (Components|Activation|SetActive (Variables|Default|GetFire_blue_larger) true false))
              (:Out%201
                (Components|Activation|SetActive (Variables|Default|GetFire_blue_larger1) true false))
              (:Out%202
                (Components|Activation|SetActive (Variables|Default|GetFire_blue_larger2) true false))
              (:Out%203
                (Components|Activation|SetActive (Variables|Default|GetFire_blue_larger3) true false)))))))))

(event OnComponentBeginOverlap(FireTrigger)
  (params (OverlappedComponent :type Primitive%20Component%20Object%20Reference) (OtherActor :type Actor%20Object%20Reference) (OtherComp :type Primitive%20Component%20Object%20Reference) (OtherBodyIndex :type Integer) (bFromSweep :type Boolean) (SweepResult :type Hit%20Result%20Structure%20%28by%20ref%29))
  (if (Actor|ActorHasTag OtherActor "player")
    (Math|Integer|IncrementInt (Variables|Default|GetColliders%20that%20detect%20player))
    (elif (Actor|ActorHasTag OtherActor "bush")
      (Game|Damage|ApplyDamage OtherActor 1.0 0 0 "/Game/BP/DamageType_Fire_Primary_Blue.DamageType_Fire_Primary_Blue_C"))))

(event OnComponentEndOverlap(FireTrigger)
  (params (OverlappedComponent :type Primitive%20Component%20Object%20Reference) (OtherActor :type Actor%20Object%20Reference) (OtherComp :type Primitive%20Component%20Object%20Reference) (OtherBodyIndex :type Integer))
  (if (Actor|ActorHasTag OtherActor "player")
    (Math|Integer|DecrementInt (Variables|Default|GetColliders%20that%20detect%20player))))

(event Custom|Enable/Disable%20Barrier
  (params (Enable? :type Boolean))
  (Collision|SetActorEnableCollision Enable?)
  (Rendering|SetActorHiddenInGame (not Enable?))
  (Actor|Tick|SetActorTickEnabled true))

(event EventBeginPlay
  (bind _asbp_top_down_character (Utilities|Casting|CastToBP_TopDownCharacter (Game|GetPlayerCharacter 0)))
  (Variables|Default|SetPlayer _asbp_top_down_character)
  (Actor|Tick|SetActorTickEnabled false)
  (Components|Activation|SetActive (Variables|Default|GetFire_blue_larger) false false)
  (Collision|SetCollisionEnabled (Variables|Default|GetInvisible%20Wall) "NoCollision"))

(event Collision|EventActorBeginOverlap
  (params (OtherActor :type Actor%20Object%20Reference)))

(event EventTick
  (params (DeltaSeconds :type Float%20%28single-precision%29))
  (if (> (Variables|Default|GetColliders%20that%20detect%20player) 0)
    (Game|Damage|ApplyDamage (Variables|Default|GetPlayer) (Variables|Default|GetDamage) 0 0 "/Game/BP/DamageType_Fire_Primary_Blue.DamageType_Fire_Primary_Blue_C")
    (Utilities|KnockbackCharacter (Variables|Default|GetPlayer) 1.0)))

(fn ConstructionScript
  (CallFunction|Enable/DisableBarrier false))