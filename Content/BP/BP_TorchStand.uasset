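; Torch stand actor that switches between lit and unlit states.
; Activate/DeactivateTorch stores the state and updates the look, toggling fire particles and swapping visibility between lit and unlit point lights.
; The construction script applies the initial state and shadow casting to both lights.
; Optionally, activation fires a numbered event once through the GameController held by BP_GameInstance.
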(event Custom|Update%20Torch%20Appearance
  (bind _torch_activated (Variables|Default|GetTorch%20Activated))
  (Components|Activation|SetActive (Variables|Default|GetFire%20Particles) _torch_activated false)
  (Rendering|SetVisibility (Variables|Default|GetPointLight%20-%20Lit) _torch_activated false)
  (Rendering|SetVisibility (Variables|Default|GetPointLight%20-%20Unlit) (not _torch_activated) false))

(event Custom|Activate/Deactivate%20Torch
  (params (Torch%20Activated :type Boolean))
  (bind _output_get (Variables|Default|SetTorch%20Activated Torch%20Activated))
  (CallFunction|UpdateTorchAppearance)
  (if (and (Variables|Default|GetTrigger%20Event%20on%20Activation) _output_get)
    (Utilities|FlowControl|DoOnce false
      (:Completed
        (bind _asbp_game_instance (Utilities|Casting|CastToBP_GameInstance (Game|GetGameInstance)))
        (Default|TriggerEvent (Variables|/Game/BP/BP_GameInstance.BP_GameInstance_C|GetGame%20Controller _asbp_game_instance) (Variables|Default|GetTrigger%20Event%20on%20Activation%20-%20Event%20Num))))))

(event EventBeginPlay)

(event Collision|EventActorBeginOverlap
  (params (OtherActor :type Actor%20Object%20Reference)))

(event EventTick
  (params (DeltaSeconds :type Float%20%28single-precision%29)))

(fn ConstructionScript
  (Components|Activation|SetAutoActivate (Variables|Default|GetFire%20Particles) (Variables|Default|GetTorch%20Activated))
  (CallFunction|UpdateTorchAppearance)
  (Rendering|Components|Light|SetCastShadows (Variables|Default|GetPointLight%20-%20Unlit) (Variables|Default|GetCast%20Shadows)))