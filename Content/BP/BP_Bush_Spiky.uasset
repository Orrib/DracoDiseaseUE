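; BP_Bush_Spiky is a bush hazard that hurts players and NPCs touching its damage collision.
; Overlap applies environmental point damage and launches characters away from the bush, with force scaled inversely by their mass.
; Only fire damage is passed to the parent's handler, and four seconds later the damage collision is disabled.
; A bush flagged as KnightCommanderSpecialBush then also triggers a game controller event through the game instance.
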(event OnComponentBeginOverlap(DamageCollision)
  (params (OverlappedComponent :type Primitive%20Component%20Object%20Reference) (OtherActor :type Actor%20Object%20Reference) (OtherComp :type Primitive%20Component%20Object%20Reference) (OtherBodyIndex :type Integer) (bFromSweep :type Boolean) (SweepResult :type Hit%20Result%20Structure%20%28by%20ref%29))
  (bind _returnvalue (Transformation|GetActorLocation OtherActor))
  (bind _scene (Variables|Default|GetScene))
  (bind _returnvalue_2 (Transformation|GetWorldLocation _scene))
  (bind _returnvalue_3 (Math|Vector|GetUnitDirection(Vector) _returnvalue_2 _returnvalue))
  (if (or (Actor|ActorHasTag OtherActor "npc") (Actor|ActorHasTag OtherActor "player"))
    (Game|Damage|ApplyPointDamage OtherActor (Variables|Default|GetDamage) _returnvalue_3 (Collision|MakeHitResult false false 0.0 0.0 "0, 0, 0" "0, 0, 0" "0,0,1" "0,0,1" 0 0) 0 self "/Engine/EngineDamageTypes/DmgTypeBP_Environmental.DmgTypeBP_Environmental_C")
    (bind _ascharacter (Utilities|Casting|CastToCharacter OtherActor))
    ;[1 1 1] Apply Impulse, accountinmg for mass
    (Character|LaunchCharacter _ascharacter (* _returnvalue_3 (/ 5e+04 (Variables|/Script/Engine.CharacterMovementComponent|GetMass (Variables|/Script/Engine.Character|GetCharacterMovement _ascharacter)))) true true)))

(event EventBeginPlay
  (|CallParentFunction))

(event Collision|EventActorBeginOverlap
  (params (OtherActor :type Actor%20Object%20Reference))
  (|CallParentFunction OtherActor))

(event EventTick
  (params (DeltaSeconds :type Float%20%28single-precision%29))
  (|CallParentFunction DeltaSeconds) ; This node is disabled and will not be called.\nDrag off pins to build functionality.
)

(event Game|Damage|EventAnyDamage
  (params (Damage :type Float%20%28single-precision%29) (DamageType :type Damage%20Type%20Object%20Reference) (InstigatedBy :type Controller%20Object%20Reference) (DamageCauser :type Actor%20Object%20Reference))
  (if (Utilities|ClassIsChildOf (Utilities|GetClass DamageType) "/Game/BP/DamageType_Fire.DamageType_Fire_C")
    (|CallParentFunction Damage DamageType InstigatedBy DamageCauser)
    (Utilities|FlowControl|Delay 4.0)
    (Collision|SetCollisionEnabled (Variables|Default|GetDamage%20Collision) "NoCollision")
    (if (Variables|Default|GetKnight%20Commander%20Special%20Bush?)
      (bind _asbp_game_instance (Utilities|Casting|CastToBP_GameInstance (Game|GetGameInstance)))
      (Default|TriggerEvent (Variables|/Game/BP/BP_GameInstance.BP_GameInstance_C|GetGame%20Controller _asbp_game_instance) 34))))

(fn ConstructionScript
  (|CallParentFunction))