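; BP_Book is a book prop actor that can vary its own look, with all logic in the Construction Script and no active event graph.
; When RandomizeColor is set, it applies a random pick from five basic color materials to several of its plane components.
; When RandomizeOpeningAmount is set, it pitches Scene1 to a random angle up to a half turn.
; Both use unseeded random nodes, so results can change whenever construction reruns.
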(event EventBeginPlay)

(event Collision|EventActorBeginOverlap
  (params (OtherActor :type Actor%20Object%20Reference)))

(event EventTick
  (params (DeltaSeconds :type Float%20%28single-precision%29)))

(fn ConstructionScript
  (Utilities|FlowControl|Sequence
    (:then_0
      (if (Variables|Default|GetRandomize%20Color)
        (Rendering|Material|SetMaterial (Variables|Default|GetPlane2) 0 (Utilities|Select :Index (Math|Random|RandomIntegerinRange 0 4) :Option%200 "/Game/Materials/M_Basic_Brown_Light.M_Basic_Brown_Light" :Option%201 "/Game/Materials/M_Basic_Brown.M_Basic_Brown" :Option%202 "/Game/Materials/M_Basic_Pink.M_Basic_Pink" :Option%203 "/Game/Materials/M_Basic_Green_Light.M_Basic_Green_Light" :Option%204 "/Game/Materials/M_Basic_Yellow.M_Basic_Yellow"))))
    (:then_1
      (if (Variables|Default|GetRandomize%20Opening%20Amount)
        (Transformation|SetRelativeRotation (Variables|Default|GetScene1) (Math|Rotator|MakeRotator 0.0 (Math|Random|RandomFloatinRange 0.0 1.8e+02) 0.0) false false)))))