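; BP_PlayerController_StartMenu is the player controller for the start menu, handling input setup and access to the cheat popup.
; On BeginPlay it resets Enhanced Input to only the IMC_Essential mapping context and caches the BP_GameInstance reference.
; The IA_Cheats_OpenCheatPopup action toggles the cheat popup through the game instance, using the popup's validity to decide whether to open or close it.
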(event Input|EnhancedActionEvents|EnhancedInputActionIA_Cheats_OpenCheatPopup
  (params (ActionValue :type Boolean) (ElapsedSeconds :type Float%20%28double-precision%29) (TriggeredSeconds :type Float%20%28double-precision%29) (InputAction :type Input%20Action%20Object%20Reference :default "/Game/TopDown/Input/Actions/IA_Cheats_OpenCheatPopup.IA_Cheats_OpenCheatPopup"))
  (bind _game_instance (Variables|Default|GetGame%20Instance))
  ;[1 1 1] Cheats
  (:Started
    (Utilities|IsValid (Variables|/Game/BP/BP_GameInstance.BP_GameInstance_C|GetCheat%20Popup _game_instance)
      (:Is%20Valid
        (Default|Open/CloseCheatsPopup _game_instance false))
      (:Is%20Not%20Valid
        (Default|Open/CloseCheatsPopup _game_instance true)))))

(event EventBeginPlay
  (bind _returnvalue (PlayerController|LocalPlayerSubsystems|GetEnhancedInputLocalPlayerSubsystem))
  (Utilities|FlowControl|Sequence
    (:then_0
      ;[0.05098 0.05098 0.05098] Add Essential Mapping Context
      (Utilities|IsValid _returnvalue
        (:Is%20Valid
          (Class|EnhancedInputSubsystemInterface|ClearAllMappings _returnvalue)
          (Input|AddMappingContext _returnvalue "/Game/TopDown/Input/IMC_Essential.IMC_Essential" 0 "(bIgnoreAllPressedKeysUntilRelease=True,bForceImmediately=False,bNotifyUserSettings=False)"))))
    (:then_1
      (bind _asbp_game_instance (Utilities|Casting|CastToBP_GameInstance (Game|GetGameInstance)))
      (Variables|Default|SetGame%20Instance _asbp_game_instance))))

(fn ConstructionScript)