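; Blue crystal sprite pickup, a child Blueprint that adds one item to the player's inventory when collected.
; OnPickup shows a rising icon and adds the item through the player controller, then runs the parent's pickup logic.
; Can Pickup? combines the parent check with a max-quantity test on the impersistent save game.
; That test queries a different item enum entry (NewEnumerator0) than the one granted (NewEnumerator6).
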(event EventBeginPlay
  (|CallParentFunction) ; This node is disabled and will not be called.\nDrag off pins to build functionality.
)

(event Collision|EventActorBeginOverlap
  (params (OtherActor :type Actor%20Object%20Reference))
  (|CallParentFunction OtherActor) ; This node is disabled and will not be called.\nDrag off pins to build functionality.
)

(event EventTick
  (params (DeltaSeconds :type Float%20%28single-precision%29))
  (|CallParentFunction DeltaSeconds) ; This node is disabled and will not be called.\nDrag off pins to build functionality.
)

(event EventOnPickup
  (params (Player%20Controller :type BP%20Top%20Down%20Controller%20Object%20Reference))
  (Utilities|FlowControl|Sequence
    (:then_0
      (CallFunction|ShowRisingIcon Player%20Controller)
      (Default|AddItemtoInventory Player%20Controller "NewEnumerator6" 1))
    (:then_1
      (|CallParentFunction Player%20Controller))))

(fn ConstructionScript
  (|CallParentFunction))

(fn CanPickup?
  (params (Top%20Down%20Controller :type BP%20Top%20Down%20Controller%20Object%20Reference))
  (bind _can_pickup_ (|CallParentFunction Top%20Down%20Controller))
  (bind _game_instance (Variables|/Game/TopDown/Blueprints/BP_TopDownController.BP_TopDownController_C|GetGame%20Instance Top%20Down%20Controller))
  (bind _save_game_instance___impersistent (Variables|/Game/BP/BP_GameInstance.BP_GameInstance_C|GetSave%20Game%20Instance%20-%20Impersistent _game_instance))
  (bind (_item_in_inventory _at_max_quantity) (Default|IsInventoryItematMaxQuantity? _save_game_instance___impersistent "NewEnumerator0"))
  (if _item_in_inventory
    (return (and (not _at_max_quantity) _can_pickup_))
    (else
      (return _can_pickup_))))