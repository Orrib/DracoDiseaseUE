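; BP_Interactable_Lore is a lore interactable that can fire a game event when its lore widget is closed.
; OnLoreClosed checks a toggle, then passes a configured event number to TriggerEvent on the GameController held by BP_GameInstance.
; The other event nodes are disabled stubs, and the construction script only calls the parent.
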(event Custom|On%20Lore%20Closed
  (if (Variables|OnLoreClosed|GetOn%20Lore%20Widget%20Closed%20-%20Trigger%20Event?)
    (bind _asbp_game_instance (Utilities|Casting|CastToBP_GameInstance (Game|GetGameInstance)))
    (Default|TriggerEvent (Variables|/Game/BP/BP_GameInstance.BP_GameInstance_C|GetGame%20Controller _asbp_game_instance) (Variables|OnLoreClosed|GetOn%20Lore%20Widget%20Closed%20-%20Event%20Num))))

(event EventBeginPlay
  (|CallParentFunction) ; This node is disabled and will not be called.\nDrag off pins to build functionality.
)

(event Collision|EventActorBeginOverlap
  (params (OtherActor :type Actor%20Object%20Reference))
  (|CallParentFunction OtherActor) ; This node is disabled and will not be called.\nDrag off pins to build functionality.
)

(event EventTick
  (params (DeltaSeconds :type Float%20%28single-precision%29))
  (|CallParentFunction DeltaSeconds) ; This node is disabled and will not be called.\nDrag off pins to build functionality.
)

(fn ConstructionScript
  (|CallParentFunction))