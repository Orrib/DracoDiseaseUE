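; Player charge-attack sword wave actor: a flipbook slash that travels forward and fades out.
; On BeginPlay, the MoveForward timeline runs at a rate derived from SlashDuration with random variation.
; It moves the slash origin and radial force from Start to End while fading the dark sprite tint.
; Construction adds a "parry" tag and offsets both slash flipbooks, including the lower hitbox, slightly into playback.
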(event EventBeginPlay
  (|CallParentFunction)
  (Components|Timeline|SetPlayRate (Variables|Default|GetMove%20Forward) (Math|Float|Power (* (Variables|Default|GetSlash%20Duration) (Math|Random|RandomFloatinRange 0.7 1.0)) -1.0))
  (bind (_direction _newtrack_0 _slash_opacity) (Timeline|Move%20Forward PlayFromStart)
    (:Update
      (Transformation|SetWorldLocation (Variables|Default|GetSlash%20Origin) (Math|Vector|Lerp(Vector) (Transformation|GetWorldLocation (Variables|Default|GetStart)) (Transformation|GetWorldLocation (Variables|Default|GetEnd)) _newtrack_0) false false)
      (Sprite|SetSpriteColor (Variables|Default|GetSwordSlash) (Math|Color|Lerp(LinearColor) "(R=0.000000,G=0.000000,B=0.000000,A=0.634000)" "(R=0.000000,G=0.000000,B=0.000000,A=0.000000)" _slash_opacity)))))

(event Collision|EventActorBeginOverlap
  (params (OtherActor :type Actor%20Object%20Reference))
  (|CallParentFunction OtherActor) ; This node is disabled and will not be called.\nDrag off pins to build functionality.
)

(event EventTick
  (params (DeltaSeconds :type Float%20%28single-precision%29))
  (|CallParentFunction DeltaSeconds) ; This node is disabled and will not be called.\nDrag off pins to build functionality.
)

(fn ConstructionScript
  (|CallParentFunction)
  (Utilities|Array|AddUnique (Variables|Default|GetTags) "parry")
  (Components|Timeline|SetPlaybackPosition (Variables|Default|GetSwordSlash) (* (Class|PaperFlipbookComponent|GetFlipbookLength (Variables|Default|GetSwordSlash%20-%20Lower%20Hitbox)) 0.1) false))