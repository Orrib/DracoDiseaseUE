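; BP_GolemRock is a rock actor that spawns a golem enemy and holds a set of patrol points.
; On BeginPlay it spawns BP_GolemEnemy at the GolemSpawn component, registers itself as RockActor on that golem's GolemController, and caches the children of PatrolPointParent as patrol points.
; The construction script can draw debug spheres at those points when DebugPatrolPoints is enabled.
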(event EventBeginPlay
  (bind _returnvalue (Game|SpawnActorfromClass "/Game/BP/BP_GolemEnemy.BP_GolemEnemy_C" (Math|Transform|MakeTransform (Transformation|GetWorldLocation (Variables|Default|GetGolem%20Spawn)) "0, 0, 0" "1.000000,1.000000,1.000000") "AdjustIfPossibleButAlwaysSpawn" "MultiplyWithRoot" 0 0))
  (Variables|/Game/BP/BP_GolemController.BP_GolemController_C|SetRock%20Actor (Variables|/Game/BP/BP_GolemEnemy.BP_GolemEnemy_C|GetGolem%20Controller _returnvalue) self)
  (Variables|Default|SetPatrol%20Pointss (Components|GetChildrenComponents (Variables|Default|GetPatrol%20Point%20Parent) false)))

(fn ConstructionScript
  ;[1 1 1] Debug Patrol Points
  (if (Variables|Default|GetDebug%20Patrol%20Points)
    (for _array_element (Components|GetChildrenComponents (Variables|Default|GetPatrol%20Point%20Parent) false)
      (Rendering|Debug|DrawDebugSphere (Transformation|GetWorldLocation _array_element) 5.0 12 "(R=0.024871,G=0.145833,B=0.000000,A=1.000000)" 0.0 3.0))))