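; BP_Interactable_Book_1 is an interactable book that switches between closed and open looks to show whether its lore has been collected.
; UpdateAppearance shows the Open component and hides Closed, children included, when LoreCollected or AlwaysOpen is true, and does the reverse otherwise.
; The construction script applies this state after the parent's construction, and OnClickedLoreButton sets LoreCollected and refreshes it.
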(event Custom|Update%20Appearance
  (bind _lore_collected (Variables|Default|GetLore%20Collected))
  (bind _always_open (Variables|Default|GetAlways%20Open))
  (bind _returnvalue (or _lore_collected _always_open))
  (Rendering|SetVisibility (Variables|Default|GetOpen) _returnvalue true)
  (Rendering|SetVisibility (Variables|Default|Get%20Closed) (not _returnvalue) true))

(event EventBeginPlay
  (|CallParentFunction))

(event Collision|EventActorBeginOverlap
  (params (OtherActor :type Actor%20Object%20Reference))
  (|CallParentFunction OtherActor) ; This node is disabled and will not be called.\nDrag off pins to build functionality.
)

(event EventTick
  (params (DeltaSeconds :type Float%20%28single-precision%29))
  (|CallParentFunction DeltaSeconds) ; This node is disabled and will not be called.\nDrag off pins to build functionality.
)

(event EventOnClickedLoreButton
  (Variables|Default|SetLore%20Collected true)
  (CallFunction|UpdateAppearance))

(fn ConstructionScript
  (|CallParentFunction)
  (CallFunction|UpdateAppearance))