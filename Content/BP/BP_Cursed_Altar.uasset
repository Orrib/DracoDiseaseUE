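; BP_Cursed_Altar is an altar actor that shows an on-screen widget when something overlaps it.
; An unused altar creates the cursed altar widget with a debuff timer, while a used one creates an "altar used" widget instead.
; End overlap removes both widgets, validity-checking only the "altar used" one.
; The HasBeenUsed flag picks the widget but is never set in this graph.
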(event Collision|EventActorBeginOverlap
  (params (OtherActor :type Actor%20Object%20Reference))
  (if (Variables|Default|GetHasBeenUsed)
    (bind _returnvalue (UserInterface|CreateWidget "/Game/UI/Widget_AltarUsed.Widget_AltarUsed_C"))
    (bind _output_get (Variables|Default|SetWidget_AltarUsedRef _returnvalue))
    (UserInterface|Viewport|AddtoViewport _output_get 0)
    (else
      (bind _returnvalue_2 (UserInterface|CreateWidget "/Game/UI/Widget_CursedAltar.Widget_CursedAltar_C"))
      (bind _output_get_2 (Variables|Default|SetWidget _returnvalue_2))
      (UserInterface|Viewport|AddtoViewport _output_get_2 0))))

(event Collision|EventActorEndOverlap
  (params (OtherActor :type Actor%20Object%20Reference))
  (bind _widget_altarusedref (Variables|Default|GetWidget_AltarUsedRef))
  (Widget|RemovefromParent (Variables|Default|GetWidget))
  (Utilities|IsValid _widget_altarusedref
    (:Is%20Valid
      (Widget|RemovefromParent _widget_altarusedref))))

(fn ConstructionScript)