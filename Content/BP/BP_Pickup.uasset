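; Base pickup actor that the player collects by overlapping its box, with a CanPickup check that passes by default.
; Collection records the object name in the save game and destroys it; flagged persistent pickups self-destroy on BeginPlay if already recorded.
; Rejection plays an error sound and flickers the mesh.
; Optional delayed collision or trigger activation, proximity spinning, randomized cone launch and a rising icon above the player's head are also provided.
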(event OnComponentBeginOverlap(Box)
  (params (OverlappedComponent :type Primitive%20Component%20Object%20Reference) (OtherActor :type Actor%20Object%20Reference) (OtherComp :type Primitive%20Component%20Object%20Reference) (OtherBodyIndex :type Integer) (bFromSweep :type Boolean) (SweepResult :type Hit%20Result%20Structure%20%28by%20ref%29))
  (Utilities|String|LogString (Utilities|GetDisplayName OtherActor))
  (if (Actor|ActorHasTag OtherActor "player")
    (bind _asbp_top_down_character (Utilities|Casting|CastToBP_TopDownCharacter OtherActor))
    (bind _asbp_top_down_controller (Utilities|Casting|CastToBP_TopDownController (Pawn|GetController _asbp_top_down_character)))
    (if (not (Variables|Default|GetPicked%20Up))
      (if (CallFunction|CanPickup? _asbp_top_down_controller)
        (Variables|Default|SetPicked%20Up true)
        (CallFunction|OnPickup _asbp_top_down_controller)
        (else
          (CallFunction|OnPickupRejected))))))

(event OnComponentBeginOverlap(SpinTrigger)
  (params (OverlappedComponent :type Primitive%20Component%20Object%20Reference) (OtherActor :type Actor%20Object%20Reference) (OtherComp :type Primitive%20Component%20Object%20Reference) (OtherBodyIndex :type Integer) (bFromSweep :type Boolean) (SweepResult :type Hit%20Result%20Structure%20%28by%20ref%29))
  (if (Variables|Default|GetSpin%20Object)
    (if (Actor|ActorHasTag OtherActor "player")
      (CallFunction|Spin))))

(event OnComponentEndOverlap(SpinTrigger)
  (params (OverlappedComponent :type Primitive%20Component%20Object%20Reference) (OtherActor :type Actor%20Object%20Reference) (OtherComp :type Primitive%20Component%20Object%20Reference) (OtherBodyIndex :type Integer))
  (if (Variables|Default|GetSpin%20Object)
    (if (Actor|ActorHasTag OtherActor "player")
      (Audio|Components|Audio|Stop (Variables|Default|GetTimeline)))))

(event Custom|On%20Pickup
  (params (Player%20Controller :type BP%20Top%20Down%20Controller%20Object%20Reference))
  (CallFunction|AddIDforPersistentDeath)
  (Actor|DestroyActor))

(event Custom|Start%20Delayed%20Spawn%20Trigger%20Activation
  (bind _box (Variables|Default|GetBox))
  (Collision|SetCollisionEnabled _box "NoCollision")
  (Utilities|FlowControl|Delay (+ (Variables|DelayedSpawnCollision|GetDelayed%20Spawn%20Collision/Trigger%20Time) (Math|Random|RandomFloatinRange 0.0 0.5)))
  (Collision|SetCollisionEnabled _box "QueryOnly"))

(event Custom|Spin
  (bind _newtrack_0 (Timeline|Timeline PlayFromStart)
    (:Update
      (Transformation|SetRelativeRotation (Variables|Default|GetObject%20Parent) (Math|Rotator|MakeRotator 0.0 0.0 (Math|Float|Lerp 0.0 3.6e+02 _newtrack_0)) false false))))

(event Custom|Show%20Rising%20Icon
  (params (Player%20Controller :type BP%20Top%20Down%20Controller%20Object%20Reference))
  (bind _returnvalue (Game|SpawnActorfromClass (Variables|Default|GetRising%20Icon) (Math|Transform|MakeTransform "0, 0, 0" "0, 0, 0" "1.000000,1.000000,1.000000") "AlwaysSpawn" "MultiplyWithRoot" 0 0.2 0))
  (Transformation|AttachComponentToComponent _returnvalue (Variables|/Game/TopDown/Blueprints/BP_TopDownCharacter.BP_TopDownCharacter_C|GetHead%20Position (Variables|/Game/TopDown/Blueprints/BP_TopDownController.BP_TopDownController_C|GetTop%20Down%20Character Player%20Controller)) "None" "SnapToTarget" "KeepWorld" "KeepWorld" false))

(event Custom|Launch%20Pickup
  (params (Launch%20Direction :type Vector))
  (Physics|SetPhysicsLinearVelocity (Variables|Default|GetGround%20Collider) (* (Math|Random|RandomUnitVectorinConeinDegrees Launch%20Direction 25.0) (Variables|Default|GetMax%20Launch%20Speed) (Math|Random|RandomFloatinRange 0.4 1.0)) false "None"))

(event Custom|Start%20Delayed%20Spawn%20Collision
  (Collision|SetActorEnableCollision false)
  (Utilities|FlowControl|Delay (Variables|DelayedSpawnCollision|GetDelayed%20Spawn%20Collision/Trigger%20Time))
  (Collision|SetActorEnableCollision true))

(event Custom|On%20Pickup%20Rejected
  (Audio|PlaySound2D "/Game/Sound/SoundFX/Cue_Error.Cue_Error" 0.3 1.0 0.0 0 0)
  (Rendering|SetActorHiddenInGame true)
  (Utilities|FlowControl|Delay 0.1)
  (Rendering|SetActorHiddenInGame false)
  (Utilities|FlowControl|Delay 0.1)
  (Rendering|SetActorHiddenInGame true)
  (Utilities|FlowControl|Delay 0.1)
  (Rendering|SetActorHiddenInGame false)
  (Utilities|FlowControl|Delay 0.1)
  (Rendering|SetActorHiddenInGame true)
  (Utilities|FlowControl|Delay 0.1)
  (Rendering|SetActorHiddenInGame false))

(event EventBeginPlay
  (CallFunction|CheckforPersistentDeathandDestroy)
  (Utilities|FlowControl|Sequence
    (:then_0
      (if (Variables|DelayedSpawnCollision|GetDelayed%20Spawn%20Collision)
        (CallFunction|StartDelayedSpawnCollision)))
    (:then_1
      (if (Variables|DelayedSpawnCollision|GetDelayed%20Spawn%20Trigger%20Activation)
        (CallFunction|StartDelayedSpawnTriggerActivation)))))

(fn ConstructionScript
  (Collision|SetActorEnableCollision (not (Variables|DelayedSpawnCollision|GetDelayed%20Spawn%20Collision))))

(fn CanPickup?
  (params (Top%20Down%20Controller :type BP%20Top%20Down%20Controller%20Object%20Reference))
  (return true))

(fn AddIDforPersistentDeath
  (bind _asbp_game_instance (Utilities|Casting|CastToBP_GameInstance (Game|GetGameInstance)))
  (Default|AddNPCIDonDeath(PersistentDeath) (Variables|/Game/BP/BP_GameInstance.BP_GameInstance_C|GetSave%20Game%20Instance%20-%20Impersistent _asbp_game_instance) (Utilities|GetObjectName self)))

(fn CheckforPersistentDeath
  (if (Variables|Default|GetPersistent%20Pickup%20%28Keep%20Dead%20across%20saves%29)
    (bind _asbp_game_instance (Utilities|Casting|CastToBP_GameInstance (Game|GetGameInstance)))
    (bind _id_found_ (Default|IsNPCDead?(PersistentDeath) (Variables|/Game/BP/BP_GameInstance.BP_GameInstance_C|GetSave%20Game%20Instance%20-%20Impersistent _asbp_game_instance) (Utilities|GetObjectName self)))
    (return _id_found_)
    (else
      (return false))))

(fn CheckforPersistentDeathandDestroy
  (if (Variables|Default|GetPersistent%20Pickup%20%28Keep%20Dead%20across%20saves%29)
    (bind _asbp_game_instance (Utilities|Casting|CastToBP_GameInstance (Game|GetGameInstance)))
    (bind _id_found_ (Default|IsNPCDead?(PersistentDeath) (Variables|/Game/BP/BP_GameInstance.BP_GameInstance_C|GetSave%20Game%20Instance%20-%20Impersistent _asbp_game_instance) (Utilities|GetObjectName self)))
    (if _id_found_
      (Actor|DestroyActor))))