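; BP_GameManager is the game manager for the book organizer challenge, a timed task of placing books correctly to earn a treasure.
; Overlap events set up the timer and book count, and a tick event counts time down, calling an empty OnLose on timeout.
; Each correct placement decrements the remaining books, notifies the HUD and spawns the reward when none remain in time.
; Placement validation is unfinished, and unplacing and win handling are stubs.
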(event OnComponentBeginOverlap(WBP_HUD)
  (params (OverlappedComponent :type Primitive%20Component%20Object%20Reference) (OtherActor :type Actor%20Object%20Reference) (OtherComp :type Primitive%20Component%20Object%20Reference) (OtherBodyIndex :type Integer) (bFromSweep :type Boolean) (SweepResult :type Hit%20Result%20Structure%20%28by%20ref%29))
  ;[1 1 1] Player goes through the trigger box call HUD
  (Variables|Default|SetTimeRemaining 2e+01)
  (Variables|Default|SetBooksRemaining 8))

(event Custom|OnTimerTick
  ;[1 1 1] If Timer is active then move to TickTimer
  (if (Variables|Default|GetbTimerActive)
    (CallFunction|TickTimer(DeltaTime))))

(event Custom|OnBooksRemainingChanged)

(event Custom|OnWin)

(event Custom|OnLose)

(event Collision|EventActorBeginOverlap
  (params (OtherActor :type Actor%20Object%20Reference))
  ;[1 1 1] Begin BookOrganizer
  (Variables|Default|SetBooksRemaining (Math|Conversions|ToInteger(Boolean) (== (Variables|Default|GetTotalBooks) (Variables|Default|GetBooksRemaining))))
  (Variables|Default|SetTimeRemaining (Math|Conversions|ToFloat(Boolean) (== (Variables|Default|GetStartTimeSeconds) (Variables|Default|GetTimeRemaining))))
  (Utilities|FlowControl|Delay 5.0)
  (Variables|Default|SetbTimerActive true))

(fn ConstructionScript)

(fn StartTimerifNeeded
  (if (Variables|Default|GetbTimerActive)
    (Variables|Default|SetbTimerActive true)))

(fn TickTimer(DeltaTime)
  (Variables|Default|SetTimeRemaining (Utilities|Operators|Subtract (Variables|Default|GetTimeRemaining) (Class|AnimExecutionContextLibrary|GetDeltaTime (Utilities|Struct|MakeAnimUpdateContext))))
  (if (and (<= (Variables|Default|GetTimeRemaining) 0.0) (> (Variables|Default|GetBooksRemaining) 0))
    (CallFunction|OnLose)))

(fn RegisterBookPlacedCorrect
  (Variables|Default|SetBooksRemaining (- (Variables|Default|GetBooksRemaining) 1))
  (FieldNotification|BroadcastFieldValueChanged :Object "/Game/BP/BookOrganizer/WBP_HUD/WBP_HUD.WBP_HUD")
  (if (and (> (Variables|Default|GetTimeRemaining) 0.0) (== (Variables|Default|GetBooksRemaining) 0))
    (CallFunction|SpawnReward)))

(fn RegisterBookUnplaced)

(fn ValidatePlacement
  (CallFunction|StartTimerifNeeded :!label _label)
  (if (and (== (LocalVariables|GetBookTargetIndex) (LocalVariables|GetBookCaseIndex)) (Variables|/Game/BP/BookOrganizer/Books/BP_Book_1.BP_Book_1_C|GetbPlaced (LocalVariables|GetBP_Book)))
    (|ForEachEAppReturnType
      (:LoopBody
        (goto _label)))))

(fn SpawnReward
  (Game|SpawnActorfromClass "/Game/BP/BookOrganizer/Reward/BP_Treasure_Special_Organizer.BP_Treasure_Special_Organizer_C" (Variables|Default|GetRewardSpawnTransform) "Undefined" "MultiplyWithRoot" 0 false 1.0 false true 0))