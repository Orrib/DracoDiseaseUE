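; BP_Volume_FixedCam is a trigger volume that switches the player's view to a fixed camera while they are inside it.
; When a "player"-tagged actor overlaps, it blends the TopDownController's view target to itself, then back to the TopDownCharacter on exit.
; References resolve through the GameInstance cached on BeginPlay.
; Tick delays cover references that are not yet valid, without rechecking afterwards.
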(event EventBeginPlay
  (bind _asbp_game_instance (Utilities|Casting|CastToBP_GameInstance (Game|GetGameInstance)))
  (Variables|Default|SetBP%20Game%20Instance _asbp_game_instance))

(event Collision|EventActorBeginOverlap
  (params (OtherActor :type Actor%20Object%20Reference))
  (bind _bp_game_instance (Variables|Default|GetBP%20Game%20Instance))
  (bind _game_controller (Variables|/Game/BP/BP_GameInstance.BP_GameInstance_C|GetGame%20Controller _bp_game_instance))
  (bind _top_down_character (Variables|/Game/BP/BP_GameController.BP_GameController_C|GetTop%20Down%20Character _game_controller))
  (bind _top_down_controller (Variables|/Game/TopDown/Blueprints/BP_TopDownCharacter.BP_TopDownCharacter_C|GetTop%20Down%20Controller _top_down_character))
  (if (Actor|ActorHasTag OtherActor "player")
    (Utilities|IsValid _game_controller
      (:Is%20Valid
        (Utilities|IsValid _top_down_character
          (:Is%20Valid
            (Utilities|IsValid _top_down_controller
              (:Is%20Valid
                _)
              (:Is%20Not%20Valid
                (Utilities|FlowControl|DelayUntilNextTick :!label _label)
                (Utilities|FlowControl|DelayUntilNextTick))))
          (:Is%20Not%20Valid
            (goto _label))))
      (:Is%20Not%20Valid
        (goto _label)))
    (Game|Player|SetViewTargetwithBlend _top_down_controller self (Variables|Default|GetCam%20Blend%20Time) "VTBlend_EaseInOut" 3.0 false)))

(event EventTick
  (params (DeltaSeconds :type Float%20%28single-precision%29)))

(event Collision|EventActorEndOverlap
  (params (OtherActor :type Actor%20Object%20Reference))
  (bind _bp_game_instance (Variables|Default|GetBP%20Game%20Instance))
  (bind _game_controller (Variables|/Game/BP/BP_GameInstance.BP_GameInstance_C|GetGame%20Controller _bp_game_instance))
  (bind _top_down_character (Variables|/Game/BP/BP_GameController.BP_GameController_C|GetTop%20Down%20Character _game_controller))
  (bind _top_down_controller (Variables|/Game/TopDown/Blueprints/BP_TopDownCharacter.BP_TopDownCharacter_C|GetTop%20Down%20Controller _top_down_character))
  (if (Actor|ActorHasTag OtherActor "player")
    (Utilities|IsValid _top_down_controller
      (:Is%20Valid
        _)
      (:Is%20Not%20Valid
        (Utilities|FlowControl|DelayUntilNextTick)))
    (Game|Player|SetViewTargetwithBlend _top_down_controller _top_down_character (Variables|Default|GetCam%20Blend%20Time) "VTBlend_EaseInOut" 3.0 false)))

(fn ConstructionScript)