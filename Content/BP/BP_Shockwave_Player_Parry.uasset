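; Player parry shockwave actor that adds animated left and right sword slash flipbooks on top of its parent's BeginPlay behavior.
; Both flipbooks' play rates are derived from the right slash's length so the animation spans ShockTime plus FadeTime.
; SlashTimeline runs at the inverse of that same duration, scaling SlashParent in world space from a narrow shape to full size.
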(event EventBeginPlay
  (bind _shock_time (Variables|Default|GetShock%20Time))
  (bind _fade_time (Variables|Default|GetFade%20Time))
  (bind _returnvalue (+ _shock_time _fade_time))
  (|CallParentFunction)
  ;[1 1 1] convert slash time to play rate
  (Components|Timeline|SetPlayRate (Variables|Default|GetSwordSlash%20-%20Left) (/ (Class|PaperFlipbookComponent|GetFlipbookLength (Variables|Default|GetSwordSlash%20-%20Right)) _returnvalue))
  (Components|Timeline|SetPlayRate (Variables|Default|GetSlash%20Timeline) (Math|Float|Power _returnvalue -1.0))
  (bind _newtrack_0 (Timeline|Slash%20Timeline PlayFromStart)
    (:Update
      (Transformation|SetWorldScale3D (Variables|Default|GetSlash%20Parent) (Math|Vector|Lerp(Vector) "0.200000,1.000000,0.200000" "1.000000,1.000000,1.000000" _newtrack_0)))))

(event Collision|EventActorBeginOverlap
  (params (OtherActor :type Actor%20Object%20Reference))
  (|CallParentFunction OtherActor) ; This node is disabled and will not be called.\nDrag off pins to build functionality.
)

(event EventTick
  (params (DeltaSeconds :type Float%20%28single-precision%29))
  (|CallParentFunction DeltaSeconds) ; This node is disabled and will not be called.\nDrag off pins to build functionality.
)

(fn ConstructionScript
  (|CallParentFunction))