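; Blessed altar interactable that can be activated from its widget's altar button when the player controller's BlessingActive check returns false.
; While inactive, showing the widget lights the main light and spins the cauldron water through a Timeline.
; Activation lights the candle, clears the water, adjusts sound volume and disables detector overlaps.
; The altar's object name is recorded in the game instance's impersistent save and restores activation on BeginPlay.
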(event Custom|CustomEvent_0
  (bind _asbp_game_instance (Utilities|Casting|CastToBP_GameInstance (Game|GetGameInstance)))
  (if (not (Default|BlessingActive? (Variables|/Game/BP/BP_GameInstance.BP_GameInstance_C|GetTop%20Down%20Controller _asbp_game_instance)))
    (CallFunction|SetAltarActive true)
    (CallFunction|SaveIDforPersistentAltarActivation)))

(event Custom|Set%20Altar%20Active
  (params (Active? :type Boolean))
  (bind _output_get (Variables|Default|SetAltar%20Active Active?))
  (if _output_get
    (Rendering|SetVisibility (Variables|Default|GetMain%20Light) false false)
    (Rendering|SetVisibility (Variables|Default|GetCandle%20Light) true false)
    (Components|Activation|SetActive (Variables|Default|GetCandle%20Fire) true false)
    (Variables|/Script/Engine.PrimitiveComponent|SetbGenerateOverlapEvents (Variables|Default|GetDetector) false)
    (Audio|Components|Audio|SetVolumeMultiplier (Variables|Default|GetBlessed%20Altar%20Sound) 0.3 :!class /Script/Engine.AudioComponent)
    (Rendering|Material|SetMaterial (Variables|Default|GetNormal_Cauldron_Normal_Cauldron_Water) 0 "/Game/Materials/MI_ClearWater.MI_ClearWater")
    (Audio|Components|Audio|Stop (Variables|Default|GetTimeline))))

(event EventBeginPlay
  (|CallParentFunction)
  (if (CallFunction|CheckSaveforAltarActivation)
    (CallFunction|SetAltarActive true)
    (else
      (Utilities|FlowControl|Sequence
        (:then_0
          (bind _aswidget_interactable_ui (Utilities|Casting|CastToWidget_InteractableUI (UserInterface|GetWidget (Variables|Default|GetWidget))))
          (EventDispatchers|BindEventtoOnClickedAltarButton _aswidget_interactable_ui (delegate Custom|CustomEvent_0)))))))

(event EventShow/HideWidgetUI
  (params (Show? :type Boolean))
  (|CallParentFunction Show?)
  (if (not (Variables|Default|GetAltar%20Active))
    (Rendering|SetVisibility (Variables|Default|GetMain%20Light) Show? false)
    (if Show?
      (bind _newtrack_0 (Timeline|Timeline Play)
        (:Update
          (Transformation|SetRelativeRotation (Variables|Default|GetNormal_Cauldron_Normal_Cauldron_Water) (Math|Rotator|Lerp(Rotator) "0, 0, 0" "0.000000,360.000000,0.000000" _newtrack_0) false false)))
      (else
        (Timeline|Timeline Stop)))))

(fn ConstructionScript
  (|CallParentFunction)
  (Rendering|SetVisibility (Variables|Default|GetMain%20Light) false false)
  (Rendering|SetVisibility (Variables|Default|GetCandle%20Light) false false))

(fn SaveIDforPersistentAltarActivation
  (bind _asbp_game_instance (Utilities|Casting|CastToBP_GameInstance (Game|GetGameInstance)))
  (Default|AddAltarIDonActivation (Variables|/Game/BP/BP_GameInstance.BP_GameInstance_C|GetSave%20Game%20Instance%20-%20Impersistent _asbp_game_instance) (Utilities|GetObjectName self)))

(fn CheckSaveforAltarActivation
  (bind _asbp_game_instance (Utilities|Casting|CastToBP_GameInstance (Game|GetGameInstance)))
  (bind _id_found_ (Default|IsAltarActivated? (Variables|/Game/BP/BP_GameInstance.BP_GameInstance_C|GetSave%20Game%20Instance%20-%20Impersistent _asbp_game_instance) (Utilities|GetObjectName self)))
  (return _id_found_))