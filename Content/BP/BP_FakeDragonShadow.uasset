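; Actor that fakes a passing dragon's shadow by moving a Paper2D flipbook between two points.
; The flipbook starts invisible with hidden shadow casting off, and StartDragonMovement turns both on.
; A Timeline with play rate set to the inverse of MoveTime lerps it from StartPos to EndPos.
; Finishing turns hidden shadow casting off but leaves visibility unchanged.
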(event Custom|Start%20Dragon%20Movement
  (bind _paperflipbook (Variables|Default|GetPaperFlipbook))
  (Rendering|SetVisibility _paperflipbook true false)
  (Class|PrimitiveComponent|SetCastHiddenShadow _paperflipbook true)
  (Components|Timeline|SetPlayRate (Variables|Default|GetTimeline) (Math|Float|Power (Variables|Default|GetMove%20Time) -1.0))
  (bind _newtrack_0 (Timeline|Timeline PlayFromStart)
    (:Update
      (Transformation|SetWorldLocation (Variables|Default|GetPaperFlipbook) (Math|Vector|Lerp(Vector) (Transformation|GetWorldLocation (Variables|Default|GetStart%20Pos)) (Transformation|GetWorldLocation (Variables|Default|GetEnd%20Pos)) _newtrack_0) false false))
    (:Finished
      (Class|PrimitiveComponent|SetCastHiddenShadow (Variables|Default|GetPaperFlipbook) false))))

(event EventBeginPlay
  (bind _paperflipbook (Variables|Default|GetPaperFlipbook))
  (Rendering|SetVisibility _paperflipbook false false)
  (Class|PrimitiveComponent|SetCastHiddenShadow _paperflipbook false))

(event Collision|EventActorBeginOverlap
  (params (OtherActor :type Actor%20Object%20Reference)))

(event EventTick
  (params (DeltaSeconds :type Float%20%28single-precision%29)))

(fn ConstructionScript)