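; BP_Pickup_RandomDrop_Bandages is a health pickup, apparently a bandage drop derived from a parent pickup Blueprint.
; On pickup, it passes its HealthReward value to the player controller's ApplyHealth and plays a 2D potion pickup sound.
; It then calls the parent's OnPickup, leaving the rest of the pickup behavior to the base class.
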(event EventBeginPlay
  (|CallParentFunction) ; This node is disabled and will not be called.\nDrag off pins to build functionality.
)

(event Collision|EventActorBeginOverlap
  (params (OtherActor :type Actor%20Object%20Reference))
  (|CallParentFunction OtherActor) ; This node is disabled and will not be called.\nDrag off pins to build functionality.
)

(event EventTick
  (params (DeltaSeconds :type Float%20%28single-precision%29))
  (|CallParentFunction DeltaSeconds) ; This node is disabled and will not be called.\nDrag off pins to build functionality.
)

(event EventOnPickup
  (params (Player%20Controller :type BP%20Top%20Down%20Controller%20Object%20Reference))
  (Utilities|FlowControl|Sequence
    (:then_0
      (Default|ApplyHealth Player%20Controller (Variables|Default|GetHealth%20Reward) false false "NewEnumerator0")
      (Audio|PlaySound2D "/Game/Sound/SoundFX/Cue_Pickup_Potion.Cue_Pickup_Potion" 1.0 1.0 0.0 0 0))
    (:then_1
      (|CallParentFunction Player%20Controller))))

(fn ConstructionScript
  (|CallParentFunction))