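; BP_Treasure_Cursed is a treasure chest actor that keeps its collision disabled until it is unlocked.
; BeginPlay turns collision off, and the UnlockChest event clears IsLocked, re-enables collision and prints "UNLOCKED" if the chest is locked.
; If IsLocked is already false, UnlockChest only prints "CHEST IS LOCKED".
; No curse behavior or overlap handling is implemented in this graph.
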(event Custom|Unlock%20Chest
  (if (Variables|Default|GetIs%20Locked)
    (Variables|Default|SetIs%20Locked false)
    (Collision|SetActorEnableCollision true)
    (Development|PrintString "UNLOCKED")
    (else
      (Development|PrintString "CHEST IS LOCKED"))))

(event Collision|EventActorBeginOverlap
  (params (OtherActor :type Actor%20Object%20Reference))
  (|CallParentFunction OtherActor) ; This node is disabled and will not be called.\nDrag off pins to build functionality.
)

(event EventTick
  (params (DeltaSeconds :type Float%20%28single-precision%29))
  (|CallParentFunction DeltaSeconds) ; This node is disabled and will not be called.\nDrag off pins to build functionality.
)

(event EventBeginPlay
  (Collision|SetActorEnableCollision false))

(fn ConstructionScript
  (|CallParentFunction))