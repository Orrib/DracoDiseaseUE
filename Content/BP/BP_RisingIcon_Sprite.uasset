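; Sprite variant of a rising icon actor that fades out partway through its rise and then removes itself.
; When the parent's RiseHalfway event fires, a Fade timeline lerps the Paper2D sprite color from opaque white to fully transparent.
; The timeline play rate is the inverse of FadeTime, so that variable controls the fade duration.
; The actor is destroyed when the fade finishes, and RiseFinished is left empty.
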(event EventBeginPlay
  (|CallParentFunction))

(event EventRiseHalfway
  (|CallParentFunction)
  (Components|Timeline|SetPlayRate (Variables|Default|GetFade) (Math|Float|Power (Variables|Default|GetFade%20Time) -1.0))
  (bind _newtrack_0 (Timeline|Fade PlayFromStart)
    (:Update
      (Sprite|SetSpriteColor (Variables|Default|GetPaperSprite) (Math|Color|Lerp(LinearColor) "(R=1.000000,G=1.000000,B=1.000000,A=1.000000)" "(R=1.000000,G=1.000000,B=1.000000,A=0.000000)" _newtrack_0)))
    (:Finished
      (Actor|DestroyActor))))

(event EventRiseFinished)

(fn ConstructionScript
  (|CallParentFunction))