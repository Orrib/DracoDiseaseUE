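; Shockwave actor that expands a cylinder on spawn, damaging player-tagged actors it overlaps, then destroys itself.
; The Shock timeline scales the cylinder, then fires a radial impulse and starts the Fade timeline, which drives opacity and disables collision.
; Both timelines derive play rate from inverse durations.
; Overlaps apply directional point damage with a hit sound; npc, box and wild damage branches are disconnected.
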(event EventBeginPlay
  ;[1 1 1] convert time to play rate
  (Components|Timeline|SetPlayRate (Variables|Default|GetShock) (Math|Float|Power (Variables|Default|GetShock%20Time) -1.0))
  (bind _newtrack_0 (Timeline|Shock PlayFromStart)
    (:Update
      (Transformation|SetRelativeScale3D (Variables|Default|GetCylinder%20Origin) (Math|Conversions|ToVector(Float) (Math|Float|MakeLiteralFloat _newtrack_0))))
    (:Finished
      ;[1 1 1] Physics Impulse
      (Class|RadialForceComponent|FireImpulse (Variables|Default|GetRadialForce))
      ;[1 1 1] convert time to play rate
      (Components|Timeline|SetPlayRate (Variables|Default|GetFade) (Math|Float|Power (Variables|Default|GetFade%20Time) -1.0))
      (bind _newtrack_0_2 (Timeline|Fade PlayFromStart)
        (:Update
          (Rendering|Material|SetScalarParameterValueonMaterials (Variables|Default|GetCylinder) "Opacity" _newtrack_0_2))
        (:Finished
          (Actor|DestroyActor))
        (:Collision%20Disabled
          (Collision|SetActorEnableCollision false))))))

(event Collision|EventActorBeginOverlap
  (params (OtherActor :type Actor%20Object%20Reference))
  (bind _returnvalue (Transformation|GetActorLocation OtherActor))
  (bind _cylinder_origin (Variables|Default|GetCylinder%20Origin))
  (bind _returnvalue_2 (Transformation|GetWorldLocation _cylinder_origin))
  (if (Actor|ActorHasTag OtherActor "player")
    ;[1 1 1] npc
    (Audio|PlaySound2D "/Game/Sound/SoundFX/Cue_Sword_Hit.Cue_Sword_Hit" 1.0 1.0 0.0 0 0 false)
    (Game|Damage|ApplyPointDamage OtherActor (Variables|Default|GetDamage) (Math|Vector|GetUnitDirection(Vector) _returnvalue_2 _returnvalue) (Collision|MakeHitResult false false 0.0 0.0 _returnvalue_2 _returnvalue "0,0,1" "0,0,1" 0 0) 0 self)))

(event EventTick
  (params (DeltaSeconds :type Float%20%28single-precision%29)))

(fn ConstructionScript)