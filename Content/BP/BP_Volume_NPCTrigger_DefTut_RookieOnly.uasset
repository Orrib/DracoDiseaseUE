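; A trigger volume for the defense tutorial that registers rookie ally soldier NPCs as they enter it.
; Each new rookie is added once to a Chapter 1 Part 3 list on the game controller, cached from the game instance shortly after BeginPlay, before the parent overlap logic runs.
; An event toggles a flash highlight, showing a cylinder whose material opacity is driven by a timeline, or stopping and hiding it.
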(event Custom|Enable/Disable%20Flash%20Effect
  (params (Enable? :type Boolean))
  (bind _cylinder (Variables|Default|GetCylinder))
  (if Enable?
    (Development|SetHiddeninGame _cylinder false false)
    (bind _newtrack_0 (Timeline|Flash%20Opacity PlayFromStart)
      (:Update
        (Rendering|Material|SetScalarParameterValueonMaterials (Variables|Default|GetCylinder) "Opacity" _newtrack_0)))
    (else
      (Audio|Components|Audio|Stop (Variables|Default|GetFlash%20Opacity))
      (Development|SetHiddeninGame _cylinder true false))))

(event EventBeginPlay
  (|CallParentFunction)
  (Utilities|FlowControl|Delay 0.2)
  (bind _asbp_game_instance (Utilities|Casting|CastToBP_GameInstance (Game|GetGameInstance)))
  (Variables|Default|SetGame%20Controller (Variables|/Game/BP/BP_GameInstance.BP_GameInstance_C|GetGame%20Controller _asbp_game_instance)))

(event Collision|EventActorBeginOverlap
  (params (OtherActor :type Actor%20Object%20Reference))
  (bind _game_controller (Variables|Default|GetGame%20Controller))
  (bind _chap_1_part_3___rookie_soldiers_who_entered_trigger (Variables|/Game/BP/BP_GameController.BP_GameController_C|GetChap%201%20Part%203%20-%20Rookie%20Soldiers%20who%20entered%20trigger _game_controller))
  (bind _asbp_npc_kingdom_ally_basic_soldier_defense_tut_rookie (Utilities|Casting|CastToBP_NPC_KingdomAlly_BasicSoldier_DefenseTutRookie OtherActor))
  (if (not (Utilities|Array|ContainsItem _chap_1_part_3___rookie_soldiers_who_entered_trigger _asbp_npc_kingdom_ally_basic_soldier_defense_tut_rookie))
    (Utilities|Array|Add _chap_1_part_3___rookie_soldiers_who_entered_trigger _asbp_npc_kingdom_ally_basic_soldier_defense_tut_rookie)
    (|CallParentFunction OtherActor)))

(event EventTick
  (params (DeltaSeconds :type Float%20%28single-precision%29))
  (|CallParentFunction DeltaSeconds) ; This node is disabled and will not be called.\nDrag off pins to build functionality.
)

(fn ConstructionScript
  (|CallParentFunction))