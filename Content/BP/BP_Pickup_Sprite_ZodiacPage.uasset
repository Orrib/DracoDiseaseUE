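; Collectible zodiac book page pickup, a child sprite pickup whose book sprite is chosen by zodiac type in the construction script.
; On BeginPlay it destroys itself if the game instance has its object name recorded as collected.
; On pickup it registers that name with the game instance, shows a midscreen message with the zodiac's name, page image and progress out of three, plays a sound, then runs parent pickup logic.
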(event EventBeginPlay
  (|CallParentFunction)
  (bind _asbp_game_instance (Utilities|Casting|CastToBP_GameInstance (Game|GetGameInstance)))
  (bind _zodiac_items_picked_up (Default|HasZodiacPickupBeenCollected? _asbp_game_instance (Utilities|GetObjectName self)))
  (if _zodiac_items_picked_up
    (Actor|DestroyActor)))

(event Collision|EventActorBeginOverlap
  (params (OtherActor :type Actor%20Object%20Reference))
  (|CallParentFunction OtherActor) ; This node is disabled and will not be called.\nDrag off pins to build functionality.
)

(event EventTick
  (params (DeltaSeconds :type Float%20%28single-precision%29))
  (|CallParentFunction DeltaSeconds) ; This node is disabled and will not be called.\nDrag off pins to build functionality.
)

(event EventOnPickup
  (params (Player%20Controller :type BP%20Top%20Down%20Controller%20Object%20Reference))
  (bind _zodiac_book_type (Variables|Default|GetZodiac%20Book%20Type))
  (bind _game_instance (Variables|/Game/TopDown/Blueprints/BP_TopDownController.BP_TopDownController_C|GetGame%20Instance Player%20Controller))
  (bind (_zodiac_name _description _zodiac_images) (Default|GetZodiacPickupDetails _game_instance _zodiac_book_type))
  (Utilities|FlowControl|Sequence
    (:then_0
      (Default|CollectZodiacPickup _game_instance _zodiac_book_type (Utilities|GetObjectName self))
      (bind _value (Default|GetZodiacNumPagesPickedUp _game_instance _zodiac_book_type))
      (Default|SetMidscreenMessage-Interactable (Variables|/Game/TopDown/Blueprints/BP_TopDownController.BP_TopDownController_C|GetGame%20Controller Player%20Controller) true (select (== _value 3) "All Pages Found!" (Utilities|String|Append (Utilities|String|ToString(Integer) _value) "/3 Pages")) "NewEnumerator1" (Utilities|Array|Get(acopy) _zodiac_images (- _value 1)) _zodiac_name 3.0)
      (Audio|PlaySound2D "/Game/Sound/SoundFX/Cue_Pickup_Coin.Cue_Pickup_Coin" 1.0 1.0 0.0 0 0 false))
    (:then_1
      (|CallParentFunction Player%20Controller))))

(fn ConstructionScript
  (|CallParentFunction)
  (Rendering|Components|Sprite|SetSprite (Variables|Default|GetPaperSprite) (Utilities|Select :Index (Variables|Default|GetZodiac%20Book%20Type) :NewEnumerator0 "/Game/Art/Pickup/Draco_disease__Elder_God_Zodiac__Book_3_Sprite.Draco_disease__Elder_God_Zodiac__Book_3_Sprite" :NewEnumerator1 "/Game/Art/Pickup/Draco_disease__Elder_God_Zodiac__Book_2_Sprite.Draco_disease__Elder_God_Zodiac__Book_2_Sprite" :NewEnumerator2 "/Game/Art/Pickup/Draco_disease__Elder_God_Zodiac__Book_Sprite.Draco_disease__Elder_God_Zodiac__Book_Sprite")))