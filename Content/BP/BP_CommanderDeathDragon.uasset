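; BP_CommanderDeathDragon is a dragon sprite actor that flies between two points, named for a commander death sequence.
; MoveDragon unhides the actor and plays a timeline from the start at one-third speed.
; Each update lerps DragonSpriteParent's world location from the StartPos component to the EndPos component, without sweep.
; BeginPlay and the construction script are empty, so movement only starts when MoveDragon is called.
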(event Custom|Move%20%20Dragon
  (Rendering|SetActorHiddenInGame false)
  (Components|Timeline|SetPlayRate (Variables|Default|GetTimeline) (Math|Float|Power 3.0 -1.0))
  (bind _newtrack_0 (Timeline|Timeline PlayFromStart)
    (:Update
      (Transformation|SetWorldLocation (Variables|Default|GetDragon%20Sprite%20Parent) (Math|Vector|Lerp(Vector) (Transformation|GetWorldLocation (Variables|Default|GetStart%20Pos)) (Transformation|GetWorldLocation (Variables|Default|GetEnd%20Pos)) _newtrack_0) false false))))

(event EventBeginPlay)

(fn ConstructionScript)