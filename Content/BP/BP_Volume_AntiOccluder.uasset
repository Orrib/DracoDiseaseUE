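; A trigger volume that hides a configured set of actors while the player is inside it, likely to clear occluders from view.
; On begin overlap with an actor tagged "player", it hides every actor in ActorsToHide and optionally disables their collision via DisableCollisionUponHiding.
; On end overlap it unhides them and re-enables collision under the same flag, without remembering their previous state.
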(event EventBeginPlay)

(event Collision|EventActorBeginOverlap
  (params (OtherActor :type Actor%20Object%20Reference))
  (if (Actor|ActorHasTag OtherActor "player")
    (for _array_element (Variables|Default|GetActors%20to%20Hide)
      (Rendering|SetActorHiddenInGame _array_element true)
      (if (Variables|Default|GetDisable%20Collision%20upon%20Hiding)
        (Collision|SetActorEnableCollision _array_element false)))))

(event EventTick
  (params (DeltaSeconds :type Float%20%28single-precision%29)))

(event Collision|EventActorEndOverlap
  (params (OtherActor :type Actor%20Object%20Reference))
  (if (Actor|ActorHasTag OtherActor "player")
    (for _array_element (Variables|Default|GetActors%20to%20Hide)
      (Rendering|SetActorHiddenInGame _array_element false)
      (if (Variables|Default|GetDisable%20Collision%20upon%20Hiding)
        (Collision|SetActorEnableCollision _array_element true)))))

(fn ConstructionScript)