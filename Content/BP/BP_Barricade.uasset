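; BP_Barricade is a barricade actor that hurts and knocks back players and NPCs that hit it.
; On Hit, it checks for the "npc" or "player" tag and applies environmental point damage directed away from its Scene component.
; Character victims are then launched along that direction, overriding their velocity, at a speed inversely proportional to their movement component's mass.
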(event EventBeginPlay)

(event Collision|EventActorBeginOverlap
  (params (OtherActor :type Actor%20Object%20Reference)))

(event EventTick
  (params (DeltaSeconds :type Float%20%28single-precision%29)))

(event Collision|EventHit
  (params (MyComp :type Primitive%20Component%20Object%20Reference) (Other :type Actor%20Object%20Reference) (OtherComp :type Primitive%20Component%20Object%20Reference) (bSelfMoved :type Boolean) (HitLocation :type Vector :default "0, 0, 0") (HitNormal :type Vector :default "0, 0, 0") (NormalImpulse :type Vector :default "0, 0, 0") (Hit :type Hit%20Result%20Structure%20%28by%20ref%29))
  (bind _returnvalue (Transformation|GetActorLocation Other))
  (bind _scene (Variables|Default|GetScene))
  (bind _returnvalue_2 (Transformation|GetWorldLocation _scene))
  (bind _returnvalue_3 (Math|Vector|GetUnitDirection(Vector) _returnvalue_2 _returnvalue))
  (if (or (Actor|ActorHasTag Other "npc") (Actor|ActorHasTag Other "player"))
    (Game|Damage|ApplyPointDamage Other (Variables|Default|GetDamage) _returnvalue_3 (Collision|MakeHitResult false false 0.0 0.0 "0, 0, 0" "0, 0, 0" "0,0,1" "0,0,1" 0 0) 0 self "/Engine/EngineDamageTypes/DmgTypeBP_Environmental.DmgTypeBP_Environmental_C")
    (bind _ascharacter (Utilities|Casting|CastToCharacter Other))
    ;[1 1 1] Apply Impulse, accountinmg for mass
    (Character|LaunchCharacter _ascharacter (* _returnvalue_3 (/ 5e+04 (Variables|/Script/Engine.CharacterMovementComponent|GetMass (Variables|/Script/Engine.Character|GetCharacterMovement _ascharacter)))) true true)))

(fn ConstructionScript)