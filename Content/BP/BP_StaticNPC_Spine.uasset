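; Static NPC actor rendered with a Spine skeleton, with a toggle for which way it faces.
; The construction script mirrors the SpineSkeletonRenderer by negating its relative X scale when the face-left flag is set, so facing is resolved at construction.
; The event graph holds only disabled default events, so the Blueprint adds no runtime logic of its own.
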(event EventBeginPlay
  (|CallParentFunction) ; This node is disabled and will not be called.\nDrag off pins to build functionality.
)

(event Collision|EventActorBeginOverlap
  (params (OtherActor :type Actor%20Object%20Reference))
  (|CallParentFunction OtherActor) ; This node is disabled and will not be called.\nDrag off pins to build functionality.
)

(event EventTick
  (params (DeltaSeconds :type Float%20%28single-precision%29))
  (|CallParentFunction DeltaSeconds) ; This node is disabled and will not be called.\nDrag off pins to build functionality.
)

(fn ConstructionScript
  (bind _spineskeletonrenderer (Variables|Default|GetSpineSkeletonRenderer))
  (bind _relativescale3d (Variables|/Script/Engine.SceneComponent|GetRelativeScale3D _spineskeletonrenderer))
  (|CallParentFunction)
  (if (Variables|Default|GetFace%20Left%20%28T/F%20=%20Left/Right%29)
    (Transformation|SetRelativeScale3D _spineskeletonrenderer (Math|Vector|MakeVector (* (.x _relativescale3d) -1.0) (.y _relativescale3d) (.z _relativescale3d)))))