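; BP_Box is a damageable crate that flashes on each hit and breaks apart at zero health, with a chance to drop a coin.
; An intact Cube and a hidden Geometry Collection swap visibility, physics and collision on death.
; The collection is then crumbled, launched upward by an impulse and, after a delay, shrunk by a timeline before the actor is destroyed.
; Hit flashes temporarily swap materials through a retriggerable delay.
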(event Custom|Damage%20Flash
  (bind _cube (Variables|Default|GetCube))
  (Rendering|Material|SetMaterial _cube 0 "/Game/Materials/M_Basic.M_Basic")
  (Utilities|FlowControl|RetriggerableDelay 0.2)
  (Rendering|Material|SetMaterial _cube 0 (Variables|Default|GetOrig%20Material)))

(event Custom|Enable/Disable%20Destructible
  (params (Enable? :type Boolean))
  (bind _returnvalue (not Enable?))
  (bind _bp_box_geometrycollection (Variables|Default|GetBP_Box_GeometryCollection))
  (bind _cube (Variables|Default|GetCube))
  (Rendering|SetVisibility _cube _returnvalue false)
  (Physics|SetSimulatePhysics _cube _returnvalue)
  (Collision|SetCollisionEnabled _cube (select Enable? "NoCollision" "QueryAndPhysics"))
  (Variables|/Script/GeometryCollectionEngine.GeometryCollectionComponent|SetObjectType _bp_box_geometrycollection (select Enable? "Chaos_Object_Dynamic" "Chaos_Object_Kinematic"))
  (Rendering|SetVisibility _bp_box_geometrycollection Enable? false)
  (Physics|SetSimulatePhysics _bp_box_geometrycollection Enable?)
  (Collision|SetCollisionEnabled _bp_box_geometrycollection (select Enable? "QueryAndPhysics" "NoCollision")))

(event EventBeginPlay
  (Variables|Default|SetOrig%20Material (Rendering|Material|GetMaterial (Variables|Default|GetCube) 0))
  (CallFunction|Enable/DisableDestructible false))

(event Game|Damage|EventAnyDamage
  (params (Damage :type Float%20%28single-precision%29) (DamageType :type Damage%20Type%20Object%20Reference) (InstigatedBy :type Controller%20Object%20Reference) (DamageCauser :type Actor%20Object%20Reference))
  (bind _bp_box_geometrycollection (Variables|Default|GetBP_Box_GeometryCollection))
  (bind _bp_box_geometrycollection_2 (Variables|Default|GetBP_Box_GeometryCollection))
  (bind _output_get (Variables|Default|SetHealth (- (Variables|Default|GetHealth) Damage)))
  (if (<= _output_get 0.0)
    (Utilities|FlowControl|Sequence
      (:then_0
        (CallFunction|DamageFlash :!label _label))
      (:then_1
        (Variables|Actor|SetbCanBeDamaged false)
        (CallFunction|Enable/DisableDestructible true)
        (Class|GeometryCollectionComponent|CrumbleCluster _bp_box_geometrycollection)
        (Physics|AddImpulseatLocation _bp_box_geometrycollection "0.000000,0.000000,700000.000000" (Transformation|GetWorldLocation (Variables|Default|GetCube)) "None")
        ;[1 1 1] spawn coin
        (Audio|PlaySound2D "/Game/Sound/SoundFX/Cue_Sword_Hit_Gore.Cue_Sword_Hit_Gore" 1.0 1.3 0.0 0 0)
        (if (Math|Random|RandomBoolwithWeight 0.6)
          (Game|SpawnActorfromClass "/Game/BP/BP_Coin.BP_Coin_C" (Math|Transform|MakeTransform (Transformation|GetActorLocation) "0, 0, 0" "1.000000,1.000000,1.000000") "AdjustIfPossibleButAlwaysSpawn" "MultiplyWithRoot" 0 false 1.0 0))
        (Utilities|FlowControl|Delay 2.0)
        (Variables|Default|SetOrig%20SCale (Variables|/Script/Engine.SceneComponent|GetRelativeScale3D _bp_box_geometrycollection_2))
        (bind _newtrack_0 (Timeline|Fade%20Destructable PlayFromStart)
          (:Update
            (Transformation|SetRelativeScale3D _bp_box_geometrycollection_2 (Math|Vector|Lerp(Vector) (Variables|Default|GetOrig%20SCale) "0, 0, 0" _newtrack_0)))
          (:Finished
            (Actor|DestroyActor)))))
    (else
      (goto _label))))

(fn ConstructionScript)