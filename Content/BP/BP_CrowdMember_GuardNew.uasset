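; BP_CrowdMember_GuardNew is a guard crowd-member actor drawn with a Spine skeleton renderer.
; After the parent construction script runs, the FaceLeftOrRightLTFF flag mirrors the character by negating the renderer's relative X scale.
; The event graph holds only disabled default events, so the Blueprint adds no runtime logic of its own.
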(event EventBeginPlay
  (|CallParentFunction) ; This node is disabled and will not be called.\nDrag off pins to build functionality.
)

(event Collision|EventActorBeginOverlap
  (params (OtherActor :type Actor%20Object%20Reference))
  (|CallParentFunction OtherActor) ; This node is disabled and will not be called.\nDrag off pins to build functionality.
)

(event EventTick
  (params (DeltaSeconds :type Float%20%28single-precision%29))
  (|CallParentFunction DeltaSeconds) ; This node is disabled and will not be called.\nDrag off pins to build functionality.
)

(fn ConstructionScript
  (bind _spineskeletonrenderer_0 (Variables|Default|GetSpineSkeletonRenderer_0))
  (bind _relativescale3d (Variables|/Script/Engine.SceneComponent|GetRelativeScale3D _spineskeletonrenderer_0))
  (|CallParentFunction)
  (if (Variables|Default|GetFace%20Left%20or%20Right%20%28L=T,%20F=F%29)
    (Transformation|SetRelativeScale3D _spineskeletonrenderer_0 (Math|Vector|MakeVector (* (.x _relativescale3d) -1.0) (.y _relativescale3d) (.z _relativescale3d)))))