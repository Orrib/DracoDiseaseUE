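; BP_Boulder is a placeable boulder that picks its rock variant through a child actor component.
; The construction script sets the child class from BoulderClasses, either at random when the index is -1 or at the given index.
; It then applies the collision setting to the spawned child and optionally randomizes its yaw, keeping pitch and roll.
; All logic runs at construction, as the event graph is empty.
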(event EventBeginPlay)

(event Collision|EventActorBeginOverlap
  (params (OtherActor :type Actor%20Object%20Reference)))

(event EventTick
  (params (DeltaSeconds :type Float%20%28single-precision%29)))

(fn ConstructionScript
  (bind _boulder_classes (Variables|Default|GetBoulder%20Classes))
  (bind _boulder_num__random_if__1_ (Variables|Default|GetBoulder%20Num%20%28Random%20if%20-1%29))
  (bind _childactor (Variables|Default|GetChildActor))
  (bind _childactor_2 (Variables|/Script/Engine.ChildActorComponent|GetChildActor _childactor))
  (bind _returnvalue (Transformation|GetActorRotation _childactor_2))
  (ChildActorComponent|SetChildActorClass (Variables|Default|GetChildActor) (select (== _boulder_num__random_if__1_ -1) (.OutItem (Utilities|Array|Random _boulder_classes)) (Utilities|Array|Get(acopy) _boulder_classes _boulder_num__random_if__1_)))
  (Collision|SetActorEnableCollision _childactor_2 (Variables|Default|GetCollision%20Enabled))
  (if (Variables|Default|GetRandom%20Z%20Rotation)
    (Transformation|SetActorRotation _childactor_2 (Math|Rotator|MakeRotator (.roll _returnvalue) (.pitch _returnvalue) (Math|Random|RandomFloatinRange 0.0 3.6e+02)))))