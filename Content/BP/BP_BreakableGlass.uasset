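; BP_BreakableGlass is a breakable actor whose Geometry Collection shatters when it takes any damage.
; The collection starts hidden, kinematic and collisionless, and Break switches it to a simulated dynamic Chaos object.
; Break crumbles its clusters and applies an impulse at the ImpulseOrigin component's location.
; After a delay, a timeline shrinks the debris to zero scale, then destroys the actor.
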(event Custom|Enable/Disable%20Destructible
  (params (Enable? :type Boolean))
  (bind _bp_box_geometrycollection (Variables|Default|GetBP_Box_GeometryCollection))
  (Development|SetHiddeninGame _bp_box_geometrycollection (not Enable?) false)
  (Variables|/Script/GeometryCollectionEngine.GeometryCollectionComponent|SetObjectType _bp_box_geometrycollection (select Enable? "Chaos_Object_Dynamic" "Chaos_Object_Kinematic"))
  (Physics|SetSimulatePhysics _bp_box_geometrycollection Enable?)
  (Collision|SetCollisionEnabled _bp_box_geometrycollection (select Enable? "QueryAndPhysics" "NoCollision")))

(event Custom|Break
  (bind _bp_box_geometrycollection (Variables|Default|GetBP_Box_GeometryCollection))
  (bind _bp_box_geometrycollection_2 (Variables|Default|GetBP_Box_GeometryCollection))
  (CallFunction|Enable/DisableDestructible true)
  (Class|GeometryCollectionComponent|CrumbleCluster _bp_box_geometrycollection)
  (Class|GeometryCollectionComponent|CrumbleCluster _bp_box_geometrycollection 1)
  (Class|GeometryCollectionComponent|CrumbleActiveClusters _bp_box_geometrycollection)
  (Physics|AddImpulseatLocation _bp_box_geometrycollection (Variables|Default|GetImpulse) (Transformation|GetWorldLocation (Variables|Default|GetImpulse%20Origin)) "None")
  (Utilities|FlowControl|Delay 4.0)
  (Variables|Default|SetOrig%20SCale (Variables|/Script/Engine.SceneComponent|GetRelativeScale3D _bp_box_geometrycollection_2))
  (bind _newtrack_0 (Timeline|Fade%20Destructable PlayFromStart)
    (:Update
      (Transformation|SetRelativeScale3D _bp_box_geometrycollection_2 (Math|Vector|Lerp(Vector) (Variables|Default|GetOrig%20SCale) "0, 0, 0" _newtrack_0)))
    (:Finished
      (Actor|DestroyActor))))

(event EventBeginPlay
  (CallFunction|Enable/DisableDestructible false))

(event Game|Damage|EventAnyDamage
  (params (Damage :type Float%20%28single-precision%29) (DamageType :type Damage%20Type%20Object%20Reference) (InstigatedBy :type Controller%20Object%20Reference) (DamageCauser :type Actor%20Object%20Reference))
  (CallFunction|Break))

(fn ConstructionScript)