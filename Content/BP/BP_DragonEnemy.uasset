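; BP_DragonEnemy is a flying PaperZD dragon enemy with swoop attacks, driven by BP_DragonController.
; BeginPlay links the controller to the animation instance, while Tick keeps the sprite upright and mirrors it by movement direction.
; Overlap detectors report players and certain-allegiance NPCs to the controller, and swoops damage players or destroy those NPCs, tracking hit actors.
; Damage flashes the sprite and triggers limited coin drops; death spawns giant meat.
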(event OnComponentBeginOverlap(Detector-Flying)
  (params (OverlappedComponent :type Primitive%20Component%20Object%20Reference) (OtherActor :type Actor%20Object%20Reference) (OtherComp :type Primitive%20Component%20Object%20Reference) (OtherBodyIndex :type Integer) (bFromSweep :type Boolean) (SweepResult :type Hit%20Result%20Structure%20%28by%20ref%29))
  (bind _dragon_controller (Variables|Default|GetDragon%20Controller))
  (if (Actor|ActorHasTag OtherActor "player")
    (Utilities|IsValid (Variables|Default|GetABP%20Dragon%20Undead) :!label _label
      (:Is%20Valid
        _)
      (:Is%20Not%20Valid
        (Utilities|FlowControl|DelayUntilNextTick)))
    (if (not (Utilities|Time|IsValidTimerHandle (Variables|/Game/BP/BP_DragonController.BP_DragonController_C|GetSwoop%20Rest%20Timer _dragon_controller)))
      (Default|OnEnemySpotted _dragon_controller OtherActor))
    (elif (Actor|ActorHasTag OtherActor "npc")
      (bind _asbp_npc (Utilities|Casting|CastToBP_NPC OtherActor))
      (if (Utilities|Enum|Equal(Enum) (Variables|/Game/TopDown/Blueprints/BP_NPC.BP_NPC_C|GetAllegiance _asbp_npc) "NewEnumerator1")
        (goto _label)))))

(event OnComponentBeginOverlap(AttackDetector)
  (params (OverlappedComponent :type Primitive%20Component%20Object%20Reference) (OtherActor :type Actor%20Object%20Reference) (OtherComp :type Primitive%20Component%20Object%20Reference) (OtherBodyIndex :type Integer) (bFromSweep :type Boolean) (SweepResult :type Hit%20Result%20Structure%20%28by%20ref%29))
  (bind _swoop_hit_actors (Variables|Default|GetSwoop%20Hit%20Actors))
  (if (Utilities|Enum|Equal(Enum) (Variables|/Game/BP/BP_DragonController.BP_DragonController_C|GetDragon%20Mode (Variables|Default|GetDragon%20Controller)) "NewEnumerator1")
    ;[1 1 1] Prevent the same actors from being hit twice by swoop
    (if (not (Utilities|Array|ContainsItem (Variables|Default|GetSwoop%20Hit%20Actors) OtherActor))
      (if (Actor|ActorHasTag OtherActor "player")
        (Game|Damage|ApplyDamage OtherActor (Variables|Default|GetDamage) (Variables|Default|GetDragon%20Controller) self)
        (Utilities|Array|AddUnique _swoop_hit_actors OtherActor)
        (elif (Actor|ActorHasTag OtherActor "npc")
          (bind _asbp_npc (Utilities|Casting|CastToBP_NPC OtherActor))
          (if (Utilities|Enum|Equal(Enum) (Variables|/Game/TopDown/Blueprints/BP_NPC.BP_NPC_C|GetAllegiance _asbp_npc) "NewEnumerator1")
            (Utilities|Array|AddUnique _swoop_hit_actors _asbp_npc)
            (Actor|DestroyActor _asbp_npc)))))))

(event Custom|Damage%20Flash
  (bind _paperflipbook (Variables|Default|GetPaperFlipbook))
  ;[1 1 1] damage
  (Sprite|SetSpriteColor _paperflipbook "(R=0.392157,G=0.000000,B=0.000000,A=0.427451)")
  (Utilities|FlowControl|RetriggerableDelay 0.2)
  (Sprite|SetSpriteColor _paperflipbook (Variables|Default|GetOrig%20Color)))

(event Custom|Die
  ;[1 1 1] damage
  (Audio|PlaySound2D "/Game/Sound/SoundFX/Cue_Death.Cue_Death" 1.5 0.5 0.0 0 0 false)
  (Game|SpawnActorfromClass "/Game/BP/BP_Meat_Giant.BP_Meat_Giant_C" (Math|Transform|MakeTransform (Transformation|GetWorldLocation (Variables|Default|GetMeat%20Spawn)) "0, 0, 0" "1.000000,1.000000,1.000000") "AdjustIfPossibleButAlwaysSpawn" "MultiplyWithRoot" 0 true 0.5 0)
  (Actor|DestroyActor))

(event EventBeginPlay
  (bind _asbp_dragon_controller (Utilities|Casting|CastToBP_DragonController (Pawn|GetController)))
  (bind _output_get (Variables|Default|SetDragon%20Controller _asbp_dragon_controller))
  (bind _asabp_dragon_undead (Utilities|Casting|CastToABP_DragonUndead (Variables|/Script/PaperZD.PaperZDAnimationComponent|GetAnimInstance (Variables|Default|GetPaperZDAnimation))))
  (bind _output_get_2 (Variables|Default|SetABP%20Dragon%20Undead _asabp_dragon_undead))
  (Variables|/Game/Animation/ABP_DragonUndead.ABP_DragonUndead_C|SetCharacter%20Movement _output_get_2 (Variables|Character|GetCharacterMovement))
  (Variables|/Game/Animation/ABP_DragonUndead.ABP_DragonUndead_C|SetDragon%20Controller _output_get_2 _output_get)
  (Variables|Default|SetOrig%20Color (Class|PaperFlipbookComponent|GetSpriteColor (Variables|Default|GetPaperFlipbook))))

(event Game|Damage|EventAnyDamage
  (params (Damage :type Float%20%28single-precision%29) (DamageType :type Damage%20Type%20Object%20Reference) (InstigatedBy :type Controller%20Object%20Reference) (DamageCauser :type Actor%20Object%20Reference))
  (bind _returnvalue (Transformation|GetActorLocation))
  ;[1 1 1] damage
  (bind _output_get (Variables|Default|SetHealth (- (Variables|Default|GetHealth) Damage)))
  (if (<= _output_get 0.0)
    (CallFunction|Die)
    (else
      (Utilities|FlowControl|Sequence
        (:then_0
          ;;[1 1 1] Drop coins when hit (max 5)
          (Utilities|FlowControl|DoN 4
            (:Exit
              (Game|SpawnActorfromClass "/Game/BP/BP_Coin.BP_Coin_C" (Math|Transform|MakeTransform _returnvalue "0, 0, 0" "1.000000,1.000000,1.000000") "AdjustIfPossibleButAlwaysSpawn" "MultiplyWithRoot" 0 false 1.0 0)
              (if (Utilities|Enum|Equal(Enum) (Variables|/Game/BP/BP_DragonController.BP_DragonController_C|GetDragon%20Mode (Variables|Default|GetDragon%20Controller)) "NewEnumerator0")
                (Utilities|FlowControl|RetriggerableDelay 0.2)
                (Game|SpawnActorfromClass "/Game/BP/BP_Coin.BP_Coin_C" (Math|Transform|MakeTransform _returnvalue "0, 0, 0" "1.000000,1.000000,1.000000") "AdjustIfPossibleButAlwaysSpawn" "MultiplyWithRoot" 0 false 1.0 0)))))
        (:then_1
          (CallFunction|DamageFlash))))))

(event EventTick
  (params (DeltaSeconds :type Float%20%28single-precision%29))
  (bind _charactermovement (Variables|Character|GetCharacterMovement))
  (bind _sprite_parent (Variables|Default|GetSprite%20Parent))
  (bind _returnvalue (Pawn|Components|CharacterMovement|GetLastUpdateVelocity _charactermovement))
  (bind _relativescale3d (Variables|/Script/Engine.SceneComponent|GetRelativeScale3D _sprite_parent))
  (Transformation|SetWorldRotation (Variables|Default|GetSprite%20Parent) "0.000000,90.000000,0.000000" false false)
  ;[1 1 1] Sprite Flip
  (Transformation|SetRelativeScale3D _sprite_parent (Math|Vector|MakeVector (Math|Float|SelectFloat (* (.y _relativescale3d) -1.0) (.y _relativescale3d) (or (and (> (.y _relativescale3d) 0.0) (< (.y _returnvalue) 0.0)) (and (< (.y _relativescale3d) 0.0) (> (.y _returnvalue) 0.0)))) 1.0 1.0)))

(fn ConstructionScript)