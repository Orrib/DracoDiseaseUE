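; Physics-driven swinging gate with two doors that plays a creak sound while it moves.
; A hit starts the creak unless its timer is already running, fading audio in from a random start offset.
; A fast looping timer polls both doors' angular velocity, then fades the audio out and clears itself once both are nearly still.
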(event Custom|Start%20Door%20Creak
  (Audio|Components|Audio|FadeIn (Variables|Default|GetAudio) 0.5 1.0 (Math|Random|RandomFloatinRange 0.0 12.0) "Linear" :!class /Script/Engine.AudioComponent)
  (bind _returnvalue (Utilities|Time|SetTimerbyEvent (delegate Custom|Door%20Creak%20Sound%20Check%20Update) 0.03 true))
  (Variables|Default|SetDoor%20Creak%20Sound%20Timer _returnvalue))

(event Custom|Door%20Creak%20Sound%20Check%20Update
  ;[1 1 1] Angular Velocity nearly 0?
  (if (and (Math|Vector|VectorIsNearlyZero (Physics|GetPhysicsAngularVelocityinDegrees (Variables|Default|GetDoor2) "None") 5.0) (Math|Vector|VectorIsNearlyZero (Physics|GetPhysicsAngularVelocityinDegrees (Variables|Default|GetDoor1) "None") 5.0))
    (Audio|Components|Audio|FadeOut (Variables|Default|GetAudio) 0.6 0.0 "Linear" :!class /Script/Engine.AudioComponent)
    (Utilities|Time|ClearandInvalidateTimerbyHandle (Variables|Default|GetDoor%20Creak%20Sound%20Timer))))

(event EventBeginPlay)

(event Collision|EventActorBeginOverlap
  (params (OtherActor :type Actor%20Object%20Reference)))

(event Collision|EventHit
  (params (MyComp :type Primitive%20Component%20Object%20Reference) (Other :type Actor%20Object%20Reference) (OtherComp :type Primitive%20Component%20Object%20Reference) (bSelfMoved :type Boolean) (HitLocation :type Vector :default "0, 0, 0") (HitNormal :type Vector :default "0, 0, 0") (NormalImpulse :type Vector :default "0, 0, 0") (Hit :type Hit%20Result%20Structure%20%28by%20ref%29))
  (if (not (Utilities|Time|IsValidTimerHandle (Variables|Default|GetDoor%20Creak%20Sound%20Timer)))
    (CallFunction|StartDoorCreak)))

(fn ConstructionScript)