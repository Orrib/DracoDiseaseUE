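; Game-state object, named as an impersistent save, that holds the player's item inventory and three quick slots.
; Item max quantity, icon, description and consumable/discardable rules are hardcoded lookups on the item enum.
; Adding raises existing stacks up to their max but inserts new entries unclamped; removing a whole stack also clears its quick slot.
; Quick slots store item enum values despite their "InventoryIndex" names, resolved by searching the inventory array.
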(fn GetInventoryItemMaxQuantity
  (params (Item :type Enum_InventoryItemName%20Enum :default "NewEnumerator0"))
  (return (Utilities|Select :Index Item :NewEnumerator2 0 :NewEnumerator0 5 :NewEnumerator1 2 :NewEnumerator3 0 :NewEnumerator4 0 :NewEnumerator6 0 :NewEnumerator5 0)))

(fn GetInventoryItemImage
  (params (Inventory%20Item :type Enum_InventoryItemName%20Enum :default "NewEnumerator0"))
  (return (Utilities|Select :Index Inventory%20Item :NewEnumerator2 0 :NewEnumerator0 "/Game/Art/Pickup/Draco_disease_Mushroom_pickup_-_cropped.Draco_disease_Mushroom_pickup_-_cropped" :NewEnumerator1 "/Game/Art/Pickup/Draco_disease_Health_potion_pickup_-_cropped.Draco_disease_Health_potion_pickup_-_cropped" :NewEnumerator3 "/Game/Art/Pickup/Draco_disease_Bandage_pickup_-_cropped.Draco_disease_Bandage_pickup_-_cropped" :NewEnumerator4 "/Game/Art/Pickup/pink-fruit_-_cropped.pink-fruit_-_cropped" :NewEnumerator6 "/Game/Art/Pickup/Draco_disease_Mana_crystal.Draco_disease_Mana_crystal" :NewEnumerator5 "/Game/Art/Pickup/Draco_disease_Mana_crystal_red.Draco_disease_Mana_crystal_red")))

(fn IsInventoryItematMaxQuantity?
  (params (Item :type Enum_InventoryItemName%20Enum :default "NewEnumerator0"))
  (bind (_item_in_inventory _struct) (Inventory|GetInventoryItemStruct(copy) Item))
  (if (Utilities|Enum|Equal(Enum) Item "NewEnumerator2")
    _
    (elif _item_in_inventory
      (return _item_in_inventory (>= (.quantity _struct) (Inventory|GetInventoryItemMaxQuantity Item)))
      (else
        _)))
  (return false true))

(fn GetInventoryItemStruct(copy)
  (params (Item :type Enum_InventoryItemName%20Enum :default "NewEnumerator0"))
  (bind _inventory (Variables|Default|GetInventory))
  (for (_ _array_index) _inventory
    (if (not (Utilities|Enum|Equal(Enum) Item "NewEnumerator2"))
      (if (Utilities|Enum|Equal(Enum) (.Item (Utilities|Struct|BreakStruct_InventoryItem (Utilities|Array|Get(acopy) _inventory _array_index))) Item)
        (return true (Utilities|Array|Get(acopy) _inventory _array_index)))))
  (return false ""))

(fn GetQuickSlotInventoryItem
  (params (SLot%20Num%20%281-3%29 :type Integer))
  (bind _quick_slot_1___inventory_index (Variables|Default|GetQuick%20Slot%201%20-%20Inventory%20Index))
  (bind _quick_slot_2___inventory_index (Variables|Default|GetQuick%20Slot%202%20-%20Inventory%20Index))
  (bind _quick_slot_3___inventory_index (Variables|Default|GetQuick%20Slot%203%20-%20Inventory%20Index))
  (bind _returnvalue (Utilities|Select :Index SLot%20Num%20%281-3%29 :Option%200 _quick_slot_1___inventory_index :Option%201 _quick_slot_2___inventory_index :Option%202 _quick_slot_3___inventory_index))
  (bind (_item_in_inventory _struct) (Inventory|GetInventoryItemStruct(copy) _returnvalue))
  (return (and _item_in_inventory (not (Utilities|Enum|Equal(Enum) _returnvalue "NewEnumerator2"))) (.Item (Utilities|Struct|BreakStruct_InventoryItem _struct))))

(fn GetQuickSlotInventoryItemStruct(copy)
  (params (SLot%20Num%20%281-3%29 :type Integer))
  (bind _quick_slot_1___inventory_index (Variables|Default|GetQuick%20Slot%201%20-%20Inventory%20Index))
  (bind _quick_slot_2___inventory_index (Variables|Default|GetQuick%20Slot%202%20-%20Inventory%20Index))
  (bind _quick_slot_3___inventory_index (Variables|Default|GetQuick%20Slot%203%20-%20Inventory%20Index))
  (bind _returnvalue (Utilities|Select :Index SLot%20Num%20%281-3%29 :Option%200 "NewEnumerator2" :Option%201 _quick_slot_1___inventory_index :Option%202 _quick_slot_2___inventory_index :Option%203 _quick_slot_3___inventory_index))
  (bind (_item_in_inventory _struct) (Inventory|GetInventoryItemStruct(copy) _returnvalue))
  (return _item_in_inventory _struct))

(fn AllQuickSlotsFull?
  (return (not (Math|Boolean|ORBoolean (Utilities|Enum|Equal(Enum) (Variables|Default|GetQuick%20Slot%201%20-%20Inventory%20Index) "NewEnumerator2") (Utilities|Enum|Equal(Enum) (Variables|Default|GetQuick%20Slot%202%20-%20Inventory%20Index) "NewEnumerator2") (Utilities|Enum|Equal(Enum) (Variables|Default|GetQuick%20Slot%203%20-%20Inventory%20Index) "NewEnumerator2")))))

(fn GetFirstEmptyQuickSlot
  (if (Utilities|Enum|Equal(Enum) (Variables|Default|GetQuick%20Slot%201%20-%20Inventory%20Index) "NewEnumerator2")
    (return 1 true)
    (elif (Utilities|Enum|Equal(Enum) (Variables|Default|GetQuick%20Slot%202%20-%20Inventory%20Index) "NewEnumerator2")
      (return 2 true)
      (elif (Utilities|Enum|Equal(Enum) (Variables|Default|GetQuick%20Slot%203%20-%20Inventory%20Index) "NewEnumerator2")
        (return 3 true)
        (else
          (return 0 false))))))

(fn IsIteminAQuickSlot?
  (params (Item :type Enum_InventoryItemName%20Enum :default "NewEnumerator2"))
  (if (Utilities|Enum|Equal(Enum) Item (Variables|Default|GetQuick%20Slot%201%20-%20Inventory%20Index))
    (return true 1)
    (elif (Utilities|Enum|Equal(Enum) (Variables|Default|GetQuick%20Slot%202%20-%20Inventory%20Index) Item)
      (return true 2)
      (elif (Utilities|Enum|Equal(Enum) (Variables|Default|GetQuick%20Slot%203%20-%20Inventory%20Index) Item)
        (return true 3)
        (else
          (return false 0))))))

(fn RemoveInventoryItem
  (params (Item :type Enum_InventoryItemName%20Enum :default "NewEnumerator0") (Quantity%20to%20Remove :type Integer))
  (bind _inventory (Variables|Default|GetInventory))
  (if (== Quantity%20to%20Remove 0)
    (Development|PrintString 0 "Error: Removing 0 Items from Inventory" true true "(R=1.000000,G=0.000000,B=0.000000,A=1.000000)" 3e+01)
    (else
      (for (_array_element _array_index) _inventory
        (if (Utilities|Enum|Equal(Enum) (.Item (Utilities|Struct|BreakStruct_InventoryItem (Utilities|Array|Get(acopy) _inventory _array_index))) Item)
          (if (>= Quantity%20to%20Remove (.Quantity (Utilities|Struct|BreakStruct_InventoryItem (Utilities|Array|Get(acopy) _inventory _array_index))))
            ;[1 1 1] Remove item from inventory
            (Utilities|Array|RemoveItem _inventory _array_element)
            (Inventory|QuickSlot|RemoveItemfromQuickSlots Item)
            (return)
            (else
              ;[1 1 1] Lower quantity
              (for _index (range 0 (- Quantity%20to%20Remove 1))
                (Math|Integer|DecrementInt (.Quantity (Utilities|Struct|BreakStruct_InventoryItem (Utilities|Array|Get(acopy) _inventory _array_index)))))))))
      (return))))

(fn AddInventoryItem
  (params (Item :type Enum_InventoryItemName%20Enum :default "NewEnumerator0") (Quantity%20to%20Add :type Integer))
  (bind _inventory (Variables|Default|GetInventory))
  (if (== Quantity%20to%20Add 0)
    (Development|PrintString 0 "Error: Adding 0 Items to Inventory" true true "(R=1.000000,G=0.000000,B=0.000000,A=1.000000)" 3e+01)
    (else
      (for (_ _array_index) _inventory
        (if (Utilities|Enum|Equal(Enum) (.Item (Utilities|Struct|BreakStruct_InventoryItem (Utilities|Array|Get(acopy) _inventory _array_index))) Item)
          ;[1 1 1] Raise quantity until max is reached
          (for _index (range 0 (- Quantity%20to%20Add 1))
            (if (not (.at%20max%20quantity (Inventory|IsInventoryItematMaxQuantity? Item)))
              (Math|Integer|IncrementInt (.Quantity (Utilities|Struct|BreakStruct_InventoryItem (Utilities|Array|Get(acopy) _inventory _array_index))))))
          (return)))
      ;[1 1 1] Add to inventory if item is not found
      (Utilities|Array|Add _inventory (Utilities|Struct|MakeStruct_InventoryItem Item Quantity%20to%20Add))
      (return))))

(fn GetInventoryItemDescription
  (params (Inventory%20Item :type Enum_InventoryItemName%20Enum :default "NewEnumerator0"))
  (return (Utilities|Select :Index Inventory%20Item :NewEnumerator2 "..." :NewEnumerator0 "A hearty common Fungi. 
Can be found just about anywhere in the world with the right amount of shade and moisture." :NewEnumerator1 "A quickly-mixed herbal potion with significant healing properties." :NewEnumerator3 "A hastily stiched band of old cloth, enough to stop any bleeding." :NewEnumerator4 "A mythical fruit with exotic properties. They often take decades to form. Young dragons cannot get enough of them!" :NewEnumerator6 "A rare mineral with powerful magical properties." :NewEnumerator5 "A rare mineral with powerful magical properties. Red crystals are even rarer.")))

(fn SetQuickSlot
  (params (Item :type Enum_InventoryItemName%20Enum :default "NewEnumerator2") (Slot%20Num%20%281-3%29 :type Integer))
  (switch int Slot%20Num%20%281-3%29
    (:1
      (Variables|Default|SetQuick%20Slot%201%20-%20Inventory%20Index Item))
    (:2
      (Variables|Default|SetQuick%20Slot%202%20-%20Inventory%20Index Item))
    (:3
      (Variables|Default|SetQuick%20Slot%203%20-%20Inventory%20Index Item))))

(fn RemoveItemfromQuickSlots
  (params (Item :type Enum_InventoryItemName%20Enum :default "NewEnumerator2"))
  (if (Utilities|Enum|Equal(Enum) Item (Variables|Default|GetQuick%20Slot%201%20-%20Inventory%20Index))
    (Inventory|QuickSlot|SetQuickSlot "NewEnumerator2" 1)
    (elif (Utilities|Enum|Equal(Enum) (Variables|Default|GetQuick%20Slot%202%20-%20Inventory%20Index) Item)
      (Inventory|QuickSlot|SetQuickSlot "NewEnumerator2" 2)
      (elif (Utilities|Enum|Equal(Enum) (Variables|Default|GetQuick%20Slot%203%20-%20Inventory%20Index) Item)
        (Inventory|QuickSlot|SetQuickSlot "NewEnumerator2" 3)))))

(fn AllQuickSlotsEmpty?
  (return (Math|Boolean|ANDBoolean (Utilities|Enum|Equal(Enum) (Variables|Default|GetQuick%20Slot%201%20-%20Inventory%20Index) "NewEnumerator2") (Utilities|Enum|Equal(Enum) (Variables|Default|GetQuick%20Slot%202%20-%20Inventory%20Index) "NewEnumerator2") (Utilities|Enum|Equal(Enum) (Variables|Default|GetQuick%20Slot%203%20-%20Inventory%20Index) "NewEnumerator2"))))

(fn IsInventoryItemConsumable?
  (params (Item :type Enum_InventoryItemName%20Enum :default "NewEnumerator0"))
  (return (not (Math|Boolean|ORBoolean (Utilities|Enum|Equal(Enum) Item "NewEnumerator4") (Utilities|Enum|Equal(Enum) Item "NewEnumerator6") (Utilities|Enum|Equal(Enum) Item "NewEnumerator5")))))

(fn IsInventoryItemDiscardable?
  (params (Item :type Enum_InventoryItemName%20Enum :default "NewEnumerator0"))
  (return (not (Math|Boolean|ORBoolean (Utilities|Enum|Equal(Enum) Item "NewEnumerator4") (Utilities|Enum|Equal(Enum) Item "NewEnumerator6") (Utilities|Enum|Equal(Enum) Item "NewEnumerator5")))))