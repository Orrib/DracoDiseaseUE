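; Guard post defense that holds one assigned NPC as its guard and shows occupancy through its sign material.
; It fills when open via a GameController event, or by right-clicking it in strategy mode with NPCs selected.
; Assignment sets the NPC's guard actor and objective.
; The NPC's killed and objective-revaluation events drive ejection, which clears the post and refreshes the sign.
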(event Custom|NPC%20Attempt%20Assignment
  (params (NPC :type BP%20NPC%20Object%20Reference))
  (Utilities|IsValid (Variables|Default|GetAssigned%20NPC)
    (:Is%20Valid
      (if (not (Utilities|HasAssignedNPC?))
        (if (CallFunction|CanAssignNPC NPC) :!label _label
          (CallFunction|AssignNPCtoGuardPost NPC))))
    (:Is%20Not%20Valid
      (goto _label))))

(event Custom|CustomEvent
  (params (NPC :type BP%20NPC%20Object%20Reference))
  (if (not (and (Utilities|Enum|Equal(Enum) (Variables|/Game/TopDown/Blueprints/BP_NPC.BP_NPC_C|GetPrimary%20Objective NPC) "NewEnumerator11") (== (Variables|/Game/TopDown/Blueprints/BP_NPC.BP_NPC_C|GetActor%20to%20Guard NPC) self)))
    (CallFunction|EjectAssignedNPC)))

(event Custom|Update%20Appearance
  (bind _sign_top (Variables|Default|GetSign%20Top))
  (Utilities|IsValid (Variables|Default|GetAssigned%20NPC)
    (:Is%20Valid
      (if (Utilities|HasAssignedNPC?)
        (Rendering|Material|SetMaterial _sign_top 0 "/Game/Materials/M_Basic_Green_Light.M_Basic_Green_Light")
        (else
          (Rendering|Material|SetMaterial _sign_top 0 "/Game/Materials/TreeBark.TreeBark" :!label _label))))
    (:Is%20Not%20Valid
      (goto _label))))

(event Custom|Assign%20NPC%20to%20Guard%20Post
  (params (NPC :type BP%20NPC%20Object%20Reference))
  (Utilities|FlowControl|Sequence
    (:then_0
      (CallFunction|EjectAssignedNPC))
    (:then_1
      (Variables|/Game/TopDown/Blueprints/BP_NPC.BP_NPC_C|SetActor%20to%20Guard NPC self)
      (Default|RevaluatePrimaryObjective NPC "NewEnumerator11")
      (Variables|Default|SetAssigned%20NPC NPC)
      (CallFunction|UpdateAppearance))
    (:then_2
      (EventDispatchers|BindEventtoOnKilled NPC (delegate Custom|Eject%20Assigned%20NPC))
      (EventDispatchers|BindEventtoOnRevaluatePrimaryObjective NPC (delegate Custom|CustomEvent)))))

(event Custom|Eject%20Assigned%20NPC
  ;[1 1 1] Is there someone currently assigned to this post? Kick them off
  (Utilities|IsValid (Variables|Default|GetAssigned%20NPC)
    (:Is%20Valid
      (if (Utilities|HasAssignedNPC?)
        (EventDispatchers|UnbindEventfromOnKilled (Variables|Default|GetAssigned%20NPC) (delegate Custom|Eject%20Assigned%20NPC))
        (EventDispatchers|UnbindEventfromOnRevaluatePrimaryObjective (Variables|Default|GetAssigned%20NPC) (delegate Custom|CustomEvent))
        (Variables|/Game/TopDown/Blueprints/BP_NPC.BP_NPC_C|SetActor%20to%20Guard (Variables|Default|GetAssigned%20NPC) 0)
        (Default|RevaluatePrimaryObjective (Variables|Default|GetAssigned%20NPC) "NewEnumerator0"))
      (Variables|Default|SetAssigned%20NPC 0))
    (:Is%20Not%20Valid
      _))
  (CallFunction|UpdateAppearance))

(event EventBeginPlay
  (|CallParentFunction)
  (Utilities|FlowControl|DelayUntilNextTick)
  ;[1 1 1] Guard Post Auto Assignment
  (EventDispatchers|BindEventtoGuardPost-AttemptNPCAssignmenttoOpenGuardPost (Variables|/Game/BP/BP_GameInstance.BP_GameInstance_C|GetGame%20Controller (Variables|Default|GetGame%20Instance)) (delegate Custom|NPC%20Attempt%20Assignment)))

(event EventTick
  (params (DeltaSeconds :type Float%20%28single-precision%29))
  ;[1 0 0] Comment
)

(event EventDefense:onRightClickSelectionUI
  (bind _game_instance (Variables|Default|GetGame%20Instance))
  (bind _top_down_controller (Variables|/Game/BP/BP_GameInstance.BP_GameInstance_C|GetTop%20Down%20Controller _game_instance))
  (Default|OnRightClicked (Variables|Default|GetWidget%20Selection%20Icon))
  (bind _at_least_1_selected (Default|HasSelectedNPCs? (Variables|/Game/BP/BP_GameInstance.BP_GameInstance_C|GetGame%20Controller _game_instance)))
  (if _at_least_1_selected
    (Default|AssignSelectedNPCtoGuardPost _top_down_controller self)
    (else
      (Default|Moveto _top_down_controller (Transformation|GetWorldLocation (Variables|Default|GetGuard%20Target%20Pos))))))

(fn ConstructionScript
  (|CallParentFunction))

(fn CanRightClickSelectionUI?
  (return (Variables|/Game/TopDown/Blueprints/BP_TopDownController.BP_TopDownController_C|GetIn%20Strategy%20Mode? (Variables|/Game/BP/BP_GameInstance.BP_GameInstance_C|GetTop%20Down%20Controller (Variables|Default|GetGame%20Instance)))))

(fn Defense:GetSelectionUISubtitleText
  (bind _assigned_npc (Variables|Default|GetAssigned%20NPC))
  (Utilities|IsValid _assigned_npc
    (:Is%20Valid
      (if (Utilities|HasAssignedNPC?)
        (return (Utilities|Text|ToText(String) (Utilities|String|Append (Utilities|String|ToString(Text) (Variables|/Game/TopDown/Blueprints/BP_NPC.BP_NPC_C|GetNPC%20Name _assigned_npc)) " on duty.")))
        (else
          _)))
    (:Is%20Not%20Valid
      _))
  (return ""))

(fn CanAssignNPC
  (params (NPC :type BP%20NPC%20Object%20Reference))
  (bind _primary_objective (Variables|/Game/TopDown/Blueprints/BP_NPC.BP_NPC_C|GetPrimary%20Objective NPC))
  (return (or (Utilities|Enum|Equal(Enum) _primary_objective "NewEnumerator0") (and (Utilities|Enum|Equal(Enum) _primary_objective "NewEnumerator11") (== (Variables|/Game/TopDown/Blueprints/BP_NPC.BP_NPC_C|GetActor%20to%20Guard NPC) self)))))