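; BP_Globe is an actor that spins while an actor tagged "player" overlaps it.
; Begin overlap plays a Timeline that lerps the yaw of Scene1 through a full turn, and end overlap stops it in place.
; BeginPlay sets the Timeline play rate to the inverse of SpinDuration, so that variable controls how long a turn takes.
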(event EventBeginPlay
  (Components|Timeline|SetPlayRate (Variables|Default|GetTimeline) (Math|Float|Power (Variables|Default|GetSpin%20Duration) -1.0)))

(event Collision|EventActorBeginOverlap
  (params (OtherActor :type Actor%20Object%20Reference))
  (if (Actor|ActorHasTag OtherActor "player")
    (bind _newtrack_0 (Timeline|Timeline Play)
      (:Update
        (Transformation|SetRelativeRotation (Variables|Default|GetScene1) (Math|Rotator|MakeRotator 0.0 0.0 (Math|Float|Lerp 0.0 3.6e+02 _newtrack_0)) false false)))))

(event Collision|EventActorEndOverlap
  (params (OtherActor :type Actor%20Object%20Reference))
  (if (Actor|ActorHasTag OtherActor "player")
    (bind _newtrack_0 (Timeline|Timeline Stop)
      (:Update
        (Transformation|SetRelativeRotation (Variables|Default|GetScene1) (Math|Rotator|MakeRotator 0.0 0.0 (Math|Float|Lerp 0.0 3.6e+02 _newtrack_0)) false false)))))

(fn ConstructionScript)