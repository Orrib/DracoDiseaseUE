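; Mountable defense structure that the player can man, or selected NPCs can be sent to in strategy mode.
; A widget "Mount" button mounts the player and shows only while they are nearby, unmounted and outside strategy mode.
; Right-clicking its selection icon sends selected NPCs to mount it, otherwise moves to its enter/exit point.
; A second proximity detector maintains a detected-enemy list, though the enemy tag check is left unconnected.
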(event OnComponentBeginOverlap(PlayerProximityDetector)
  (params (OverlappedComponent :type Primitive%20Component%20Object%20Reference) (OtherActor :type Actor%20Object%20Reference) (OtherComp :type Primitive%20Component%20Object%20Reference) (OtherBodyIndex :type Integer) (bFromSweep :type Boolean) (SweepResult :type Hit%20Result%20Structure%20%28by%20ref%29))
  (if (Actor|ActorHasTag OtherActor "player")
    (Variables|Default|SetPlayer%20Inside true)
    (CallFunction|UpdateDefenseUIInteractability)))

(event OnComponentEndOverlap(PlayerProximityDetector)
  (params (OverlappedComponent :type Primitive%20Component%20Object%20Reference) (OtherActor :type Actor%20Object%20Reference) (OtherComp :type Primitive%20Component%20Object%20Reference) (OtherBodyIndex :type Integer))
  (if (Actor|ActorHasTag OtherActor "player")
    (Variables|Default|SetPlayer%20Inside false)
    (CallFunction|UpdateDefenseUIInteractability)))

(event OnComponentBeginOverlap(EnemyProximityDetector)
  (params (OverlappedComponent :type Primitive%20Component%20Object%20Reference) (OtherActor :type Actor%20Object%20Reference) (OtherComp :type Primitive%20Component%20Object%20Reference) (OtherBodyIndex :type Integer) (bFromSweep :type Boolean) (SweepResult :type Hit%20Result%20Structure%20%28by%20ref%29))
  (if (Utilities|ActorIsEnemy? OtherActor)
    (Utilities|Array|Add (Variables|Default|GetDetected%20Enemies) OtherActor)))

(event OnComponentEndOverlap(EnemyProximityDetector)
  (params (OverlappedComponent :type Primitive%20Component%20Object%20Reference) (OtherActor :type Actor%20Object%20Reference) (OtherComp :type Primitive%20Component%20Object%20Reference) (OtherBodyIndex :type Integer))
  (if (Utilities|ActorIsEnemy? OtherActor)
    (Utilities|Array|RemoveItem (Variables|Default|GetDetected%20Enemies) OtherActor)))

(event Custom|Show/Hide%20Defense%20UI
  (params (Show? :type Boolean))
  (bind _defenseui_component (Variables|Default|GetDefenseUI%20Component))
  (bind _widget_defense_ui (Variables|Default|GetWidget%20Defense%20UI))
  (Rendering|SetVisibility _defenseui_component Show? false)
  (Collision|SetCollisionEnabled _defenseui_component (select Show? "QueryOnly" "NoCollision"))
  (Default|Show/Hide _widget_defense_ui Show?)
  (Default|SetButtonAction _widget_defense_ui "Mount"))

(event Custom|Defense%20Mount/Dismount
  (params (Mount? :type Boolean) (Mounted%20By%20Player? :type Boolean) (%28optional%29%20Mounted%20Pawn :type Pawn%20Object%20Reference))
  (Variables|Default|SetMounted Mount?)
  (Variables|Default|SetPlayer%20Mounted Mounted%20By%20Player?)
  (bind _output_get (Variables|Default|SetMounted%20Pawn %28optional%29%20Mounted%20Pawn))
  (CallFunction|UpdateDefenseUIInteractability)
  (if (not (and Mount? (not Mounted%20By%20Player?)))
    (bind _asbp_npc (Utilities|Casting|CastToBP_NPC _output_get))
    (Default|OnNPCMount/DismountDefense _asbp_npc Mount?)))

(event Custom|CustomEvent
  (CallFunction|DefenseMount/Dismount true true (Variables|/Game/TopDown/Blueprints/BP_TopDownController.BP_TopDownController_C|GetTop%20Down%20Character (Variables|/Game/BP/BP_GameInstance.BP_GameInstance_C|GetTop%20Down%20Controller (Variables|Default|GetGame%20Instance)))))

(event Custom|Update%20Defense%20UI%20Interactability
  (Default|Show/Hide (Variables|Default|GetWidget%20Defense%20UI) (not (Math|Boolean|ORBoolean (Variables|/Game/TopDown/Blueprints/BP_TopDownController.BP_TopDownController_C|GetIn%20Strategy%20Mode? (Variables|/Game/BP/BP_GameInstance.BP_GameInstance_C|GetTop%20Down%20Controller (Variables|Default|GetGame%20Instance))) (Variables|Default|GetPlayer%20Mounted) (not (Variables|Default|GetPlayer%20Inside))))))

(event EventBeginPlay
  (|CallParentFunction)
  (bind _aswidget_defense_ui (Utilities|Casting|CastToWidget_DefenseUI (UserInterface|GetWidget (Variables|Default|GetDefenseUI%20Component))))
  (bind _output_get (Variables|Default|SetWidget%20Defense%20UI _aswidget_defense_ui))
  (EventDispatchers|BindEventtoOnActionButtonPressed _output_get (delegate Custom|CustomEvent)))

(event EventInitialUIRefresh
  (|CallParentFunction)
  (CallFunction|Show/HideDefenseUI true)
  (CallFunction|UpdateDefenseUIInteractability))

(event EventOnEnter/ExitStrategyMode
  (params (Enter? :type Boolean))
  (|CallParentFunction Enter?)
  (CallFunction|UpdateDefenseUIInteractability))

(event EventDefense:onRightClickSelectionUI
  (bind _game_instance (Variables|Default|GetGame%20Instance))
  (bind _top_down_controller (Variables|/Game/BP/BP_GameInstance.BP_GameInstance_C|GetTop%20Down%20Controller _game_instance))
  (Default|OnRightClicked (Variables|Default|GetWidget%20Selection%20Icon))
  (bind _at_least_1_selected (Default|HasSelectedNPCs? (Variables|/Game/BP/BP_GameInstance.BP_GameInstance_C|GetGame%20Controller _game_instance)))
  (if _at_least_1_selected
    (Default|MoveNPCtoMountDefense _top_down_controller self)
    (else
      (Default|Moveto _top_down_controller (Transformation|GetWorldLocation (Variables|Default|GetEnter/Exit%20Position))))))

(fn ConstructionScript
  (|CallParentFunction))

(fn CanRightClickSelectionUI?
  (bind _game_instance (Variables|Default|GetGame%20Instance))
  (if (not (Variables|Default|GetMounted))
    (if (Variables|/Game/TopDown/Blueprints/BP_TopDownController.BP_TopDownController_C|GetIn%20Strategy%20Mode? (Variables|/Game/BP/BP_GameInstance.BP_GameInstance_C|GetTop%20Down%20Controller _game_instance))
      (bind _at_least_1_selected (Default|HasSelectedNPCs? (Variables|/Game/BP/BP_GameInstance.BP_GameInstance_C|GetGame%20Controller _game_instance)))
      (if _at_least_1_selected
        (if (Variables|Default|GetAlly%20Mountable)
          (return true)
          (else
            _))
        (else
          (return true)))))
  (return false))