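; BP_CrowdTrail spawns randomly chosen crowd members at the start of a spline, handing each the spline and a random speed.
; While a tagged player overlaps it, a self-retriggering loop uses a gate and random delay to pace spawns.
; A weighted roll makes some members rushers with scaled speed and a shorter minimum delay.
; Types reroll once to reduce repeats, guards spawn through their own branch, and Y-scale mirroring sets facing.
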(event Custom|Spawn%20Member
  (params (Member%20Type%20New :type Enum_CrowdMember%20Enum :default "NewEnumerator0"))
  (bind _spline (Variables|Default|GetSpline))
  (bind _spline_2 (Variables|Default|GetSpline))
  (bind _crowd_member_faces_right_ (Variables|Default|GetCrowd%20Member%20Faces%20Right?))
  (bind _member_min_speed (Variables|Default|GetMember%20Min%20Speed))
  (bind _member_max_speed (Variables|Default|GetMember%20Max%20Speed))
  (bind _rusher_ (Variables|Default|GetRusher?))
  (bind _rusher_factor (Variables|Default|GetRusher%20Factor))
  (bind _returnvalue (Spline|GetTransformatSplinePoint _spline_2 0 "World" false))
  (bind _returnvalue_2 (Math|Random|RandomFloatinRange _member_min_speed _member_max_speed))
  (bind _returnvalue_3 (select _crowd_member_faces_right_ 1.0 -1.0))
  (bind _returnvalue_4 (* _returnvalue_2 _rusher_factor))
  (bind _returnvalue_5 (select _rusher_ _returnvalue_4 _returnvalue_2))
  (bind _output_get (Variables|Default|SetCrowd%20Member%20Class (Utilities|Select :Index Member%20Type%20New :NewEnumerator0 "/Game/BP/BP_CrowdMember.BP_CrowdMember_C" :NewEnumerator1 "/Game/BP/BP_CrowdMember_ManFarmer.BP_CrowdMember_ManFarmer_C" :NewEnumerator2 "/Game/BP/BP_CrowdMember_Woman.BP_CrowdMember_Woman_C" :NewEnumerator3 "/Game/BP/BP_CrowdMember_WomanBasket.BP_CrowdMember_WomanBasket_C" :NewEnumerator4 "/Game/BP/BP_CrowdMember.BP_CrowdMember_C")))
  ;[1 1 1] Guard?
  (if (Utilities|Enum|Equal(Enum) Member%20Type%20New "NewEnumerator4")
    (bind _returnvalue_6 (Game|SpawnActorfromClass "/Game/BP/BP_CrowdMember_GuardNewer.BP_CrowdMember_GuardNewer_C" (Math|Transform|MakeTransform (.location _returnvalue) "0, 0, 0" "1.000000,1.000000,1.000000") "AlwaysSpawn" "MultiplyWithRoot" 0 _spline _returnvalue_5 _rusher_ 0))
    (Transformation|SetRelativeScale3D (Variables|/Script/Engine.Actor|GetRootComponent _returnvalue_6) (Math|Vector|MakeVector 1.0 _returnvalue_3 1.0))
    (Utilities|FlowControl|Delay 0.2 :!label _label)
    (CallFunction|AttemptSpawnRandomMember)
    (else
      (bind _returnvalue_7 (Game|SpawnActorfromClass _output_get (Math|Transform|MakeTransform (.location _returnvalue) "0, 0, 0" "1.000000,1.000000,1.000000") "AlwaysSpawn" "MultiplyWithRoot" 0 _spline _returnvalue_5 false 0))
      (Utilities|FlowControl|Sequence
        (:then_0
          ;[1 1 1] guard?
          (if (== _output_get "/Game/BP/BP_CrowdMember_GuardNew.BP_CrowdMember_GuardNew_C")
            (Utilities|Casting|CastToBP_CrowdMember_GuardNew _returnvalue_7)))
        (:then_1
          (Transformation|SetRelativeScale3D (Variables|/Game/BP/BP_CrowdMember.BP_CrowdMember_C|GetParent _returnvalue_7) (Math|Vector|MakeVector 1.0 _returnvalue_3 1.0))
          (goto _label))))))

(event Custom|Spawn%20Random%20Member
  (bind _possible_crowd_member_types_new (Variables|Default|GetPossible%20Crowd%20Member%20Types%20New))
  (bind _outitem (Utilities|Array|Random _possible_crowd_member_types_new))
  (bind _output_get (Variables|Default|SetCrowd%20Member%20Type%20New _outitem))
  ;[1 1 1] reroll to avoid repeat members
  (if (Utilities|Enum|Equal(Enum) _output_get (Variables|Default|GetLast%20Crowd%20Member%20Type%20New))
    (Variables|Default|SetCrowd%20Member%20Type%20New _outitem))
  (bind _output_get_2 (Variables|Default|SetLast%20Crowd%20Member%20Type%20New (Variables|Default|GetCrowd%20Member%20Type%20New)))
  (CallFunction|SpawnMember _output_get_2))

(event Custom|Attempt%20Spawn%20Random%20Member
  (Utilities|FlowControl|Sequence
    (:then_0
      (Variables|Default|SetRusher? (Math|Random|RandomBoolwithWeight (Variables|Default|GetChance%20for%20Rusher%20%280-1%29))))
    (:then_1
      (Utilities|FlowControl|Delay (Math|Random|RandomFloatinRange (select (Variables|Default|GetRusher?) 0.1 (Variables|Default|GetMin%20Time%20Between%20Spawns)) (Variables|Default|GetMax%20Time%20Between%20Spawns)))
      (Utilities|FlowControl|Sequence
        (:then_0
          (goto _label Open))
        (:then_1
          _))))
  (Utilities|FlowControl|Gate false :!label _label
    (:Exit
      (if (Variables|Default|GetPlayer%20Near)
        (CallFunction|SpawnRandomMember)
        (goto _label Close)))))

(event Collision|EventActorBeginOverlap
  (params (OtherActor :type Actor%20Object%20Reference))
  (if (Actor|ActorHasTag OtherActor "player")
    (Variables|Default|SetPlayer%20Near true)
    (CallFunction|AttemptSpawnRandomMember)))

(event Collision|EventActorEndOverlap
  (params (OtherActor :type Actor%20Object%20Reference))
  (if (Actor|ActorHasTag OtherActor "player")
    (Variables|Default|SetPlayer%20Near false)))

(fn ConstructionScript)