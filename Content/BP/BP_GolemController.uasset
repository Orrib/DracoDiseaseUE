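; AI controller for the golem, driving its state and a random patrol behaviour.
; It starts in the Rock state a tick after BeginPlay and enables player input so debug key H can switch it to PatrollingRock.
; Patrol moves to a random RockActor patrol point, then repeats after a random delay on success or failure while that state holds.
; An unconnected move-to-rock test with debug prints remains.
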(event Custom|Change%20Golem%20State
  (params (New%20State :type Enum_GolemState%20Enum :default "NewEnumerator0"))
  (bind _output_get (Variables|Default|SetCurrent%20State New%20State))
  (switch Utilities|FlowControl|Switch|SwitchonEnum_GolemState _output_get
    (:NewEnumerator5
      (CallFunction|Patrol))))

(event Custom|Patrol
  (if (Utilities|Enum|Equal(Enum) (Variables|Default|GetCurrent%20State) "NewEnumerator5")
    (AI|AIMoveTo 0 (Transformation|GetWorldLocation (.OutItem (Utilities|Array|Random (Variables|/Game/BP/BP_GolemRock.BP_GolemRock_C|GetPatrol%20Pointss (Variables|Default|GetRock%20Actor))))) 0 5.0 "Default" "Disable" true true true "Enable"
      (:OnRequestFailed
        _)
      (:OnMoveFinished
        _))
    (Utilities|FlowControl|Delay (Math|Random|RandomFloatinRange 1.0 5.0))
    (CallFunction|Patrol)))

(event EventBeginPlay
  (Utilities|FlowControl|DelayUntilNextTick)
  (CallFunction|ChangeGolemState "NewEnumerator0")
  (Input|EnableInput (Game|GetPlayerController 0)))

(event EventTick
  (params (DeltaSeconds :type Float%20%28single-precision%29)))

(event Input|KeyboardEvents|DebugKeyH
  (params (Key :type Key%20Structure :default "None") (ActionValue :type Input%20Action%20Value%20Structure))
  (:Pressed
    (CallFunction|ChangeGolemState "NewEnumerator5")))

(fn ConstructionScript)