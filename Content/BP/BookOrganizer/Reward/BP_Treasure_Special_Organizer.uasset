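; BP_Treasure_Special_Organizer is a special treasure chest pickup for the BookOrganizer reward set that signals a maze goal when opened.
; It extends a parent treasure Blueprint, running the inherited pickup logic first, then calling Goal on MazeMaster if that reference is valid.
; BeginPlay, overlap and Tick are disabled stubs, and the construction script only calls the parent.
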(event EventBeginPlay
  (|CallParentFunction) ; This node is disabled and will not be called.\nDrag off pins to build functionality.
)

(event Collision|EventActorBeginOverlap
  (params (OtherActor :type Actor%20Object%20Reference))
  (|CallParentFunction OtherActor) ; This node is disabled and will not be called.\nDrag off pins to build functionality.
)

(event EventTick
  (params (DeltaSeconds :type Float%20%28single-precision%29))
  (|CallParentFunction DeltaSeconds) ; This node is disabled and will not be called.\nDrag off pins to build functionality.
)

(event EventOnPickup
  (params (Player%20Controller :type BP%20Top%20Down%20Controller%20Object%20Reference))
  (bind _maze_master (Variables|Default|GetMaze%20Master))
  ;[1 1 1] Chest Opens
  (|CallParentFunction Player%20Controller)
  (Utilities|IsValid _maze_master
    (:Is%20Valid
      (Default|Goal _maze_master))))

(fn ConstructionScript
  (|CallParentFunction))