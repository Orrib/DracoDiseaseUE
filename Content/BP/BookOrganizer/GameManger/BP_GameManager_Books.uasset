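; BP_GameManager_Books runs a timed book-organizing challenge that starts when the player overlaps it.
; It validates book placement by index, updates the HUD through a dispatcher, and spawns a treasure when all books are placed in time.
; Tick and a looping timer both track timeout, which fades the screen and teleports the player back.
; A Gate controls the near-finish audio cue, and leaving clears the HUD and timer.
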(event Custom|TickCountdown
  (bind _returnvalue (Utilities|Time|GetTimeSeconds))
  (bind _starttime (Variables|Default|GetStartTime))
  (bind _returnvalue_2 (- _returnvalue _starttime))
  ;[1 1 1] Begin The Book Organizer
  ;;[0.6771 0.6771 0.6771] Begin Countdown
  ;;;[0 0 0] 10.6 secs left
  (Utilities|FlowControl|Sequence
    (:then_0
      ;;;[0.09896 0.09896 0.09896] Timer Hits Zero
      (if (>= _returnvalue_2 (Variables|Default|GetCountdown))
        (CallFunction|ResetEvent)))
    (:then_1
      (if (> _returnvalue_2 (- (Variables|Default|GetCountdown) 10.6))
        (Development|PrintString "destroy yourself now")
        (Utilities|FlowControl|Gate false :!label _label
          (:Exit
            (Audio|Components|Audio|Play (Variables|Default|GetCue_TimerNearingFinish) 0.0)
            (goto _label Close)))))))

(event Custom|TeleportPlayer
  ;[1 1 1] Player Teleport Back To Start
  (Transformation|SetActorLocation (Game|Player|GetPlayerPawn 0) (Transformation|GetActorLocation (Variables|Default|GetOuterPosition)) false true))

(event Custom|ResetEvent
  (bind _cue_timernearingfinish (Variables|Default|GetCue_TimerNearingFinish))
  ;[1 1 1] Reset Event
  (Widget|RemovefromParent (Variables|Default|GetHUDRef))
  ;;[0 0 0] ResetTimer
  (Utilities|Time|ClearandInvalidateTimerbyHandle (Variables|Default|GetTimerHandle_Countdown))
  (Utilities|FlowControl|Sequence
    (:then_0
      (Utilities|IsValid _cue_timernearingfinish
        (:Is%20Valid
          (Audio|Components|Audio|FadeOut _cue_timernearingfinish 1.0 0.0 "SCurve" :!class /Script/Engine.AudioComponent))
        (:Is%20Not%20Valid
          _))
      (Default|CreateScreenFade (Variables|Default|Getgame%20controller) "(R=0.000000,G=0.000000,B=0.000000,A=1.000000)" 0.5 0.5 true 0.5)
      (Utilities|FlowControl|Delay 0.5)
      (CallFunction|TeleportPlayer))
    (:then_1
      ;[1 1 1] Begin The Book Organizer
      ;;[0.6771 0.6771 0.6771] Begin Countdown
      ;;;[0 0 0] 10.6 secs left
      (Utilities|FlowControl|Gate false) ; enters at Open
    )))

(event Custom|LeavingEvent
  (bind _cue_timernearingfinish (Variables|Default|GetCue_TimerNearingFinish))
  (bind _hudref (Variables|Default|GetHUDRef))
  ;[1 1 1] Leaving Event
  (Utilities|IsValid _hudref
    (:Is%20Valid
      (Widget|RemovefromParent _hudref))
    (:Is%20Not%20Valid
      _))
  (Utilities|Time|ClearandInvalidateTimerbyHandle (Variables|Default|GetTimerHandle_Countdown))
  (Utilities|FlowControl|Sequence
    (:then_0
      (Utilities|IsValid _cue_timernearingfinish
        (:Is%20Valid
          (Audio|Components|Audio|FadeOut _cue_timernearingfinish 1.0 0.0 "SCurve" :!class /Script/Engine.AudioComponent))
        (:Is%20Not%20Valid)))
    (:then_1
      ;[1 1 1] Begin The Book Organizer
      ;;[0.6771 0.6771 0.6771] Begin Countdown
      ;;;[0 0 0] 10.6 secs left
      (Utilities|FlowControl|Gate false) ; enters at Open
    )))

(event Custom|OnBooksRemainingChanged_Event
  (params (NewRemaining :type Integer))
  ;[1 1 1] Begin The Book Organizer
  (Default|SetRemaining (Variables|Default|GetHUDRef) NewRemaining))

(event Collision|EventActorEndOverlap
  (params (OtherActor :type Actor%20Object%20Reference))
  ;[1 1 1] Leaving Event
  (if (Actor|ActorHasTag OtherActor "player")
    (CallFunction|LeavingEvent)))

(event EventBeginPlay
  (bind _asbp_game_instance (Utilities|Casting|CastToBP_GameInstance (Game|GetGameInstance)))
  (Variables|Default|Setgame%20controller (Variables|/Game/BP/BP_GameInstance.BP_GameInstance_C|GetGame%20Controller _asbp_game_instance)))

(event EventTick
  (params (DeltaSeconds :type Float%20%28single-precision%29))
  ;[1 1 1] When The Timer Hits 0, Game Over (If the timer hit 0, and the objective hasn't been finished,
  ;  reset and try again.)
  (if (Variables|Default|GetbTimerActive)
    (bind _output_get (Variables|Default|SetTimeRemaining (Math|Float|Max(Float) (- (Variables|Default|GetTimeRemaining) DeltaSeconds) 0.0)))
    (Development|PrintString (Utilities|String|ToString(Float) _output_get) true true "(R=0.000000,G=0.660000,B=1.000000,A=1.000000)" _output_get)
    (Default|CallOnTimerTick (Math|Float|Max(Float) (- (Variables|Default|GetTimeRemaining) DeltaSeconds) 0.0))
    (if (Math|Boolean|ANDBoolean (> (Variables|Default|GetBooksRemaining) 0) (<= (Variables|Default|GetTimeRemaining) 0.0) (not (Variables|Default|GetbGameOverHandled)))
      (CallFunction|ResetEvent))))

(event Collision|EventActorBeginOverlap
  (params (OtherActor :type Actor%20Object%20Reference))
  ;[1 1 1] Begin The Book Organizer
  (if (Actor|ActorHasTag OtherActor "player")
    (if (Utilities|Time|IsValidTimerHandle (Variables|Default|GetTimerHandle_Countdown))
      (CallFunction|ResetEvent))
    (Variables|Default|SetBooksRemaining (Variables|Default|GetTotalBooks))
    (Variables|Default|SetTimeRemaining (Variables|Default|GetStartTime))
    (Variables|Default|SetbTimerActive true)
    (Utilities|IsValid (Variables|Default|GetHUDRef)
      (:Is%20Not%20Valid
        (bind _returnvalue (UserInterface|CreateWidget "/Game/BP/BookOrganizer/WBP_HUD/WBP_HUD.WBP_HUD_C" (Game|GetPlayerController 0) (Variables|Default|GetCountdown)))
        (bind _output_get (Variables|Default|SetHUDRef _returnvalue))
        (UserInterface|Viewport|AddtoViewport _output_get 0)
        (Audio|PlaySound2D "/Game/Sound/SoundFX/Cue_Select.Cue_Select" 0.7 1.15 0.0 0 0)
        (bind _returnvalue_2 (Utilities|Time|SetTimerbyEvent (delegate Custom|TickCountdown) 2e+01 true))
        (Variables|Default|SetTimerHandle_Countdown _returnvalue_2)
        (Utilities|FlowControl|DoOnce false
          (:Completed
            (EventDispatchers|BindEventtoOnBooksRemainingChanged (delegate Custom|OnBooksRemainingChanged_Event))
            (Default|SetRemaining (Variables|Default|GetHUDRef) (Variables|Default|GetBooksRemaining))))))))

(fn ConstructionScript)

(fn ValidatePlacement
  (params (BookTargetIndex :type Integer) (BookCaseIndex :type Integer) (BookRef :type BP%20Book%20Base%20Object%20Reference) (BookcaseRef :type BP%20Book%20Case%20Book%20Object%20Reference))
  (return (and (== BookTargetIndex BookCaseIndex) (not (Variables|/Game/BP/BookOrganizer/Bookbase/BP_BookBase.BP_BookBase_C|GetbPlaced BookRef)))))

(fn RegisterBookPlacedCorrect()
  (Variables|Default|SetBooksRemaining (Math|Integer|Clamp(Integer) (- (Variables|Default|GetBooksRemaining) 1) 0 (Variables|Default|GetTotalBooks)))
  (Default|CallOnBooksRemainingChanged (Variables|Default|GetBooksRemaining))
  (if true
    (if (Math|Boolean|ANDBoolean (== (Variables|Default|GetBooksRemaining) 0) (> (Variables|Default|GetTimeRemaining) 0.0) (not false))
      (Variables|Default|SetbTimerActive false)
      (CallFunction|SpawnReward()))))

(fn SpawnReward()
  (Game|SpawnActorfromClass "/Game/BP/BookOrganizer/Reward/BP_Treasure_Special_Organizer.BP_Treasure_Special_Organizer_C" (Variables|Default|GetRewardSpawnTransform) "Undefined" "MultiplyWithRoot" 0 false 1.0 false true 0))

(fn ResetAllBooks()
  (Utilities|IsValid (Variables|Default|GetHUDRef)
    (:Is%20Valid
      (Default|SetRemaining (Variables|Default|GetHUDRef) (Variables|Default|GetBooksRemaining))
      (bind _outactors (Actor|GetAllActorsOfClass "/Game/BP/BookOrganizer/Bookbase/BP_BookBase.BP_BookBase_C"))
      (for _array_element _outactors
        _)
      (Default|ResetBook() _array_element)
      (Variables|Default|SetBooksRemaining (Variables|Default|GetTotalBooks))
      (Variables|Default|SetTimeRemaining (Variables|Default|GetStartTime))
      (Variables|Default|SetbTimerActive false)
      (Variables|Default|SetbGameOverHandled false)
      (Default|SetRemaining (Variables|Default|GetHUDRef) (Variables|Default|GetBooksRemaining)))))