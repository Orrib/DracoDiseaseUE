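; BP_ZomEyes is an actor for blinking eyes, presumably a zombie's, that either start at BeginPlay or stay hidden until triggered.
; A player-tagged overlap on BoxMid or hit on BoxLower reveals them through a shared DoOnce.
; After a random delay, a timeline scales Parent's Y and Z, its play rate the inverse of a randomized, clamped BlinkTime.
; The construction script enables one trigger box by boolean, overriding its initial StartImmediately-based setup.
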(event OnComponentBeginOverlap(Box-Mid)
  (params (OverlappedComponent :type Primitive%20Component%20Object%20Reference) (OtherActor :type Actor%20Object%20Reference) (OtherComp :type Primitive%20Component%20Object%20Reference) (OtherBodyIndex :type Integer) (bFromSweep :type Boolean) (SweepResult :type Hit%20Result%20Structure%20%28by%20ref%29))
  (if (and (Actor|ActorHasTag OtherActor "player") (not (Audio|Components|Audio|IsPlaying (Variables|Default|GetTimeline))))
    (Utilities|FlowControl|DoOnce false
      (:Completed
        (CallFunction|StartBlinking)))))

(event OnComponentHit(Box-Lower)
  (params (HitComponent :type Primitive%20Component%20Object%20Reference) (OtherActor :type Actor%20Object%20Reference) (OtherComp :type Primitive%20Component%20Object%20Reference) (NormalImpulse :type Vector :default "0, 0, 0") (Hit :type Hit%20Result%20Structure%20%28by%20ref%29))
  (if (and (not (Audio|Components|Audio|IsPlaying (Variables|Default|GetTimeline))) (Actor|ActorHasTag OtherActor "player"))
    (Utilities|FlowControl|DoOnce false
      (:Completed
        (CallFunction|StartBlinking)))))

(event Custom|Start%20Blinking
  (Rendering|SetVisibility (Variables|Default|GetDefaultSceneRoot) true true)
  (Utilities|FlowControl|Delay (Math|Random|RandomFloatinRange 0.0 1.0))
  (Components|Timeline|SetPlayRate (Variables|Default|GetTimeline) (Math|Float|Power (Math|Float|Clamp(Float) (+ (Variables|Default|GetBlink%20Time) (Math|Random|RandomFloatinRange -1.0 2.0)) 0.0 2e+01) -1.0))
  (bind _newtrack_0 (Timeline|Timeline PlayFromStart)
    (:Update
      (Transformation|SetRelativeScale3D (Variables|Default|Getparent) (Math|Vector|MakeVector 1.0 _newtrack_0 _newtrack_0)))))

(event EventBeginPlay
  (if (Variables|Default|GetStart%20Immediately)
    (CallFunction|StartBlinking)
    (else
      (Rendering|SetVisibility (Variables|Default|GetDefaultSceneRoot) false true))))

(event Collision|EventActorBeginOverlap
  (params (OtherActor :type Actor%20Object%20Reference)))

(event EventTick
  (params (DeltaSeconds :type Float%20%28single-precision%29)))

(fn ConstructionScript
  (bind _start_immediately (Variables|Default|GetStart%20Immediately))
  (bind _box___mid (Variables|Default|GetBox%20-%20Mid))
  (bind _box___mid_2 (Variables|Default|GetBox%20-%20Mid))
  (bind _box___lower (Variables|Default|GetBox%20-%20Lower))
  (bind _enable_middle_or_lowqer_triogger__t_f___middlr_lower_ (Variables|Default|GetEnable%20Middle%20or%20Lowqer%20Triogger%20%28T/F%20=%20Middlr/Lower%29))
  (bind _returnvalue (not _start_immediately))
  (Rendering|SetVisibility _box___mid _returnvalue false)
  (Collision|SetCollisionEnabled _box___mid (select _returnvalue "QueryAndPhysics" "NoCollision"))
  (Rendering|SetVisibility _box___lower false false)
  (Collision|SetCollisionEnabled _box___lower "NoCollision")
  (Rendering|SetVisibility (select _enable_middle_or_lowqer_triogger__t_f___middlr_lower_ _box___lower _box___mid_2) true false)
  (Collision|SetCollisionEnabled (select _enable_middle_or_lowqer_triogger__t_f___middlr_lower_ _box___lower _box___mid_2) "QueryAndPhysics"))