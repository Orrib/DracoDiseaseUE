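; Base book actor for a book-organizing game, which the player picks up and places on shelf slots.
; Overlapping a "player"-tagged actor attaches it to HoldSocket; OnDropped looks for overlapping BP_BookSlots and calls TryAcceptBookcase, otherwise restoring the starting transform.
; The pickup path's drop branch never fires because PlacementLock is cleared just beforehand.
; The nearest-slot search is unfinished: its result is unused and never assigned a slot.
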(event OnComponentBeginOverlap(Box)
  (params (OverlappedComponent :type Primitive%20Component%20Object%20Reference) (OtherActor :type Actor%20Object%20Reference) (OtherComp :type Primitive%20Component%20Object%20Reference) (OtherBodyIndex :type Integer) (bFromSweep :type Boolean) (SweepResult :type Hit%20Result%20Structure%20%28by%20ref%29))
  ;[1 1 1] Player PicksUp Book
  (Development|PrintString "Picked Up")
  (if (Math|Boolean|ANDBoolean (not (Variables|Default|GetbPlaced)) (not (Variables|Default|GetHeld)) (Actor|ActorHasTag OtherActor "player"))
    (Variables|Default|SetHeld true)
    (Variables|Default|SetbPlacementLock false)
    (Development|PrintString "Holding")
    (Transformation|AttachComponentToComponent 0 "HoldSocket" "KeepRelative" "KeepRelative" "KeepRelative" true)
    (Variables|/Script/Engine.PrimitiveComponent|SetbGenerateOverlapEvents (Variables|Default|GetBox) false)
    (if (not (not (Variables|Default|GetbPlacementLock)))
      (Development|PrintString "Dropped off")
      (CallFunction|OnDropped))))

(event EventBeginPlay
  (|CallParentFunction)
  (Variables|Default|SetOriginalTransform (Transformation|GetActorTransform))
  (Variables|Default|SetbPlaced false))

(fn ConstructionScript
  (|CallParentFunction))

(fn FindNearestBookcase
  (params (Bookcases :type Array%20of%20Actor%20Object%20References))
  ;[1 1 1] If Book is in correct distance of bookcase then..
  (LocalVariables|SetBestDist 9999999.0)
  (LocalVariables|SetNearest%20Bookcase 0)
  (for _array_element Bookcases
    (bind _asbp_book_slot (Utilities|Casting|CastToBP_BookSlot _array_element))
    (bind _output_get (LocalVariables|SetSnapLoc (Transformation|GetWorldLocation (Variables|/Game/BP/BookOrganizer/BookCase/BP_BookSlot.BP_BookSlot_C|GetSnapPoint _asbp_book_slot))))
    (bind _output_get_2 (LocalVariables|SetDist (Math|Vector|VectorLength (- _output_get (LocalVariables|GetBookLoc)))))
    (if (< _output_get_2 (LocalVariables|GetBestDist))
      (LocalVariables|SetBestDist (LocalVariables|GetDist))
      (bind _output_get_3 (LocalVariables|SetNearest%20Bookcase (LocalVariables|GetNearest%20Bookcase)))))
  (return _output_get_3))

(fn ReturntoOriginal
  (Transformation|SetActorTransform (Variables|Default|GetOriginalTransform)))

(fn ResetBook()
  ;[1 1 1] Reset Location
  (if (not (Variables|Default|GetHeld))
    (Variables|Default|SetbPlaced false)
    (Collision|SetActorEnableCollision false)
    (Transformation|SetActorTransform (Variables|Default|GetOriginalTransform))))

(fn OnDropped
  ;[1 1 1] When Book is placed on shelf
  (if (and (Variables|Default|GetHeld) (not (Variables|Default|GetbPlaced)))
    (Variables|Default|SetBookcases (Collision|GetOverlappingActors "/Game/BP/BookOrganizer/BookCase/BP_BookSlot.BP_BookSlot_C" :!class /Script/Engine.Actor))
    (Development|PrintString (Utilities|String|ToString(Integer) (Utilities|Array|Length (Variables|Default|GetBookcases))))
    (if (> (Utilities|Array|Length (Variables|Default|GetBookcases)) 0)
      (Transformation|DetachFromActor "KeepWorld" "KeepWorld" "KeepWorld")
      (Collision|SetActorEnableCollision true)
      (CallFunction|FindNearestBookcase)
      (Default|TryAcceptBookcase (Variables|Default|GetBookSlot))
      (else
        (CallFunction|ReturntoOriginal)))
    (else
      (CallFunction|ReturntoOriginal))))