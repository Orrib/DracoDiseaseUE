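; Mountable crossbow turret that shows a Mount widget when the player is near and registers itself with the game controller.
; While player-mounted outside strategy mode, Tick rotates the base toward the cursor hit or a lock-on target tracked on the HUD.
; Attacks launch a pooled-free spawned dart straight ahead or with suggested velocity for a location or moving actor.
; A reload timer gates firing and restores the hidden arrow mesh.
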(event OnComponentBeginOverlap(Detector)
  (params (OverlappedComponent :type Primitive%20Component%20Object%20Reference) (OtherActor :type Actor%20Object%20Reference) (OtherComp :type Primitive%20Component%20Object%20Reference) (OtherBodyIndex :type Integer) (bFromSweep :type Boolean) (SweepResult :type Hit%20Result%20Structure%20%28by%20ref%29))
  (if (Actor|ActorHasTag OtherActor "player")
    (CallFunction|Show/HideUI true)))

(event OnComponentEndOverlap(Detector)
  (params (OverlappedComponent :type Primitive%20Component%20Object%20Reference) (OtherActor :type Actor%20Object%20Reference) (OtherComp :type Primitive%20Component%20Object%20Reference) (OtherBodyIndex :type Integer))
  (if (Actor|ActorHasTag OtherActor "player")
    (CallFunction|Show/HideUI false)))

(event Custom|Show/Hide%20UI
  (params (Show? :type Boolean))
  (bind _widget_defenseui (Variables|Default|GetWidget_DefenseUI))
  (Rendering|SetVisibility _widget_defenseui Show? false)
  (Collision|SetCollisionEnabled _widget_defenseui (select Show? "QueryOnly" "NoCollision"))
  (Default|Show/Hide (Variables|Default|GetTurret%20UI) Show? "Mount"))

(event Custom|Attempt%20Attack%20%28target%20a%20location%20or%20actor%29
  (params (Target%20Actor :type Actor%20Object%20Reference) (Target%20Location :type Vector) (Failed :type Boolean) (Fire%20at%20Target%20Location%20%28or%20just%20shoot%20straight%20ahead%29 :type Boolean))
  (bind _arrow (Variables|Default|GetArrow))
  (bind _arrow_2 (Variables|Default|GetArrow))
  (bind _projectile_velocity (Variables|Default|GetProjectile%20Velocity))
  (bind _returnvalue (Transformation|GetWorldRotation _arrow_2))
  (bind _returnvalue_2 (Math|Vector|GetForwardVector _arrow))
  (bind _returnvalue_3 (Transformation|GetWorldLocation _arrow))
  (bind _returnvalue_4 (* _returnvalue_2 _projectile_velocity))
  (if Failed
    ;[1 1 1] Projectile cannot spawn
    (Audio|PlaySound2D "/Game/Sound/SoundFX/Cue_Error.Cue_Error" 0.5 1.0 0.0 0 0 false :!label _label)
    (elif (not (Utilities|Time|IsValidTimerHandle (Variables|Default|GetTurret%20Attack%20Timer)))
      (bind _returnvalue_5 (Game|SpawnActorfromClass "/Game/BP/BP_Projectile_CrossbowDart.BP_Projectile_CrossbowDart_C" (Math|Transform|MakeTransform (Transformation|GetWorldLocation _arrow_2) (Math|Rotator|MakeRotator (.roll _returnvalue) (.pitch _returnvalue) (.yaw _returnvalue)) "1.000000,1.000000,1.000000") "AdjustIfPossibleButDontSpawnIfColliding" "MultiplyWithRoot" 0 0))
      (Utilities|IsValid _returnvalue_5
        (:Is%20Valid
          (Audio|PlaySound2D "/Game/Sound/SoundFX/Cue_Crossbow_Shot_Cue.Cue_Crossbow_Shot_Cue" 0.5 1.0 0.0 0 0 false)
          (Utilities|IsValid Target%20Actor
            (:Is%20Valid
              (bind _outlaunchvelocity (Class|GameplayStatics|SuggestProjectileVelocityMovingTarget _returnvalue_3 Target%20Actor "0, 0, 0" 0.0 0.2 "None"))
              (Transformation|SetActorRotation _returnvalue_5 (Math|Rotator|FindLookatRotation _returnvalue_3 (Transformation|GetActorLocation Target%20Actor)) true)
              (Default|Launch _returnvalue_5 (select Fire%20at%20Target%20Location%20%28or%20just%20shoot%20straight%20ahead%29 _outlaunchvelocity _returnvalue_4)))
            (:Is%20Not%20Valid
              (bind _tossvelocity (Class|GameplayStatics|BlueprintSuggestProjectileVelocity _returnvalue_3 Target%20Location _projectile_velocity 0.0 "DoNotTrace" 0.0 false false))
              (Transformation|SetActorRotation _returnvalue_5 (Math|Rotator|FindLookatRotation _returnvalue_3 Target%20Location) true)
              (Default|Launch _returnvalue_5 (select Fire%20at%20Target%20Location%20%28or%20just%20shoot%20straight%20ahead%29 _tossvelocity _returnvalue_4))))
          (Rendering|SetVisibility (Variables|Default|GetSM_CrossbowArrow) false false)
          ;[1 1 1] turret reload
          (bind _returnvalue_6 (Utilities|Time|SetTimerbyEvent (delegate Custom|CustomEvent_1) (Variables|Default|GetReload%20Time)))
          (Variables|Default|SetTurret%20Attack%20Timer _returnvalue_6)
          (Utilities|FlowControl|Delay 0.7)
          (Audio|PlaySound2D "/Game/Sound/SoundFX/Cue_Crossbow_Reload_Cue.Cue_Crossbow_Reload_Cue" 1.0 1.0 0.0 0 0))
        (:Is%20Not%20Valid
          (goto _label))))))

(event Custom|CustomEvent
  (CallFunction|PlayerMount/Dismount true true))

(event Custom|Player%20Mount/Dismount
  (params (Mount? :type Boolean) (Mounted%20By%20Player? :type Boolean))
  (bind _output_get (Variables|Default|SetMounted Mount?))
  (bind _output_get_2 (Variables|Default|SetPlayer%20Mounted Mounted%20By%20Player?))
  (CallFunction|Show/HideUI (not _output_get))
  (if _output_get_2
    (bind _asbp_game_instance (Utilities|Casting|CastToBP_GameInstance (Game|GetGameInstance)))
    (Default|Mount/DismountTurret (Variables|/Game/BP/BP_GameInstance.BP_GameInstance_C|GetTop%20Down%20Controller _asbp_game_instance) _output_get self)
    (else
      (Transformation|SetRelativeRotation (Variables|Default|GetTurret%20Base) (Variables|Default|GetTurret%20Base%20Orig%20Relative%20Rotation) false false))))

(event Custom|On%20Enter/Exit%20Strategy%20Mode
  (params (Enter/Exit%20%28t/f%29 :type Boolean))
  (Development|SetHiddeninGame (Variables|Default|GetWidget_DefenseUI) Enter/Exit%20%28t/f%29 false))

(event Custom|Lock%20On/%20Lock%20Off
  (params (Lock-On? :type Boolean) (Lock%20On%20Target :type Actor%20Object%20Reference))
  (Default|Show/HideLockon (Variables|/Game/TopDown/Blueprints/BP_TopDownController.BP_TopDownController_C|GetHUD (Variables|Default|GetTop%20Down%20Controller)) Lock-On?)
  (if Lock-On?
    (bind _asbp_npc (Utilities|Casting|CastToBP_NPC Lock%20On%20Target)
      (:then
        (Variables|Default|SetLock%20On%20Target%20Offset (- (Transformation|GetWorldLocation (Variables|/Game/TopDown/Blueprints/BP_NPC.BP_NPC_C|Getlock%20on%20target%20UI%20location _asbp_npc)) (Transformation|GetActorLocation _asbp_npc))))
      (:CastFailed
        (Variables|Default|SetLock%20On%20Target%20Offset "0, 0, 0")))
    (Variables|Default|SetLock%20On%20Target Lock%20On%20Target)
    (else
      (Variables|Default|SetLock%20On%20Target 0))))

(event Custom|CustomEvent_1
  ;[1 1 1] turret reload
  (Rendering|SetVisibility (Variables|Default|GetSM_CrossbowArrow) true false)
  (Utilities|Time|ClearandInvalidateTimerbyHandle (Variables|Default|GetTurret%20Attack%20Timer)))

(event EventBeginPlay
  (Variables|Default|SetTurret%20Base%20Orig%20Relative%20Rotation (Variables|/Script/Engine.SceneComponent|GetRelativeRotation (Variables|Default|GetTurret%20Base)))
  (Utilities|FlowControl|DelayUntilNextTick)
  (bind _asbp_game_instance (Utilities|Casting|CastToBP_GameInstance (Game|GetGameInstance)))
  (Variables|Default|SetTop%20Down%20Controller (Variables|/Game/BP/BP_GameInstance.BP_GameInstance_C|GetTop%20Down%20Controller _asbp_game_instance))
  (Utilities|Array|Add (Variables|/Game/BP/BP_GameController.BP_GameController_C|GetTurrets (Variables|/Game/BP/BP_GameInstance.BP_GameInstance_C|GetGame%20Controller _asbp_game_instance)) self)
  (bind _aswidget_defense_ui (Utilities|Casting|CastToWidget_DefenseUI (UserInterface|GetWidget (Variables|Default|GetWidget_DefenseUI))))
  (bind _output_get (Variables|Default|SetTurret%20UI _aswidget_defense_ui))
  (EventDispatchers|BindEventtoOnActionButtonPressed _output_get (delegate Custom|CustomEvent))
  (CallFunction|Show/HideUI false))

(event EventTick
  (params (DeltaSeconds :type Float%20%28single-precision%29))
  (bind _turret_base (Variables|Default|GetTurret%20Base))
  (bind _top_down_controller (Variables|Default|GetTop%20Down%20Controller))
  (bind _turret_base_2 (Variables|Default|GetTurret%20Base))
  (bind _lock_on_target (Variables|Default|GetLock%20On%20Target))
  (bind _lock_on_target_2 (Variables|Default|GetLock%20On%20Target))
  (bind _hitresult (Game|Player|GetHitResultUnderCursorbyChannel _top_down_controller "TraceTypeQuery1" true))
  (bind _returnvalue (Transformation|GetWorldLocation _turret_base_2))
  (bind _returnvalue_2 (Transformation|GetActorLocation _lock_on_target))
  (bind (_bblockinghit _binitialoverlap _time _distance _location) (Collision|BreakHitResult _hitresult))
  (bind _returnvalue_3 (Math|Rotator|FindLookatRotation _returnvalue _returnvalue_2))
  (bind _returnvalue_4 (Math|Rotator|FindLookatRotation _returnvalue _location))
  (if (Variables|Default|GetMounted)
    ;[1 1 1] Player Mounted
    (if (Variables|Default|GetPlayer%20Mounted)
      (if (not (Variables|/Game/TopDown/Blueprints/BP_TopDownController.BP_TopDownController_C|GetIn%20Strategy%20Mode? (Variables|Default|GetTop%20Down%20Controller)))
        (Utilities|FlowControl|Sequence
          (:then_0
            ;[1 1 1] Turn turret
            (Utilities|IsValid _lock_on_target
              (:Is%20Valid
                (Transformation|SetWorldRotation _turret_base (Math|Rotator|MakeRotator (* (.pitch _returnvalue_3) -1.0) (.roll _returnvalue_3) (+ (.yaw _returnvalue_3) -9e+01)) false false))
              (:Is%20Not%20Valid
                (if _bblockinghit
                  (Transformation|SetWorldRotation _turret_base (Math|Rotator|MakeRotator (* (.pitch _returnvalue_4) -1.0) (.roll _returnvalue_4) (+ (.yaw _returnvalue_4) -9e+01)) false false)))))
          (:then_1
            ;[1 1 1] Lock On Target
            (Utilities|IsValid _lock_on_target_2
              (:Is%20Valid
                (Default|SetLockonLocationfromWorldSpace (Variables|/Game/TopDown/Blueprints/BP_TopDownController.BP_TopDownController_C|GetHUD (Variables|Default|GetTop%20Down%20Controller)) (+ (Variables|Default|GetLock%20On%20Target%20Offset) (Transformation|GetActorLocation _lock_on_target_2))))
              (:Is%20Not%20Valid
                (CallFunction|LockOn/LockOff false)))))))))

(fn ConstructionScript)