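; BP_BookSlot is a bookcase slot for a book-ordering puzzle, apparently unfinished.
; A box overlap prints a debug message and casts to BP_BookBase, but the registering, snapping and attaching logic after it is disconnected.
; RegisterBook records books in PlacedBooks by slot index, clears a book's previous slot, then calls CheckAllBooksCorrect.
; That check has an empty loop, so it never compares against ExpectedOrder or sets PuzzleSolved.
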(event OnComponentBeginOverlap(BoxCollision)
  (params (OverlappedComponent :type Primitive%20Component%20Object%20Reference) (OtherActor :type Actor%20Object%20Reference) (OtherComp :type Primitive%20Component%20Object%20Reference) (OtherBodyIndex :type Integer) (bFromSweep :type Boolean) (SweepResult :type Hit%20Result%20Structure%20%28by%20ref%29))
  (Development|PrintString "Book Placed")
  (Utilities|Casting|CastToBP_BookBase OtherActor))

(event EventBeginPlay
  (Variables|Default|SetOwning%20Bookcase (Variables|Default|GetOwningBookcase))
  (Variables|Default|SetBook%20Slots (Utilities|Select :Index (Variables|Default|GetSlotIndex) :Option%200 (Variables|Default|GetBook%20Slots) :Option%201 0)))

(fn ConstructionScript)

(fn RegisterBook
  (params (Book :type BP%20Book%20Base%20Object%20Reference) (SlotIndex :type Integer))
  (bind _placedbooks (Variables|Default|GetPlacedBooks))
  (bind _placedbooks_2 (Variables|Default|GetPlacedBooks))
  (bind _returnvalue (Utilities|Array|FindItem _placedbooks_2 Book))
  (bind _returnvalue_2 (Utilities|Array|Length _placedbooks))
  (bind _returnvalue_3 (< SlotIndex _returnvalue_2))
  (if (Variables|Default|GetbPuzzleSolved)
    (return)
    (elif (and _returnvalue_3 (>= _returnvalue_3 0))
      (Utilities|FlowControl|Sequence
        (:then_0
          (if (and (!= _returnvalue -1) (!= _returnvalue SlotIndex))
            (Utilities|Array|SetArrayElem (Variables|Default|GetPlacedBooks) _returnvalue 0)))
        (:then_1
          (Utilities|Array|SetArrayElem (Variables|Default|GetPlacedBooks) SlotIndex Book)
          (CallFunction|CheckAllBooksCorrect :!label _label))
        (:then_2
          (goto _label)))
      (else
        (return)))))

(fn CheckAllBooksCorrect
  (bind _expectedorder (Variables|Default|GetExpectedOrder))
  (bind _placedbooks (Variables|Default|GetPlacedBooks))
  (bind _returnvalue (Utilities|Array|Length _placedbooks))
  (bind _returnvalue_2 (Utilities|Array|Length _expectedorder))
  (bind _returnvalue_3 (Class|KismetMathLibrary|AndIntInt _returnvalue _returnvalue_2))
  (LocalVariables|SetAllCorrect true)
  (if (Variables|Default|GetbPuzzleSolved)
    (return)
    (elif (== _returnvalue_3 _returnvalue_3)
      (for _index (range 0 (- (Utilities|Array|Length (Variables|Default|GetPlacedBooks)) -1))
        _)
      (else
        (return)))))