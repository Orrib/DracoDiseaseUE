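; BP_Trigger_Monologue is a one-shot trigger actor that shows a monologue line when the player walks into it.
; On overlap with an actor tagged "player", a DoOnce gate and a configurable delay run before it reaches the TopDownCharacter through the game instance's GameController.
; It passes its text and display time to ShowMonologue, then destroys itself.
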(event EventBeginPlay)

(event Collision|EventActorBeginOverlap
  (params (OtherActor :type Actor%20Object%20Reference))
  (if (Actor|ActorHasTag OtherActor "player")
    (Utilities|FlowControl|DoOnce false
      (:Completed
        (Utilities|FlowControl|Delay (Variables|Default|GetDelay%20Time))
        (Utilities|FlowControl|Sequence
          (:then_0
            (bind _asbp_game_instance (Utilities|Casting|CastToBP_GameInstance (Game|GetGameInstance)))
            (Default|ShowMonologue (Variables|/Game/BP/BP_GameController.BP_GameController_C|GetTop%20Down%20Character (Variables|/Game/BP/BP_GameInstance.BP_GameInstance_C|GetGame%20Controller _asbp_game_instance)) (Variables|Default|GetText) (Variables|Default|GetShow%20Time)))
          (:then_1
            (Actor|DestroyActor)))))))

(event EventTick
  (params (DeltaSeconds :type Float%20%28single-precision%29)))

(fn ConstructionScript)