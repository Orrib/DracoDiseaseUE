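; BP_EnemyController is a debug-style actor that sends all BP_NPC actors toward a tagged target on a key press.
; BeginPlay enables player input and caches the first actor tagged "enemytarget".
; Pressing G issues AIMoveTo on each BP_NPC toward that actor, printing on arrival, and draws a debug sphere at the target's location.
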(event EventBeginPlay
  (Input|EnableInput (Game|GetPlayerController 0))
  (bind _outactors (Actor|GetAllActorswithTag "enemytarget"))
  (Variables|Default|SetEnemy%20Target (Utilities|Array|Get(acopy) _outactors)))

(event Collision|EventActorBeginOverlap
  (params (OtherActor :type Actor%20Object%20Reference)))

(event EventTick
  (params (DeltaSeconds :type Float%20%28single-precision%29)))

(event Input|KeyboardEvents|G
  (params (Key :type Key%20Structure))
  (bind _enemy_target (Variables|Default|GetEnemy%20Target))
  (:Pressed
    (bind _outactors (Actor|GetAllActorsOfClass "/Game/TopDown/Blueprints/BP_NPC.BP_NPC_C"))
    (for _array_element _outactors
      (AI|AIMoveTo _array_element "0, 0, 0" _enemy_target 5.0 true
        (:OnSuccess
          (Development|PrintString "arrived"))))
    (Rendering|Debug|DrawDebugSphere (Transformation|GetActorLocation _enemy_target) 2e+01 12 "(R=1.000000,G=1.000000,B=1.000000,A=1.000000)" 2.0)))

(fn ConstructionScript)