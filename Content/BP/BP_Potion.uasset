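; Potion pickup Blueprint that stores one potion in the player's inventory when collected, showing a rising icon.
; OnPickup first checks the game instance's save object; if the item is already at max quantity, it spawns a replacement potion sprite pickup in place and plays an error sound.
; Both outcomes finish through the parent pickup logic.
; An unconnected branch holds instant-heal logic with screen effect, UI and sound feedback, which never runs.
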(event EventBeginPlay)

(event EventOnPickup
  (params (Player%20Controller :type BP%20Top%20Down%20Controller%20Object%20Reference))
  (bind _game_instance (Variables|/Game/TopDown/Blueprints/BP_TopDownController.BP_TopDownController_C|GetGame%20Instance Player%20Controller))
  (bind _save_game_instance___impersistent (Variables|/Game/BP/BP_GameInstance.BP_GameInstance_C|GetSave%20Game%20Instance%20-%20Impersistent _game_instance))
  (bind (_item_in_inventory _at_max_quantity) (Default|IsInventoryItematMaxQuantity? _save_game_instance___impersistent "NewEnumerator1"))
  (if _item_in_inventory
    (if _at_max_quantity
      (Game|SpawnActorfromClass "/Game/BP/BP_Pickup_Sprite_Potion.BP_Pickup_Sprite_Potion_C" (Math|Transform|MakeTransform (Transformation|GetActorLocation) "0, 0, 0" "1.000000,1.000000,1.000000") "AlwaysSpawn" "MultiplyWithRoot" 0 false 1.0 0)
      (Audio|PlaySound2D "/Game/Sound/SoundFX/Cue_Error.Cue_Error" 0.3 1.0 0.0 0 0)
      (|CallParentFunction Player%20Controller)
      (else
        (Utilities|FlowControl|Sequence :!label _label
          (:then_0
            (CallFunction|ShowRisingIcon Player%20Controller)
            (Default|AddItemtoInventory Player%20Controller "NewEnumerator1" 1))
          (:then_1
            (|CallParentFunction Player%20Controller)))))
    (else
      (goto _label))))

(fn ConstructionScript)