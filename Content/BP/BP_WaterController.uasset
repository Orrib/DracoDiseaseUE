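; BP_WaterController spawns recurring splashes at the water surface for player, npc and wild-tagged actors inside a water volume.
; WaterMesh overlap events add and remove those actors from a tracked list, starting a looping timer on entry and clearing it when an exit empties the list.
; Each tick of the timer spawns a Splash at every tracked actor's XY and WaterTopNormal's height, dropping invalid entries.
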(event OnActorBeginOverlap(WaterMesh)
  (params (OverlappedActor :type Actor%20Object%20Reference) (OtherActor :type Actor%20Object%20Reference))
  (if (Math|Boolean|ORBoolean (Actor|ActorHasTag OtherActor "npc") (Actor|ActorHasTag OtherActor "player") (Actor|ActorHasTag OtherActor "wild"))
    (Utilities|Array|AddUnique (Variables|Default|GetTracked%20Actors) OtherActor)
    (if (not (Utilities|Time|IsValidTimerHandle (Variables|Default|GetSplash%20Timer)))
      (bind _returnvalue (Utilities|Time|SetTimerbyEvent (delegate Custom|CustomEvent) (Variables|Default|GetRefresh%20Time%20%28in%20secs%29) true))
      (Variables|Default|SetSplash%20Timer _returnvalue))))

(event OnActorEndOverlap(WaterMesh)
  (params (OverlappedActor :type Actor%20Object%20Reference) (OtherActor :type Actor%20Object%20Reference))
  (bind _tracked_actors (Variables|Default|GetTracked%20Actors))
  (if (Math|Boolean|ORBoolean (Actor|ActorHasTag OtherActor "npc") (Actor|ActorHasTag OtherActor "player") (Actor|ActorHasTag OtherActor "wild"))
    (Utilities|Array|RemoveItem _tracked_actors OtherActor)
    (if (Utilities|Array|IsEmpty _tracked_actors)
      (Utilities|Time|ClearandInvalidateTimerbyHandle (Variables|Default|GetSplash%20Timer)))))

(event Custom|CustomEvent
  (bind _tracked_actors (Variables|Default|GetTracked%20Actors))
  (for _array_element _tracked_actors
    (Utilities|IsValid _array_element
      (:Is%20Valid
        (Game|SpawnActorfromClass (Variables|Default|GetSplash) (Math|Transform|MakeTransform (Math|Vector|MakeVector (.x (Transformation|GetActorLocation _array_element)) (.y (Transformation|GetActorLocation _array_element)) (.z (Transformation|GetWorldLocation (Variables|Default|GetWater%20Top%20Normal)))) "0, 0, 0" "1.000000,1.000000,1.000000") "AlwaysSpawn" "MultiplyWithRoot" 0 0))
      (:Is%20Not%20Valid
        (Utilities|Array|RemoveItem _tracked_actors _array_element)))))

(event EventBeginPlay)

(event Collision|EventActorBeginOverlap
  (params (OtherActor :type Actor%20Object%20Reference)))

(fn ConstructionScript)