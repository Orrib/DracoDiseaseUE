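; BP_Defense_Spikes is a single-use spike trap that reacts when something overlaps its Box component.
; Actors tagged "player" take DamageToPlayer damage, while actors tagged "npc" are destroyed outright.
; Either hit plays a sword sound and destroys the trap.
; The construction script calls the parent's, then adds a random quarter-turn yaw rotation to vary the trap's orientation.
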(event OnComponentBeginOverlap(Box)
  (params (OverlappedComponent :type Primitive%20Component%20Object%20Reference) (OtherActor :type Actor%20Object%20Reference) (OtherComp :type Primitive%20Component%20Object%20Reference) (OtherBodyIndex :type Integer) (bFromSweep :type Boolean) (SweepResult :type Hit%20Result%20Structure%20%28by%20ref%29))
  (if (Actor|ActorHasTag OtherActor "player")
    (Game|Damage|ApplyDamage OtherActor (Variables|Default|GetDamage%20to%20Player) 0 self)
    (Audio|PlaySound2D "/Game/Sound/SoundFX/Cue_Sword.Cue_Sword" 1.0 1.0 0.0 0 0 :!label _label)
    (Actor|DestroyActor)
    (elif (Actor|ActorHasTag OtherActor "npc")
      (Actor|DestroyActor OtherActor)
      (goto _label))))

(event EventBeginPlay)

(event Collision|EventActorBeginOverlap
  (params (OtherActor :type Actor%20Object%20Reference)))

(event EventTick
  (params (DeltaSeconds :type Float%20%28single-precision%29)))

(fn ConstructionScript
  (|CallParentFunction)
  (Class|Actor|AddActorWorldRotation (Math|Rotator|MakeRotator 0.0 0.0 (Utilities|Select :Index (Math|Random|RandomIntegerinRange 0 3) :Option%200 0.0 :Option%201 9e+01 :Option%202 1.8e+02 :Option%203 2.7e+02))))