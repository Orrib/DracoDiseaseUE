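; BP_RisingIcon_Text is a rising icon variant that displays a text string through a TextRender component.
; On BeginPlay it runs the parent logic and applies its Text value.
; At the halfway point of the rise it plays a Fade timeline, scaled by the inverse of FadeTime, then destroys the actor.
; The RiseFinished event is left empty, so the end of the fade handles destruction.
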(event EventBeginPlay
  (|CallParentFunction)
  (Rendering|Components|TextRender|SetText (Variables|Default|GetTextRender) (Variables|Default|GetText)))

(event EventRiseHalfway
  (|CallParentFunction)
  (Components|Timeline|SetPlayRate (Variables|Default|GetFade) (Math|Float|Power (Variables|Default|GetFade%20Time) -1.0))
  (Timeline|Fade PlayFromStart
    (:Finished
      (Actor|DestroyActor))))

(event EventRiseFinished)

(fn ConstructionScript
  (|CallParentFunction))