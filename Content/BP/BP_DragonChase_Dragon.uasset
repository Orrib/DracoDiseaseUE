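; Dragon actor for a chase sequence that flies a paper flipbook in and out on a timeline and breathes fire that damages the player.
; Enabling fire toggles both effects and actor tick, which applies fire damage every frame while an overlap counter shows the player inside an attack box.
; A hitbox type selects rear or line collision, with optional debug display.
; Orientation mirrors the scene's Y scale and swaps the visible fire effect.
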(event OnComponentBeginOverlap(Box-RearAttack)
  (params (OverlappedComponent :type Primitive%20Component%20Object%20Reference) (OtherActor :type Actor%20Object%20Reference) (OtherComp :type Primitive%20Component%20Object%20Reference) (OtherBodyIndex :type Integer) (bFromSweep :type Boolean) (SweepResult :type Hit%20Result%20Structure%20%28by%20ref%29))
  (if (Actor|ActorHasTag OtherActor "player")
    (Math|Integer|IncrementInt (Variables|Default|GetColliders%20that%20detect%20player))))

(event OnComponentBeginOverlap(Box-LineAttack)
  (params (OverlappedComponent :type Primitive%20Component%20Object%20Reference) (OtherActor :type Actor%20Object%20Reference) (OtherComp :type Primitive%20Component%20Object%20Reference) (OtherBodyIndex :type Integer) (bFromSweep :type Boolean) (SweepResult :type Hit%20Result%20Structure%20%28by%20ref%29))
  (if (Actor|ActorHasTag OtherActor "player")
    (Math|Integer|IncrementInt (Variables|Default|GetColliders%20that%20detect%20player))))

(event OnComponentEndOverlap(Box-RearAttack)
  (params (OverlappedComponent :type Primitive%20Component%20Object%20Reference) (OtherActor :type Actor%20Object%20Reference) (OtherComp :type Primitive%20Component%20Object%20Reference) (OtherBodyIndex :type Integer))
  (if (Actor|ActorHasTag OtherActor "player")
    (Math|Integer|DecrementInt (Variables|Default|GetColliders%20that%20detect%20player))))

(event OnComponentEndOverlap(Box-LineAttack)
  (params (OverlappedComponent :type Primitive%20Component%20Object%20Reference) (OtherActor :type Actor%20Object%20Reference) (OtherComp :type Primitive%20Component%20Object%20Reference) (OtherBodyIndex :type Integer))
  (if (Actor|ActorHasTag OtherActor "player")
    (Math|Integer|DecrementInt (Variables|Default|GetColliders%20that%20detect%20player))))

(event Custom|Enable/Disable%20Fire
  (params (Enable? :type Boolean))
  (CallFunction|SetDragonOrientation (Variables|Default|GetDragon%20Orientation%20-%20Right/%20Left%20%28T/%20F%29))
  (Components|Activation|SetActive (Variables|Default|GetFire) Enable? false)
  (Actor|Tick|SetActorTickEnabled Enable?))

(event Custom|Set%20Attack%20Hitbox
  (params (Hitbox%20Type :type Enum_DragonChaseAttackHitboxType%20Enum :default "NewEnumerator0"))
  (bind _box___rear_attack (Variables|Default|GetBox%20-%20Rear%20Attack))
  (bind _box___line_attack (Variables|Default|GetBox%20-%20Line%20Attack))
  (bind _debug_colliders (Variables|Default|GetDebug%20colliders))
  (bind _output_get (Variables|Default|SetHitbox%20Type Hitbox%20Type))
  (switch Utilities|FlowControl|Switch|SwitchonEnum_DragonChaseAttackHitboxType _output_get
    (:NewEnumerator0
      (Collision|SetCollisionEnabled _box___line_attack "NoCollision")
      (Collision|SetCollisionEnabled _box___rear_attack "QueryOnly")
      (if _debug_colliders
        (Development|SetHiddeninGame _box___rear_attack false false)
        (Development|SetHiddeninGame _box___line_attack true false)))
    (:NewEnumerator1
      (Collision|SetCollisionEnabled _box___line_attack "QueryOnly")
      (Collision|SetCollisionEnabled _box___rear_attack "NoCollision")
      (if _debug_colliders
        (Development|SetHiddeninGame _box___line_attack false false)
        (Development|SetHiddeninGame _box___rear_attack true false)))
    (:NewEnumerator2
      (Collision|SetCollisionEnabled _box___rear_attack "NoCollision")
      (Development|SetHiddeninGame _box___rear_attack true false))))

(event Custom|Dragon%20Fly%20In
  (bind _newtrack_0 (Timeline|Timeline PlayFromStart)
    (:Update
      (Transformation|SetWorldLocation (Variables|Default|GetPaperFlipbook) (Math|Vector|Lerp(Vector) (Transformation|GetWorldLocation (Variables|Default|GetDragon%20Start%20Pos)) (Transformation|GetWorldLocation (Variables|Default|GetDragon%20Normal%20Pos)) _newtrack_0) false false))))

(event Custom|Dragon%20Fly%20Out
  (bind _newtrack_0 (Timeline|Timeline ReverseFromEnd)
    (:Update
      (Transformation|SetWorldLocation (Variables|Default|GetPaperFlipbook) (Math|Vector|Lerp(Vector) (Transformation|GetWorldLocation (Variables|Default|GetDragon%20Start%20Pos)) (Transformation|GetWorldLocation (Variables|Default|GetDragon%20Normal%20Pos)) _newtrack_0) false false))))

(event Custom|Set%20Dragon%20Orientation
  (params (Right/Left%20%28T/F%29 :type Boolean))
  (bind _output_get (Variables|Default|SetDragon%20Orientation%20-%20Right/%20Left%20%28T/%20F%29 Right/Left%20%28T/F%29))
  (Transformation|SetWorldScale3D (Variables|Default|GetScene) (Math|Vector|MakeVector 1.0 (select Right/Left%20%28T/F%29 1.0 -1.0) 1.0))
  (Rendering|SetVisibility (Variables|Default|GetFire) _output_get false)
  (Rendering|SetVisibility (Variables|Default|GetFire_reversed) (not _output_get) false))

(event EventBeginPlay
  (bind _asbp_top_down_character (Utilities|Casting|CastToBP_TopDownCharacter (Game|GetPlayerCharacter 0)))
  (Variables|Default|SetPlayer _asbp_top_down_character))

(event Collision|EventActorBeginOverlap
  (params (OtherActor :type Actor%20Object%20Reference)))

(event EventTick
  (params (DeltaSeconds :type Float%20%28single-precision%29))
  (if (> (Variables|Default|GetColliders%20that%20detect%20player) 0)
    (Game|Damage|ApplyDamage (Variables|Default|GetPlayer) (Variables|Default|GetDamage) 0 0 "/Game/BP/DamageType_Fire_Primary_Blue.DamageType_Fire_Primary_Blue_C")))

(fn ConstructionScript
  (CallFunction|SetAttackHitbox (Variables|Default|GetHitbox%20Type)))