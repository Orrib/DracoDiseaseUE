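; BP_GorePart is a short-lived gore debris actor with a Cube component and a Paper2D sprite.
; Its construction script randomizes the Cube's scale and the sprite's pitch rotation for visual variety.
; After a random delay of several seconds from BeginPlay, a timeline drives the sprite's alpha, presumably fading it out, then destroys the actor.
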(event EventBeginPlay
  (Utilities|FlowControl|Delay (Math|Random|RandomFloatinRange 7.0 9.0))
  (bind _newtrack_0 (Timeline|Timeline PlayFromStart)
    (:Update
      (Sprite|SetSpriteColor (Variables|Default|GetPaperSprite) (Utilities|Struct|MakeLinearColor 1.0 1.0 1.0 _newtrack_0)))
    (:Finished
      (Actor|DestroyActor))))

(fn ConstructionScript
  (CallFunction|RadnomizeScale)
  (CallFunction|RandomizeRotation))

(fn RadnomizeScale
  (bind _cube (Variables|Default|GetCube))
  (Transformation|SetRelativeScale3D _cube (* (Variables|/Script/Engine.SceneComponent|GetRelativeScale3D _cube) (Math|Random|RandomFloatinRange 1.3 1.0))))

(fn RandomizeRotation
  (Transformation|SetRelativeRotation (Variables|Default|GetPaperSprite) (Math|Rotator|MakeRotator 0.0 (Math|Random|RandomFloatinRange 0.0 3.6e+02) 0.0) false true))