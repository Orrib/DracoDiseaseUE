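; BP_Orb is an orb actor that lights up when overlapped and stays active for a set duration.
; Overlap calls Activate, which, if not already active, broadcasts OnOrbActivated with the orb's index and sets a timer for Deactivate.
; Deactivate clears the state, restores the off glow and broadcasts OnOrbDeactivated.
; A dynamic material instance drives Glow Power, with a timeline replaying the glow lerp on every overlap.
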(event EventBeginPlay
  (bind _returnvalue (Rendering|Material|CreateDynamicMaterialInstance "/Game/Materials/M_Orb.M_Orb" "None" "None" :!class /Script/Engine.KismetMaterialLibrary))
  (bind _output_get (Variables|Default|SetDynamic%20Material _returnvalue))
  (Rendering|Material|SetMaterial (Variables|Default|Getsm_WeaponRack) 0 _output_get)
  (Rendering|Material|SetScalarParameterValue (Variables|Default|GetDynamic%20Material) "Glow Power" (Variables|Default|GetGlow%20Off) :!class /Script/Engine.MaterialInstanceDynamic))

(event Collision|EventActorBeginOverlap
  (params (OtherActor :type Actor%20Object%20Reference))
  (CallFunction|Activate)
  (bind _glow_power (Timeline|Timeline PlayFromStart)
    (:Update
      (Rendering|Material|SetScalarParameterValue (Variables|Default|GetDynamic%20Material) "Glow Power" (Math|Float|Lerp (Variables|Default|GetGlow%20Off) (Variables|Default|GetGlow%20On) _glow_power) :!class /Script/Engine.MaterialInstanceDynamic))))

(fn ConstructionScript)

(fn Activate
  (if (not (Variables|Default|GetIs%20Active))
    (Variables|Default|SetIs%20Active true)
    (Rendering|Material|SetScalarParameterValue (Variables|Default|GetDynamic%20Material) "Glow Power" (Variables|Default|GetGlow%20On) :!class /Script/Engine.MaterialInstanceDynamic)
    (Default|CallOnOrbActivated (Variables|Default|GetOrb%20Index))
    (Utilities|Time|SetTimerbyFunctionName 0 "Deactivate" (Variables|Default|GetActivation%20Duration))))

(fn Deactivate
  (Variables|Default|SetIs%20Active false)
  (Rendering|Material|SetScalarParameterValue (Variables|Default|GetDynamic%20Material) "Glow Power" (Variables|Default|GetGlow%20Off) :!class /Script/Engine.MaterialInstanceDynamic)
  (Default|CallOnOrbDeactivated (Variables|Default|GetOrb%20Index)))