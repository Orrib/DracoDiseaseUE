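; Monorail traincar Blueprint variant that carries a randomized set of 2D villager passengers.
; The construction script gives each Paper2D flipbook component a coin flip to either show one of four random villager idle animations or be hidden.
; After running the parent tick, Tick resets five scene components to zero world rotation every frame, so they keep a fixed orientation as the car rotates.
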(event EventBeginPlay
  (|CallParentFunction) ; This node is disabled and will not be called.\nDrag off pins to build functionality.
)

(event Collision|EventActorBeginOverlap
  (params (OtherActor :type Actor%20Object%20Reference))
  (|CallParentFunction OtherActor) ; This node is disabled and will not be called.\nDrag off pins to build functionality.
)

(event EventTick
  (params (DeltaSeconds :type Float%20%28single-precision%29))
  (|CallParentFunction DeltaSeconds)
  (Transformation|SetWorldRotation (Variables|Default|GetScene4) "0, 0, 0" false false))

(fn ConstructionScript
  (|CallParentFunction)
  (for _array_element (Actor|GetComponentsByClass "/Script/Paper2D.PaperFlipbookComponent")
    (if (Math|Random|RandomBool)
      (Sprite|SetFlipbook _array_element (Utilities|Select :Index (Math|Random|RandomIntegerinRange 0 3) :Option%200 "/Game/Art/Villagers/Woman_Basket/BASKET_WOMAN_IDLE.BASKET_WOMAN_IDLE" :Option%201 "/Game/Art/Villagers/Man_Farmer/FARMER_MAN_IDLE.FARMER_MAN_IDLE" :Option%202 "/Game/Art/Villagers/Man/MAN_IDLE.MAN_IDLE" :Option%203 "/Game/Art/Villagers/Woman/WOMAN_IDLE.WOMAN_IDLE"))
      (else
        (Rendering|SetVisibility _array_element false false)))))