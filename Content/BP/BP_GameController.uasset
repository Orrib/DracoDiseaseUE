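; Central game controller for a wave-based castle defense game, registering itself with the game instance and handling music, popups, NPC selection and restart/quit.
; Five wave Timelines fire spawn events that place wizard enemies at random spawn points and assign their objective, updating the wave UI.
; Castle damage updates the UI and, at zero health, pauses the game with a Game Over popup whose button reloads the level.
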(event Custom|Play%20Background%20Music
  ;[1 0 0] temp
  (if (Variables|/Game/BP/BP_GameInstance.BP_GameInstance_C|GetMusic%20Enabled (Variables|Default|GetGame%20Instance))
    (Audio|PlaySound2D "/Game/Sound/Music/Cue_Music_Background.Cue_Music_Background" 1.0 1.0 0.0 0 0)))

(event Custom|Select%20NPC
  (params (NPC :type BP%20NPC%20Object%20Reference))
  ;[1 1 1] Selection
  (Utilities|Array|Add (Variables|Default|GetSelected%20NPCs) NPC)
  (Default|OnSelect/UnselectNPC NPC true))

(event Custom|Damage%20Castle
  (params (Damage :type Float%20%28double-precision%29))
  ;[1 1 1] Castle Health
  (bind _output_get (Variables|Default|SetCastle%20Health%20%280-1%29 (- (Variables|Default|GetCastle%20Health%20%280-1%29) Damage)))
  (Default|UpdateCastleHealth (Variables|/Game/TopDown/Blueprints/BP_TopDownController.BP_TopDownController_C|GetUI (Variables|/Game/TopDown/Blueprints/BP_TopDownCharacter.BP_TopDownCharacter_C|GetTop%20Down%20Controller (Variables|Default|GetTop%20Down%20Character))) _output_get)
  (Audio|PlaySound2D "/Game/Sound/SoundFX/Cue_Error.Cue_Error" 1.5 0.8 0.0 0 0)
  (if (<= _output_get 0.0)
    (CallFunction|InitiateGameOver "The castle was destroyed.")))

(event Custom|testy
  (Development|PrintString "testy"))

(event Custom|Unselect%20NPC
  (params (Item :type BP%20NPC%20Object%20Reference))
  ;[1 1 1] Selection
  (Utilities|Array|RemoveItem (Variables|Default|GetSelected%20NPCs) Item)
  (Default|OnSelect/UnselectNPC Item false))

(event Custom|Unselect%20All
  (bind _selected_npcs (Variables|Default|GetSelected%20NPCs))
  ;[1 1 1] Selection
  (for _array_element _selected_npcs
    (Utilities|IsValid _array_element
      (:Is%20Valid
        (Default|OnSelect/UnselectNPC _array_element false)
        (Utilities|Array|Clear _selected_npcs)))))

(event Custom|Initiate%20Game%20Over
  (params (Reason%20Text :type String))
  (Game|SetGamePaused true)
  (bind _created_popup_widget (CallFunction|CreatePopup false false false "Game Over!" (Utilities|Text|ToText(String) (Utilities|String|Append "The Kingdom is lost..." (Utilities|String|Append " 
 
" Reason%20Text))) "Restart"))
  (EventDispatchers|BindEventtoOnClickButton1 _created_popup_widget (delegate Custom|CustomEvent)))

(event Custom|CustomEvent
  ;[1 1 1] restart game
  (CallFunction|RestartLevel))

(event Custom|Restart%20Level
  (Game|SetGamePaused false)
  (bind _returnvalue (Game|GetCurrentLevelName true))
  (Game|OpenLevel(byName) (Utilities|String|StringToName _returnvalue)))

(event Custom|Quit%20Game
  (Game|SetGamePaused false)
  (Game|QuitGame 0 "Quit" false))

(event Custom|Start%20Next%20Wave
  (bind _top_down_character (Variables|Default|GetTop%20Down%20Character))
  (bind _current_wave (Variables|Default|GetCurrent%20Wave))
  (bind _total_num_waves (Variables|Default|GetTotal%20Num%20Waves))
  (bind _returnvalue (+ _total_num_waves 1))
  (bind _top_down_controller (Variables|/Game/TopDown/Blueprints/BP_TopDownCharacter.BP_TopDownCharacter_C|GetTop%20Down%20Controller _top_down_character))
  (bind _returnvalue_2 (< _current_wave _returnvalue))
  (bind _ui (Variables|/Game/TopDown/Blueprints/BP_TopDownController.BP_TopDownController_C|GetUI _top_down_controller))
  ;[1 1 1] Waves
  (bind _result (Math|Integer|IncrementInt _current_wave)
    (:%20%20
      (Utilities|FlowControl|Sequence
        (:then_0
          (switch int _result
            (:1
              (Timeline|Wave%201 PlayFromStart
                (:Finished
                  (Default|UpdateWaves _ui (Variables|Default|GetCurrent%20Wave) true (not _returnvalue_2) :!label _label))
                (:Spawn%20Enemy
                  (CallFunction|SpawnEnemy :!label _label_2))))
            (:2
              (Timeline|Wave%202 PlayFromStart
                (:Finished
                  (goto _label))
                (:Spawn%20Enemy
                  (goto _label_2))))
            (:3
              (Timeline|Wave%203 PlayFromStart
                (:Finished
                  (goto _label))
                (:Spawn%20Enemy
                  (goto _label_2))))
            (:4
              (Timeline|Wave%204 PlayFromStart
                (:Finished
                  (goto _label))
                (:Spawn%20Enemy
                  (goto _label_2))))
            (:5
              (Timeline|Wave%205 PlayFromStart
                (:Finished
                  (goto _label))
                (:Spawn%20Enemy
                  (goto _label_2))))))
        (:then_1
          (if _returnvalue_2
            (Default|UpdateWaves _ui (Variables|Default|GetCurrent%20Wave) false false)))))))

(event Custom|Spawn%20Enemy
  (bind _enemy_spawns (Variables|Default|GetEnemy%20Spawns))
  (bind _outitem (Utilities|Array|Random _enemy_spawns))
  (bind _returnvalue (Transformation|GetActorTransform _outitem))
  ;[1 1 1] Waves
  (bind _returnvalue_2 (Game|SpawnActorfromClass "/Game/TopDown/Blueprints/BP_NPC_WizardEnemy.BP_NPC_WizardEnemy_C" (Math|Transform|MakeTransform (.location _returnvalue) (.rotation _returnvalue) "1.000000,1.000000,1.000000") "AdjustIfPossibleButAlwaysSpawn" "MultiplyWithRoot" 0 0))
  (Default|RevaluatePrimaryObjective _returnvalue_2 "NewEnumerator1"))

(event EventBeginPlay
  (bind _asbp_game_instance (Utilities|Casting|CastToBP_GameInstance (Game|GetGameInstance)))
  (bind _output_get (Variables|Default|SetGame%20Instance _asbp_game_instance))
  (Variables|/Game/BP/BP_GameInstance.BP_GameInstance_C|SetGame%20Controller _output_get self)
  (CallFunction|PlayBackgroundMusic)
  (Utilities|FlowControl|DelayUntilNextTick)
  (Variables|Default|SetTop%20Down%20Character (Variables|/Game/TopDown/Blueprints/BP_TopDownController.BP_TopDownController_C|GetTop%20Down%20Character (Variables|/Game/BP/BP_GameInstance.BP_GameInstance_C|GetTop%20Down%20Controller _output_get)))
  (bind _outactors (Actor|GetAllActorswithTag "enemytarget"))
  (Variables|Default|SetWizard%20Enemy%20Target (Utilities|Array|Get(acopy) _outactors)))

(event Collision|EventActorBeginOverlap
  (params (OtherActor :type Actor%20Object%20Reference)))

(event EventTick
  (params (DeltaSeconds :type Float%20%28single-precision%29)))

(fn ConstructionScript)

(fn CreatePopup
  (params (Show%20Button%202 :type Boolean) (Show%20Button%203 :type Boolean) (Show%20Button%204 :type Boolean) (Title :type Text) (Description :type Text) (Button%201%20Text :type Text) (Button%202%20Text :type Text) (Button%203%20Text :type Text) (Button%204%20Text :type Text))
  (bind _returnvalue (UserInterface|CreateWidget "/Game/UI/Widget_Popup.Widget_Popup_C" 0 Show%20Button%202 Show%20Button%203 Show%20Button%204 Title Description Button%201%20Text Button%202%20Text Button%203%20Text Button%204%20Text))
  (UserInterface|Viewport|AddtoViewport _returnvalue 1)
  (return _returnvalue))

(fn GetSelectedNPCs
  (bind _selected_npcs (Variables|Default|GetSelected%20NPCs))
  (return (Utilities|Array|IsNotEmpty _selected_npcs) _selected_npcs))