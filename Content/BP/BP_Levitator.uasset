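; BP_Levitator moves a referenced actor vertically in a repeating levitation cycle that starts on BeginPlay.
; A Levitate timeline drives a lerp between the world heights of StartZPos and EndZPosApex, keeping the actor's original X and Y.
; The play rate is the reciprocal of the duration variable, and the timeline restarts from the beginning after a delay each time it finishes.
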(event EventBeginPlay
  (Variables|Default|SetOrig%20Location (Transformation|GetActorLocation (Variables|Default|GetActor%20to%20Levitate)))
  (Components|Timeline|SetPlayRate (Variables|Default|GetLevitate) (Math|Float|Power (Variables|Default|GetLevitate%20Duration%20%28secs%29) -1.0))
  (bind _newtrack_1 (Timeline|Levitate PlayFromStart)
    (:Update
      (Transformation|SetActorLocation (Variables|Default|GetActor%20to%20Levitate) (Math|Vector|MakeVector (.x (Variables|Default|GetOrig%20Location)) (.y (Variables|Default|GetOrig%20Location)) (Math|Float|Lerp (.z (Transformation|GetWorldLocation (Variables|Default|GetStart%20Z%20Pos))) (.z (Transformation|GetWorldLocation (Variables|Default|GetEnd%20Z%20Pos%20%28Apex%29))) _newtrack_1)) false false))
    (:Finished
      (Utilities|FlowControl|Delay (Variables|Default|GetLevitate%20Delay%20%28secs%29))
      (Timeline|Levitate PlayFromStart))))

(fn ConstructionScript)