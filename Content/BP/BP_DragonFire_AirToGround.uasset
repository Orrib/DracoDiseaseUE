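; Airborne undead dragon hazard that breathes blue fire on the ground, chasing the player or an alternate actor horizontally at fixed height.
; Enabling fire starts a looping timer that briefly pauses it at a randomized interval, toggling collision, effect and movement together.
; The box repeatedly damages the player, with distance-scaled knockback when grounded, and damages tagged bushes, boxes and ground fire on entry.
; The dragon's hidden shadow follows the enabled state.
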(event OnComponentBeginOverlap(Box)
  (params (OverlappedComponent :type Primitive%20Component%20Object%20Reference) (OtherActor :type Actor%20Object%20Reference) (OtherComp :type Primitive%20Component%20Object%20Reference) (OtherBodyIndex :type Integer) (bFromSweep :type Boolean) (SweepResult :type Hit%20Result%20Structure%20%28by%20ref%29))
  (if (Actor|ActorHasTag OtherActor "player")
    (Math|Integer|IncrementInt (Variables|Default|GetColliders%20that%20detect%20player)
      (:%20%20
        (bind _returnvalue (Utilities|Time|SetTimerbyEvent (delegate Custom|CustomEvent) 0.6 true))
        (Variables|Default|SetFire%20Damage%20Timer _returnvalue)))
    (elif (Actor|ActorHasTag OtherActor "bush")
      (Game|Damage|ApplyDamage OtherActor 5.0 0 0 "/Game/BP/DamageType_Fire_Blue.DamageType_Fire_Blue_C" :!label _label)
      (elif (Actor|ActorHasTag OtherActor "box")
        (goto _label)
        (elif (Actor|ActorHasTag OtherActor "ground_fire")
          (goto _label))))))

(event OnComponentEndOverlap(Box)
  (params (OverlappedComponent :type Primitive%20Component%20Object%20Reference) (OtherActor :type Actor%20Object%20Reference) (OtherComp :type Primitive%20Component%20Object%20Reference) (OtherBodyIndex :type Integer))
  (if (Actor|ActorHasTag OtherActor "player")
    (bind _result (Math|Integer|DecrementInt (Variables|Default|GetColliders%20that%20detect%20player))
      (:%20%20
        (if (== _result 0)
          (Utilities|Time|ClearandInvalidateTimerbyHandle (Variables|Default|GetFire%20Damage%20Timer)))))))

(event Custom|Enable/Disable%20Fire
  (params (Enable? :type Boolean))
  (Variables|Default|SetFire%20State%20%28T/F%20=%20On/Off%29 Enable?)
  (Variables|Default|SetFire%20Paused false)
  (CallFunction|UpdateFireAppearance)
  (Actor|Tick|SetActorTickEnabled Enable?)
  (Class|PrimitiveComponent|SetCastHiddenShadow (Variables|Default|GetDragon_Undead_Flying) Enable?))

(event Custom|CustomEvent
  (if (> (Variables|Default|GetColliders%20that%20detect%20player) 0)
    (Game|Damage|ApplyDamage (Variables|Default|GetPlayer) (Variables|Default|GetDamage) 0 0 "/Game/BP/DamageType_Fire_Blue.DamageType_Fire_Blue_C")
    (Utilities|KnockbackCharacter (Variables|Default|GetPlayer) 1.0)))

(event Custom|CustomEvent_0
  (Variables|Default|SetFire%20Paused true)
  (CallFunction|UpdateFireAppearance)
  (Utilities|FlowControl|RetriggerableDelay 1.5)
  (if (Variables|Default|GetFire%20Paused)
    (Variables|Default|SetFire%20Paused false)
    (CallFunction|UpdateFireAppearance)))

(event Custom|Update%20Fire%20Appearance
  (Collision|SetCollisionEnabled (Variables|Default|GetBox) (select (and (Variables|Default|GetFire%20State%20%28T/F%20=%20On/Off%29) (not (Variables|Default|GetFire%20Paused))) "QueryOnly" "NoCollision"))
  (Variables|/Script/Engine.PrimitiveComponent|SetbGenerateOverlapEvents (Variables|Default|GetBox) (and (Variables|Default|GetFire%20State%20%28T/F%20=%20On/Off%29) (not (Variables|Default|GetFire%20Paused))))
  (Components|Activation|SetActive (Variables|Default|GetFire_blue) (and (Variables|Default|GetFire%20State%20%28T/F%20=%20On/Off%29) (not (Variables|Default|GetFire%20Paused))) false)
  (Actor|Tick|SetActorTickEnabled (and (Variables|Default|GetFire%20State%20%28T/F%20=%20On/Off%29) (not (Variables|Default|GetFire%20Paused))))
  (if (Variables|Default|GetFire%20State%20%28T/F%20=%20On/Off%29)
    (if (not (Utilities|Time|IsValidTimerHandle (Variables|Default|GetFire%20Pause%20Timer)))
      (bind _returnvalue (Utilities|Time|SetTimerbyEvent (delegate Custom|CustomEvent_0) (Math|Random|RandomFloatinRange 4.0 6.0) true))
      (Variables|Default|SetFire%20Pause%20Timer _returnvalue))
    (else
      (Utilities|Time|ClearandInvalidateTimerbyHandle (Variables|Default|GetFire%20Pause%20Timer))
      (Variables|Default|SetFire%20Paused false))))

(event EventBeginPlay
  (bind _asbp_top_down_character (Utilities|Casting|CastToBP_TopDownCharacter (Game|GetPlayerCharacter 0)))
  (Variables|Default|SetPlayer _asbp_top_down_character)
  (CallFunction|Enable/DisableFire false))

(event Collision|EventActorBeginOverlap
  (params (OtherActor :type Actor%20Object%20Reference)))

(event EventTick
  (params (DeltaSeconds :type Float%20%28single-precision%29))
  (bind _returnvalue (Transformation|GetActorLocation))
  (bind _returnvalue_2 (Utilities|Time|GetWorldDeltaSeconds))
  (bind _follow_alt_actor (Variables|Default|GetFollow%20Alt%20Actor))
  (bind _speed (Variables|Default|GetSpeed))
  (bind _alt_actor (Variables|Default|GetAlt%20Actor))
  (bind _player (Variables|Default|GetPlayer))
  (bind _returnvalue_3 (select _follow_alt_actor _alt_actor _player))
  (bind _returnvalue_4 (Transformation|GetActorLocation _returnvalue_3))
  (bind _returnvalue_5 (- _returnvalue_4 _returnvalue))
  (bind _returnvalue_6 (Math|Vector|Normalize _returnvalue_5))
  (bind _returnvalue_7 (* _returnvalue_6 _speed _returnvalue_2))
  (bind _returnvalue_8 (+ _returnvalue _returnvalue_7))
  (Transformation|SetActorLocation (Math|Vector|MakeVector (.x _returnvalue_8) (.y _returnvalue_8) (.z (Transformation|GetActorLocation))) false false))

(fn ConstructionScript)