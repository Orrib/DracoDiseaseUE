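; BP_Mover is a utility Blueprint that moves a referenced ActorToMove from its Start component's world location to its End component's.
; Move plays a Timeline from the start, with play rate set to the inverse of MoveTime to scale its duration.
; Each update lerps the actor's location by the track value without sweeping, and completion broadcasts OnMoveComplete.
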(event Custom|Move
  (Components|Timeline|SetPlayRate (Variables|Default|GetTimeline) (Math|Float|Power (Variables|Default|GetMove%20Time) -1.0))
  (bind _newtrack_0 (Timeline|Timeline PlayFromStart)
    (:Update
      (Transformation|SetActorLocation (Variables|Default|GetActor%20To%20Move) (Math|Vector|Lerp(Vector) (Transformation|GetWorldLocation (Variables|Default|GetStart)) (Transformation|GetWorldLocation (Variables|Default|GetEnd)) _newtrack_0) false false))
    (:Finished
      (Default|CallOnMoveComplete))))

(event EventBeginPlay)

(event Collision|EventActorBeginOverlap
  (params (OtherActor :type Actor%20Object%20Reference)))

(event EventTick
  (params (DeltaSeconds :type Float%20%28single-precision%29)))

(fn ConstructionScript)