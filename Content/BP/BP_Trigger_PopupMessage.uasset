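; Trigger actor that shows a configurable popup message when an actor tagged "player" overlaps it.
; It asks the GameController held by BP_GameInstance to create the popup, passing title, description and up to four button labels.
; It can pause the game until the first button is clicked, then unpause.
; With OnlyShowOnce set, it destroys itself afterward, or immediately when not pausing.
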(event Custom|CustomEvent
  (Game|SetGamePaused false)
  (if (Variables|Default|GetOnly%20Show%20Once)
    (Actor|DestroyActor)))

(event EventBeginPlay
  (bind _asbp_game_instance (Utilities|Casting|CastToBP_GameInstance (Game|GetGameInstance)))
  (Variables|Default|SetBP%20Game%20Instance _asbp_game_instance))

(event Collision|EventActorBeginOverlap
  (params (OtherActor :type Actor%20Object%20Reference))
  (if (Actor|ActorHasTag OtherActor "player")
    (bind _created_popup_widget (Default|CreatePopup (Variables|/Game/BP/BP_GameInstance.BP_GameInstance_C|GetGame%20Controller (Variables|Default|GetBP%20Game%20Instance)) (Variables|Default|GetShow%20Button%202) (Variables|Default|GetShow%20Button%203) (Variables|Default|GetShow%20Button%204) (Variables|Default|GetTitle) (Variables|Default|GetDescription) (Variables|Default|GetButton%201%20Text) (Variables|Default|GetButton%202%20Text) (Variables|Default|GetButton%203%20Text) (Variables|Default|GetButton%204%20Text)))
    (if (Variables|Default|GetPause%20Game%20for%20popup)
      (Game|SetGamePaused true)
      (EventDispatchers|BindEventtoOnClickButton1 _created_popup_widget (delegate Custom|CustomEvent))
      (elif (Variables|Default|GetOnly%20Show%20Once)
        (Actor|DestroyActor)))))

(event EventTick
  (params (DeltaSeconds :type Float%20%28single-precision%29)))

(fn ConstructionScript)