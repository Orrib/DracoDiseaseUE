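; BP_CrowdMember is a crowd actor with a Paper2D flipbook that travels once along an assigned CrowdTrailSpline, then destroys itself.
; On BeginPlay, if the spline is valid, a timeline moves the actor along it at constant velocity without sweeping.
; Timeline play rate is proportional to spline length times Speed, and the flipbook plays at six times that rate, tying animation to movement.
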(event EventBeginPlay
  (bind _speed (Variables|Default|GetSpeed))
  (bind _crowd_trail_spline (Variables|Default|GetCrowd%20Trail%20Spline))
  (bind _returnvalue (Spline|GetSplineLength _crowd_trail_spline))
  (bind _returnvalue_2 (* _returnvalue _speed 0.0001))
  (Utilities|IsValid _crowd_trail_spline
    (:Is%20Valid
      (Components|Timeline|SetPlayRate (Variables|Default|GetTimeline) _returnvalue_2)
      (Components|Timeline|SetPlayRate (Variables|Default|GetPaperFlipbook) (* _returnvalue_2 6.0))
      (bind _newtrack_0 (Timeline|Timeline PlayFromStart)
        (:Update
          (Transformation|SetActorLocation (Spline|GetLocationatTime (Variables|Default|GetCrowd%20Trail%20Spline) _newtrack_0 "World" true) false false))
        (:Finished
          (Actor|DestroyActor))))))

(fn ConstructionScript)