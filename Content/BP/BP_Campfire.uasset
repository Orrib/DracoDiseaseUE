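; BP_Campfire is a campfire that can be switched on or off and burns and knocks back characters that hit it.
; The TurnFireOnOff event stores the state, updates light, fire visibility and damage collider collision, and fades audio in when lit.
; The construction script applies the same appearance update.
; Collider hits on npc or player tagged actors deal fire point damage and launch Characters away, scaled inversely by mass.
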(event OnComponentHit(FireDamageCollider)
  (params (HitComponent :type Primitive%20Component%20Object%20Reference) (OtherActor :type Actor%20Object%20Reference) (OtherComp :type Primitive%20Component%20Object%20Reference) (NormalImpulse :type Vector :default "0, 0, 0") (Hit :type Hit%20Result%20Structure%20%28by%20ref%29))
  (bind _returnvalue (Transformation|GetActorLocation OtherActor))
  (bind _scene (Variables|Default|GetScene))
  (bind _returnvalue_2 (Transformation|GetWorldLocation _scene))
  (bind _returnvalue_3 (Math|Vector|GetUnitDirection(Vector) _returnvalue_2 _returnvalue))
  (if (or (Actor|ActorHasTag OtherActor "npc") (Actor|ActorHasTag OtherActor "player"))
    (Game|Damage|ApplyPointDamage OtherActor (Variables|Default|GetDamage) _returnvalue_3 (Collision|MakeHitResult false false 0.0 0.0 "0, 0, 0" "0, 0, 0" "0,0,1" "0,0,1" 0 0) 0 self "/Game/BP/DamageType_Fire_Orange.DamageType_Fire_Orange_C")
    (bind _ascharacter (Utilities|Casting|CastToCharacter OtherActor))
    ;[1 1 1] Apply Impulse, accountinmg for mass
    (Character|LaunchCharacter _ascharacter (* _returnvalue_3 (/ 3e+04 (Variables|/Script/Engine.CharacterMovementComponent|GetMass (Variables|/Script/Engine.Character|GetCharacterMovement _ascharacter)))) true true)))

(event Custom|Turn%20Fire%20On/Off%20%28T/F%29
  (params (On/Off :type Boolean))
  (bind _output_get (Variables|Default|SetFire%20On/Off On/Off))
  (CallFunction|UpdateFireAppearance)
  (if _output_get
    (Audio|Components|Audio|FadeIn (Variables|Default|GetAudio) 2.0 1.0 0.0 "Linear" :!class /Script/Engine.AudioComponent)))

(event Custom|Update%20Fire%20Appearance
  (bind _fire_on_off (Variables|Default|GetFire%20On/Off))
  (Rendering|SetVisibility (Variables|Default|GetPointLight) _fire_on_off false)
  (Rendering|SetVisibility (Variables|Default|GetFire) _fire_on_off false)
  (Collision|SetCollisionEnabled (Variables|Default|GetFire%20Damage%20Collider) (select _fire_on_off "QueryAndPhysics" "NoCollision")))

(event EventBeginPlay
  (CallFunction|TurnFireOn/Off(T/F) (Variables|Default|GetFire%20On/Off)))

(fn ConstructionScript
  (CallFunction|UpdateFireAppearance))