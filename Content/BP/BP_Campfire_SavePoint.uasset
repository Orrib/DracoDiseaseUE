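; BP_Campfire_SavePoint is a campfire checkpoint that lights up and shows a "Progress Saved" message when the player reaches it.
; A sphere overlap passes through a Gate and checks for the "player" tag, then closes the Gate so it fires only once.
; It then turns the fire on and sends the timed message through the GameInstance's GameController; no save-game write happens in this graph.
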(event OnComponentBeginOverlap(Sphere9)
  (params (OverlappedComponent :type Primitive%20Component%20Object%20Reference) (OtherActor :type Actor%20Object%20Reference) (OtherComp :type Primitive%20Component%20Object%20Reference) (OtherBodyIndex :type Integer) (bFromSweep :type Boolean) (SweepResult :type Hit%20Result%20Structure%20%28by%20ref%29))
  (Utilities|FlowControl|Gate false :!label _label
    (:Exit
      (if (Actor|ActorHasTag OtherActor "player")
        (Utilities|FlowControl|Sequence
          (:then_0
            (goto _label Close))
          (:then_1
            (CallFunction|TurnFireOn/Off(T/F) true)
            (bind _asbp_game_instance (Utilities|Casting|CastToBP_GameInstance (Game|GetGameInstance)))
            (Default|StartMessage (Variables|/Game/BP/BP_GameInstance.BP_GameInstance_C|GetGame%20Controller _asbp_game_instance) "Progress Saved" "NewEnumerator0" 3.0)))))))

(event EventBeginPlay
  (|CallParentFunction) ; This node is disabled and will not be called.\nDrag off pins to build functionality.
)

(event Collision|EventActorBeginOverlap
  (params (OtherActor :type Actor%20Object%20Reference))
  (|CallParentFunction OtherActor) ; This node is disabled and will not be called.\nDrag off pins to build functionality.
)

(event EventTick
  (params (DeltaSeconds :type Float%20%28single-precision%29))
  (|CallParentFunction DeltaSeconds) ; This node is disabled and will not be called.\nDrag off pins to build functionality.
)

(fn ConstructionScript
  (|CallParentFunction))