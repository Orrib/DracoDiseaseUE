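; AI controller for the dragon enemy that switches between spline patrol flight and swooping at spotted targets.
; In Flying mode, a reciprocal-rate timeline samples the game controller's flying spline and Tick teleports the dragon to that point.
; When an enemy is spotted, a second timeline lerps the dragon to the target's captured location.
; On finish it returns to Flying and clears the dragon's swoop hit list.
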(event Custom|On%20Enemy%20Spotted
  (params (Target :type Actor%20Object%20Reference))
  (Variables|Default|SetTarget Target)
  (Variables|Default|SetTarget%20Spotted%20Location (Transformation|GetActorLocation Target))
  (Variables|Default|SetDragon%20Start%20Location (Transformation|GetActorLocation (Variables|Default|GetCharacter%20-%20BP%20Dragon%20Enemy)))
  (CallFunction|ChangeDragonMode "NewEnumerator1"))

(event Custom|Change%20Dragon%20Mode
  (params (New%20Mode :type Enum_DragonMode%20Enum :default "NewEnumerator0"))
  (bind _output_get (Variables|Default|SetDragon%20Mode New%20Mode))
  (switch Utilities|FlowControl|Switch|SwitchonEnum_DragonMode _output_get
    (:NewEnumerator0
      (Audio|Components|Audio|Stop (Variables|Default|GetSwoop%20Target))
      (Pawn|Components|CharacterMovement|SetMovementMode (Variables|/Script/Engine.Character|GetCharacterMovement (Variables|Default|GetCharacter%20-%20BP%20Dragon%20Enemy)) "MOVE_Flying" 0)
      (Components|Timeline|SetPlayRate (Variables|Default|GetSpline%20Update) (Math|Float|Power (Variables|Default|GetFlying%20Patrol%20Time) -1.0))
      (bind _newtrack_0 (Timeline|Spline%20Update Play)
        (:Update
          (Variables|Default|SetTarget%20Spline%20Point (Spline|GetLocationatTime (Variables|/Game/BP/BP_DragonFlyingSpline.BP_DragonFlyingSpline_C|GetSpline (Variables|Default|GetDragon%20Flying%20Spline)) _newtrack_0 "World" false)))))
    (:NewEnumerator1
      (Audio|Components|Audio|Stop (Variables|Default|GetSpline%20Update))
      (Components|Timeline|SetPlayRate (Variables|Default|GetSwoop%20Target) (Math|Float|Power (Variables|Default|GetSwoop%20Time) -1.0))
      (bind _newtrack_0_2 (Timeline|Swoop%20Target PlayFromStart)
        (:Update
          (Transformation|SetActorLocation (Variables|Default|GetCharacter%20-%20BP%20Dragon%20Enemy) (Math|Vector|Lerp(Vector) (Variables|Default|GetDragon%20Start%20Location) (Variables|Default|GetTarget%20Spotted%20Location) _newtrack_0_2) false false))
        (:Finished
          (CallFunction|ChangeDragonMode "NewEnumerator0")
          (Utilities|Array|Clear (Variables|/Game/BP/BP_DragonEnemy.BP_DragonEnemy_C|GetSwoop%20Hit%20Actors (Variables|Default|GetCharacter%20-%20BP%20Dragon%20Enemy))))))))

(event EventBeginPlay
  (bind _asbp_dragon_enemy (Utilities|Casting|CastToBP_DragonEnemy (Pawn|GetControlledPawn)))
  (Variables|Default|SetCharacter%20-%20BP%20Dragon%20Enemy _asbp_dragon_enemy)
  (Utilities|FlowControl|DelayUntilNextTick)
  (Utilities|FlowControl|DelayUntilNextTick)
  (CallFunction|ChangeDragonMode "NewEnumerator0")
  (bind _asbp_game_instance (Utilities|Casting|CastToBP_GameInstance (Game|GetGameInstance)))
  (Variables|Default|SetDragon%20Flying%20Spline (Variables|/Game/BP/BP_GameController.BP_GameController_C|GetDragon%20Flying%20Spline (Variables|/Game/BP/BP_GameInstance.BP_GameInstance_C|GetGame%20Controller _asbp_game_instance))))

(event EventTick
  (params (DeltaSeconds :type Float%20%28single-precision%29))
  (switch Utilities|FlowControl|Switch|SwitchonEnum_DragonMode (Variables|Default|GetDragon%20Mode)
    (:NewEnumerator0
      (Transformation|SetActorLocation (Variables|Default|GetCharacter%20-%20BP%20Dragon%20Enemy) (Variables|Default|GetTarget%20Spline%20Point) false false))))

(fn ConstructionScript)