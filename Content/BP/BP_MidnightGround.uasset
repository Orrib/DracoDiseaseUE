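; BP_MidnightGround is a ground piece for Midnight mode that reports which edge or corner the player enters and removes itself once left behind.
; Directional triggers filter for the "player" tag and pass the tile to BP_MidnightModeController, found at BeginPlay.
; The West trigger's call is disconnected, so that side reports nothing.
; Leaving DetectionTrigger starts a five-second self-destruct timer, which re-entering cancels.
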(event OnComponentBeginOverlap(TriggerNorth)
  (params (OverlappedComponent :type Primitive%20Component%20Object%20Reference) (OtherActor :type Actor%20Object%20Reference) (OtherComp :type Primitive%20Component%20Object%20Reference) (OtherBodyIndex :type Integer) (bFromSweep :type Boolean) (SweepResult :type Hit%20Result%20Structure%20%28by%20ref%29))
  (Utilities|IsPlayer? OtherActor
    (:true
      (Default|OnNorthTriggerEnter (Variables|Default|GetMidnight%20Mode%20COntroller) self))))

(event OnComponentBeginOverlap(TriggerSouth)
  (params (OverlappedComponent :type Primitive%20Component%20Object%20Reference) (OtherActor :type Actor%20Object%20Reference) (OtherComp :type Primitive%20Component%20Object%20Reference) (OtherBodyIndex :type Integer) (bFromSweep :type Boolean) (SweepResult :type Hit%20Result%20Structure%20%28by%20ref%29))
  (Utilities|IsPlayer? OtherActor
    (:true
      (Default|OnSouthTriggerEnter (Variables|Default|GetMidnight%20Mode%20COntroller) self))))

(event OnComponentBeginOverlap(TriggerWest)
  (params (OverlappedComponent :type Primitive%20Component%20Object%20Reference) (OtherActor :type Actor%20Object%20Reference) (OtherComp :type Primitive%20Component%20Object%20Reference) (OtherBodyIndex :type Integer) (bFromSweep :type Boolean) (SweepResult :type Hit%20Result%20Structure%20%28by%20ref%29)))

(event OnComponentBeginOverlap(TriggerEast)
  (params (OverlappedComponent :type Primitive%20Component%20Object%20Reference) (OtherActor :type Actor%20Object%20Reference) (OtherComp :type Primitive%20Component%20Object%20Reference) (OtherBodyIndex :type Integer) (bFromSweep :type Boolean) (SweepResult :type Hit%20Result%20Structure%20%28by%20ref%29))
  (Utilities|IsPlayer? OtherActor
    (:true
      (Default|OnEastTriggerEnter (Variables|Default|GetMidnight%20Mode%20COntroller) self))))

(event OnComponentEndOverlap(DetectionTrigger)
  (params (OverlappedComponent :type Primitive%20Component%20Object%20Reference) (OtherActor :type Actor%20Object%20Reference) (OtherComp :type Primitive%20Component%20Object%20Reference) (OtherBodyIndex :type Integer))
  ;[1 1 1] Detection Trigger
  (Utilities|IsPlayer? OtherActor
    (:true
      ;;[1 1 1] self Destruct after 3 seconds
      (bind _returnvalue (Utilities|Time|SetTimerbyEvent (delegate Custom|CustomEvent) 5.0))
      (Variables|Default|SetSelf%20Destruct%20Timer _returnvalue))))

(event OnComponentBeginOverlap(DetectionTrigger)
  (params (OverlappedComponent :type Primitive%20Component%20Object%20Reference) (OtherActor :type Actor%20Object%20Reference) (OtherComp :type Primitive%20Component%20Object%20Reference) (OtherBodyIndex :type Integer) (bFromSweep :type Boolean) (SweepResult :type Hit%20Result%20Structure%20%28by%20ref%29))
  ;[1 1 1] Detection Trigger
  (Utilities|IsPlayer? OtherActor
    (:true
      (Utilities|Time|ClearandInvalidateTimerbyHandle (Variables|Default|GetSelf%20Destruct%20Timer)))))

(event OnComponentBeginOverlap(TriggerSW)
  (params (OverlappedComponent :type Primitive%20Component%20Object%20Reference) (OtherActor :type Actor%20Object%20Reference) (OtherComp :type Primitive%20Component%20Object%20Reference) (OtherBodyIndex :type Integer) (bFromSweep :type Boolean) (SweepResult :type Hit%20Result%20Structure%20%28by%20ref%29))
  (Utilities|IsPlayer? OtherActor
    (:true
      (Default|OnSWTriggerEnter (Variables|Default|GetMidnight%20Mode%20COntroller) self))))

(event OnComponentBeginOverlap(TriggerNE)
  (params (OverlappedComponent :type Primitive%20Component%20Object%20Reference) (OtherActor :type Actor%20Object%20Reference) (OtherComp :type Primitive%20Component%20Object%20Reference) (OtherBodyIndex :type Integer) (bFromSweep :type Boolean) (SweepResult :type Hit%20Result%20Structure%20%28by%20ref%29))
  (Utilities|IsPlayer? OtherActor
    (:true
      (Default|OnNETriggerEnter (Variables|Default|GetMidnight%20Mode%20COntroller) self))))

(event OnComponentBeginOverlap(TriggerNW)
  (params (OverlappedComponent :type Primitive%20Component%20Object%20Reference) (OtherActor :type Actor%20Object%20Reference) (OtherComp :type Primitive%20Component%20Object%20Reference) (OtherBodyIndex :type Integer) (bFromSweep :type Boolean) (SweepResult :type Hit%20Result%20Structure%20%28by%20ref%29))
  (Utilities|IsPlayer? OtherActor
    (:true
      (Default|OnNWTriggerEnter (Variables|Default|GetMidnight%20Mode%20COntroller) self))))

(event OnComponentBeginOverlap(TriggerSE)
  (params (OverlappedComponent :type Primitive%20Component%20Object%20Reference) (OtherActor :type Actor%20Object%20Reference) (OtherComp :type Primitive%20Component%20Object%20Reference) (OtherBodyIndex :type Integer) (bFromSweep :type Boolean) (SweepResult :type Hit%20Result%20Structure%20%28by%20ref%29))
  (Utilities|IsPlayer? OtherActor
    (:true
      (Default|OnSETriggerEnter (Variables|Default|GetMidnight%20Mode%20COntroller) self))))

(event Custom|CustomEvent
  ;[1 1 1] Detection Trigger
  ;;[1 1 1] self Destruct after 3 seconds
  (Actor|DestroyActor))

(event EventBeginPlay
  (bind _returnvalue (Actor|GetActorOfClass "/Game/BP/BP_MidnightModeController.BP_MidnightModeController_C"))
  (Variables|Default|SetMidnight%20Mode%20COntroller _returnvalue))

(event Collision|EventActorBeginOverlap
  (params (OtherActor :type Actor%20Object%20Reference)))

(event EventTick
  (params (DeltaSeconds :type Float%20%28single-precision%29)))

(fn ConstructionScript)