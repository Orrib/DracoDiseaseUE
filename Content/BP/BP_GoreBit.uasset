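; BP_GoreBit is a gore piece that varies its look each time it is constructed.
; Its construction script multiplies the Cube component's relative scale by a random factor between 1 and 2, with the range bounds entered in reverse.
; It then assigns the Cube's first material slot a random pick from the PossibleMaterials array.
; The event graph holds no active logic.
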(event EventBeginPlay)

(fn ConstructionScript
  (CallFunction|RadnomizeScale)
  (CallFunction|SetMaterial))

(fn RadnomizeScale
  (bind _cube (Variables|Default|GetCube))
  (Transformation|SetRelativeScale3D _cube (* (Variables|/Script/Engine.SceneComponent|GetRelativeScale3D _cube) (Math|Random|RandomFloatinRange 2.0 1.0))))

(fn SetMaterial
  (Rendering|Material|SetMaterial (Variables|Default|GetCube) 0 (.OutItem (Utilities|Array|Random (Variables|Default|GetPossible%20Materials)))))