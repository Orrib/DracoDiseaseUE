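; BP_CrowdMember_GuardNewer is a guard crowd NPC that walks or runs along a CrowdTrailSpline and destroys itself when the trail ends.
; BeginPlay jumps the PaperZD animation to Walk or Run and lowers the soldier AnimInstance's play rate for runners.
; A timeline, its rate scaled by spline length and Speed, drives the actor's location along the spline.
; The construction script optionally mirrors the Spine renderer's X scale to set facing.
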(event Collision|EventActorBeginOverlap
  (params (OtherActor :type Actor%20Object%20Reference))
  (|CallParentFunction OtherActor) ; This node is disabled and will not be called.\nDrag off pins to build functionality.
)

(event EventTick
  (params (DeltaSeconds :type Float%20%28single-precision%29))
  (|CallParentFunction DeltaSeconds) ; This node is disabled and will not be called.\nDrag off pins to build functionality.
)

(event EventBeginPlay
  (bind _crowd_trail_spline (Variables|Default|GetCrowd%20Trail%20Spline))
  (bind _paperzdanimation (Variables|Default|GetPaperZDAnimation))
  (bind _runner_ (Variables|Default|GetRunner?))
  (bind _animinstance (Variables|/Script/PaperZD.PaperZDAnimationComponent|GetAnimInstance _paperzdanimation))
  (|CallParentFunction)
  (Class|PaperZDAnimInstance|JumptoNode _animinstance (select _runner_ "Run" "Walk") "None")
  (Utilities|FlowControl|Sequence
    (:then_0
      (bind _asabp_static_npc_basic_soldier (Utilities|Casting|CastToABP_StaticNPC_BasicSoldier _animinstance))
      (Variables|/Game/Animation/ABP_StaticNPC_BasicSoldier.ABP_StaticNPC_BasicSoldier_C|SetPlay%20Rate _asabp_static_npc_basic_soldier (select _runner_ 0.7 1.0)))
    (:then_1
      (Utilities|IsValid _crowd_trail_spline
        (:Is%20Valid
          (Components|Timeline|SetPlayRate (Variables|Default|GetTimeline) (* (Spline|GetSplineLength _crowd_trail_spline) (Variables|Default|GetSpeed) 0.0001))
          (bind _newtrack_0 (Timeline|Timeline PlayFromStart)
            (:Update
              (Transformation|SetActorLocation (Spline|GetLocationatTime (Variables|Default|GetCrowd%20Trail%20Spline) _newtrack_0 "World" true) false false))
            (:Finished
              (Actor|DestroyActor))))))))

(fn ConstructionScript
  (bind _spineskeletonrenderer (Variables|Default|GetSpineSkeletonRenderer))
  (bind _relativescale3d (Variables|/Script/Engine.SceneComponent|GetRelativeScale3D _spineskeletonrenderer))
  (|CallParentFunction)
  (if (Variables|Default|GetFace%20Left%20%28T/F%20=%20Left/Right%29)
    (Transformation|SetRelativeScale3D _spineskeletonrenderer (Math|Vector|MakeVector (* (.x _relativescale3d) -1.0) (.y _relativescale3d) (.z _relativescale3d)))))