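; Controller for Midnight Mode, a timed escape sequence where the player is constantly pushed forward through endless terrain until the demo's victory popup.
; BeginPlay adjusts UI, input, speed and camera, starts looping enemy spawns in an arc ahead, and schedules story messages and the ending.
; Eight directional trigger events grow the ground by spawning random tiles at unoccupied coordinates in a grid map.
; The popup offers checkpoint restarts, Survival Mode or quitting.
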(event Custom|On%20SE%20Trigger%20Enter
  (params (Input%20Midnight%20Ground :type BP%20Midnight%20Ground%20Object%20Reference))
  (bind _grid_coord (Variables|/Game/BP/BP_MidnightGround.BP_MidnightGround_C|GetGrid%20Coord Input%20Midnight%20Ground))
  (bind _returnvalue (+ (.x _grid_coord) 1.0))
  (bind _returnvalue_2 (- (.y _grid_coord) 1.0))
  (bind _returnvalue_3 (Math|Vector2D|MakeVector2D _returnvalue _returnvalue_2))
  (if (not (Utilities|Map|Contains (Variables|Default|GetMidnight%20Ground%20Grid) _returnvalue_3))
    (CallFunction|SpawnMidnightGround (+ (Transformation|GetActorLocation Input%20Midnight%20Ground) (Math|Vector|MakeVector -1e+04 1e+04 0.0)) _returnvalue_3)))

(event Custom|On%20North%20Trigger%20Enter
  (params (Input%20Midnight%20Ground :type BP%20Midnight%20Ground%20Object%20Reference))
  (bind _grid_coord (Variables|/Game/BP/BP_MidnightGround.BP_MidnightGround_C|GetGrid%20Coord Input%20Midnight%20Ground))
  (bind _returnvalue (+ (.y _grid_coord) 1.0))
  (bind _returnvalue_2 (Math|Vector2D|MakeVector2D (.x _grid_coord) _returnvalue))
  (if (not (Utilities|Map|Contains (Variables|Default|GetMidnight%20Ground%20Grid) _returnvalue_2))
    (CallFunction|SpawnMidnightGround (+ (Transformation|GetActorLocation Input%20Midnight%20Ground) (Math|Vector|MakeVector 1e+04 0.0 0.0)) _returnvalue_2)))

(event Custom|On%20NE%20Trigger%20Enter
  (params (Input%20Midnight%20Ground :type BP%20Midnight%20Ground%20Object%20Reference))
  (bind _grid_coord (Variables|/Game/BP/BP_MidnightGround.BP_MidnightGround_C|GetGrid%20Coord Input%20Midnight%20Ground))
  (bind _returnvalue (+ (.x _grid_coord) 1.0))
  (bind _returnvalue_2 (+ (.y _grid_coord) 1.0))
  (bind _returnvalue_3 (Math|Vector2D|MakeVector2D _returnvalue _returnvalue_2))
  (if (not (Utilities|Map|Contains (Variables|Default|GetMidnight%20Ground%20Grid) _returnvalue_3))
    (CallFunction|SpawnMidnightGround (+ (Transformation|GetActorLocation Input%20Midnight%20Ground) (Math|Vector|MakeVector 1e+04 1e+04 0.0)) _returnvalue_3)))

(event Custom|OnClickButton1_Event
  (bind _top_down_character (Variables|Default|GetTop%20Down%20Character))
  (bind _top_down_controller (Variables|/Game/TopDown/Blueprints/BP_TopDownCharacter.BP_TopDownCharacter_C|GetTop%20Down%20Controller _top_down_character))
  (bind _game_instance (Variables|/Game/TopDown/Blueprints/BP_TopDownController.BP_TopDownController_C|GetGame%20Instance _top_down_controller))
  ;[1 1 1] button 2 - restart demo
  (Variables|/Game/BP/BP_GameSave.BP_GameSave_C|SetCheckpoint%20-%20Battlefield%20Opening (Variables|/Game/BP/BP_GameInstance.BP_GameInstance_C|GetSave%20Game%20Instance _game_instance) "NewEnumerator1")
  (Default|SaveGame _game_instance)
  (Game|SetGamePaused false)
  (Default|OpenLevel(ByReference) _game_instance "/Game/Maps/Map_Battlefield.Map_Battlefield"))

(event Custom|On%20SW%20Trigger%20Enter
  (params (Input%20Midnight%20Ground :type BP%20Midnight%20Ground%20Object%20Reference))
  (bind _grid_coord (Variables|/Game/BP/BP_MidnightGround.BP_MidnightGround_C|GetGrid%20Coord Input%20Midnight%20Ground))
  (bind _returnvalue (- (.x _grid_coord) 1.0))
  (bind _returnvalue_2 (- (.y _grid_coord) 1.0))
  (bind _returnvalue_3 (Math|Vector2D|MakeVector2D _returnvalue _returnvalue_2))
  (if (not (Utilities|Map|Contains (Variables|Default|GetMidnight%20Ground%20Grid) _returnvalue_3))
    (CallFunction|SpawnMidnightGround (+ (Transformation|GetActorLocation Input%20Midnight%20Ground) (Math|Vector|MakeVector -1e+04 -1e+04 0.0)) _returnvalue_3)))

(event Custom|CustomEvent
  (bind _top_down_character (Variables|Default|GetTop%20Down%20Character))
  (bind _top_down_controller (Variables|/Game/TopDown/Blueprints/BP_TopDownCharacter.BP_TopDownCharacter_C|GetTop%20Down%20Controller _top_down_character))
  (bind _game_instance (Variables|/Game/TopDown/Blueprints/BP_TopDownController.BP_TopDownController_C|GetGame%20Instance _top_down_controller))
  ;[1 1 1] button 1 - restart commander fight
  (Variables|/Game/BP/BP_GameSave.BP_GameSave_C|SetCheckpoint%20-%20Battlefield%20Opening (Variables|/Game/BP/BP_GameInstance.BP_GameInstance_C|GetSave%20Game%20Instance _game_instance) "NewEnumerator2")
  (Default|SaveGame _game_instance)
  (Game|SetGamePaused false)
  (Default|OpenLevel(ByReference) _game_instance "/Game/Maps/Map_Battlefield.Map_Battlefield"))

(event Custom|Start%20Spawning%20Enemies
  (bind _spawn_distance_from_player (Variables|Default|GetSpawn%20Distance%20From%20Player))
  (bind _top_down_character (Variables|Default|GetTop%20Down%20Character))
  (bind _returnvalue (Transformation|GetActorLocation _top_down_character))
  (Utilities|FlowControl|Delay (Math|Random|RandomFloatinRange 0.3 1.0) :!label _label)
  (bind _output_get (Variables|Default|Set%28temp%29%20Spawn%20Outlier%20NPC? (Math|Random|RandomBoolwithWeight 0.35)))
  (Game|SpawnActorfromClass (Utilities|Array|Get(acopy) (Variables|Default|GetWizard%20Enemy%20Choices) (select (Math|Random|RandomBoolwithWeight 0.8) 1 (select (Variables|Default|Get%28temp%29%20Spawn%20Outlier%20NPC?) 1 0))) (Math|Transform|MakeTransform (Math|Vector|MakeVector (+ (* (Math|Trig|Cos(Degrees) (select _output_get (Math|Random|RandomFloatinRange 65.0 115.0) (Math|Random|RandomFloatinRange 83.0 97.0))) _spawn_distance_from_player) (.x _returnvalue)) (+ (* (Math|Trig|Sin(Degrees) (select _output_get (Math|Random|RandomFloatinRange 65.0 115.0) (Math|Random|RandomFloatinRange 83.0 97.0))) _spawn_distance_from_player) (.y _returnvalue)) (.z _returnvalue)) "0, 0, 0" "1.000000,1.000000,1.000000") "AdjustIfPossibleButDontSpawnIfColliding" "MultiplyWithRoot" 0 "NewEnumerator0" "/Game/BP/BP_Pickup_RandomDrop.BP_Pickup_RandomDrop_C" 0 4.5e+02 false 0)
  (goto _label))

(event Custom|CustomEvent_1
  ;[1 1 1] Button 3 - survival mode
  (Variables|/Game/BP/BP_GameSave.BP_GameSave_C|SetCheckpoint%20-%20Survival%20Mode (Variables|/Game/BP/BP_GameInstance.BP_GameInstance_C|GetSave%20Game%20Instance (Variables|Default|GetGame%20Instance)) "NewEnumerator1")
  (Default|StartSurvivalMode (Variables|/Game/BP/BP_GameInstance.BP_GameInstance_C|GetGame%20Controller (Variables|/Game/TopDown/Blueprints/BP_TopDownController.BP_TopDownController_C|GetGame%20Instance (Variables|/Game/TopDown/Blueprints/BP_TopDownCharacter.BP_TopDownCharacter_C|GetTop%20Down%20Controller (Variables|Default|GetTop%20Down%20Character))))))

(event Custom|On%20East%20Trigger%20Enter
  (params (Input%20Midnight%20Ground :type BP%20Midnight%20Ground%20Object%20Reference))
  (bind _grid_coord (Variables|/Game/BP/BP_MidnightGround.BP_MidnightGround_C|GetGrid%20Coord Input%20Midnight%20Ground))
  (bind _returnvalue (+ (.x _grid_coord) 1.0))
  (bind _returnvalue_2 (Math|Vector2D|MakeVector2D _returnvalue (.y _grid_coord)))
  (if (not (Utilities|Map|Contains (Variables|Default|GetMidnight%20Ground%20Grid) _returnvalue_2))
    (CallFunction|SpawnMidnightGround (+ (Transformation|GetActorLocation Input%20Midnight%20Ground) (Math|Vector|MakeVector 0.0 1e+04 0.0)) _returnvalue_2)))

(event Custom|On%20West%20Trigger%20Enter
  (params (Input%20Midnight%20Ground :type BP%20Midnight%20Ground%20Object%20Reference))
  (bind _grid_coord (Variables|/Game/BP/BP_MidnightGround.BP_MidnightGround_C|GetGrid%20Coord Input%20Midnight%20Ground))
  (bind _returnvalue (- (.x _grid_coord) 1.0))
  (bind _returnvalue_2 (Math|Vector2D|MakeVector2D _returnvalue (.y _grid_coord)))
  (if (not (Utilities|Map|Contains (Variables|Default|GetMidnight%20Ground%20Grid) _returnvalue_2))
    (CallFunction|SpawnMidnightGround (+ (Transformation|GetActorLocation Input%20Midnight%20Ground) (Math|Vector|MakeVector 0.0 -1e+04 0.0)) _returnvalue_2)))

(event Custom|CustomEvent_0
  ;[1 1 1] Button 4 - main menu
  (Default|QuitLevel (Variables|/Game/BP/BP_GameInstance.BP_GameInstance_C|GetGame%20Controller (Variables|/Game/TopDown/Blueprints/BP_TopDownController.BP_TopDownController_C|GetGame%20Instance (Variables|/Game/TopDown/Blueprints/BP_TopDownCharacter.BP_TopDownCharacter_C|GetTop%20Down%20Controller (Variables|Default|GetTop%20Down%20Character))))))

(event Custom|On%20South%20Trigger%20Enter
  (params (Input%20Midnight%20Ground :type BP%20Midnight%20Ground%20Object%20Reference))
  (bind _grid_coord (Variables|/Game/BP/BP_MidnightGround.BP_MidnightGround_C|GetGrid%20Coord Input%20Midnight%20Ground))
  (bind _returnvalue (- (.y _grid_coord) 1.0))
  (bind _returnvalue_2 (Math|Vector2D|MakeVector2D (.x _grid_coord) _returnvalue))
  (if (not (Utilities|Map|Contains (Variables|Default|GetMidnight%20Ground%20Grid) _returnvalue_2))
    (CallFunction|SpawnMidnightGround (+ (Transformation|GetActorLocation Input%20Midnight%20Ground) (Math|Vector|MakeVector -1e+04 0.0 0.0)) _returnvalue_2)))

(event Custom|On%20NW%20Trigger%20Enter
  (params (Input%20Midnight%20Ground :type BP%20Midnight%20Ground%20Object%20Reference))
  (bind _grid_coord (Variables|/Game/BP/BP_MidnightGround.BP_MidnightGround_C|GetGrid%20Coord Input%20Midnight%20Ground))
  (bind _returnvalue (+ (.y _grid_coord) 1.0))
  (bind _returnvalue_2 (- (.x _grid_coord) 1.0))
  (bind _returnvalue_3 (Math|Vector2D|MakeVector2D _returnvalue_2 _returnvalue))
  (if (not (Utilities|Map|Contains (Variables|Default|GetMidnight%20Ground%20Grid) _returnvalue_3))
    (CallFunction|SpawnMidnightGround (+ (Transformation|GetActorLocation Input%20Midnight%20Ground) (Math|Vector|MakeVector 1e+04 -1e+04 0.0)) _returnvalue_3)))

(event Custom|Move%20Character%20Forward
  (bind _top_down_character (Variables|Default|GetTop%20Down%20Character))
  (bind _charactermovement (Variables|/Script/Engine.Character|GetCharacterMovement _top_down_character))
  ;[1 1 1] Move character forward constantly
  (Utilities|IsValid _top_down_character
    (:Is%20Valid
      (if (AI|Components|NavMovement|IsMovingonGround _charactermovement)
        (Physics|AddForce _charactermovement (* (Math|Vector|GetRightVector "0, 0, 0") (Variables|Default|GetCharacter%20Forward%20Speed)))))))

(event Custom|Spawn%20Midnight%20Ground
  (params (Spawn%20Transform%20Location :type Vector) (Grid%20Coord :type Vector%202D%20Structure))
  (bind _returnvalue (Game|SpawnActorfromClass (.OutItem (Utilities|Array|Random (Variables|Default|GetSpawnable%20Midnight%20Ground%20Classes))) (Math|Transform|MakeTransform Spawn%20Transform%20Location "0, 0, 0" "1.000000,1.000000,1.000000") "AlwaysSpawn" "MultiplyWithRoot" 0 Grid%20Coord 0))
  (Utilities|Map|Add (Variables|Default|GetMidnight%20Ground%20Grid) Grid%20Coord _returnvalue))

(event Custom|End%20Midnight%20Mode
  (Game|SetGamePaused true)
  (bind _created_popup_widget (Default|CreatePopup (Variables|/Game/TopDown/Blueprints/BP_TopDownController.BP_TopDownController_C|GetGame%20Controller (Variables|/Game/TopDown/Blueprints/BP_TopDownCharacter.BP_TopDownCharacter_C|GetTop%20Down%20Controller (Variables|Default|GetTop%20Down%20Character))) true true true "Victory!" "You made it back to defend the kingdom! 
 
Thanks for playing Draco Disease!" "Restart Fight 
with Commander" "Restart Demo" "Survival Mode" "Main Menu"))
  (EventDispatchers|AssignOnClickButton1 _created_popup_widget (delegate Custom|CustomEvent))
  (EventDispatchers|BindEventtoOnClickButton2 _created_popup_widget (delegate Custom|OnClickButton1_Event))
  (EventDispatchers|BindEventtoOnClickButton3 _created_popup_widget (delegate Custom|CustomEvent_1))
  (EventDispatchers|BindEventtoOnClickButton4 _created_popup_widget (delegate Custom|CustomEvent_0)))

(event EventBeginPlay
  (Utilities|FlowControl|Sequence
    (:then_0
      (Utilities|Map|Add :TargetMap (Variables|Default|GetMidnight%20Ground%20Grid) :Value (Variables|Default|GetOriginal%20Midnight%20Ground))
      (bind _asbp_game_instance (Utilities|Casting|CastToBP_GameInstance (Game|GetGameInstance)))
      (Variables|Default|SetGame%20Instance _asbp_game_instance))
    (:then_1
      (Utilities|FlowControl|DelayUntilNextTick)
      (Utilities|FlowControl|DelayUntilNextTick)
      (Default|Show/HideCastleHealth (Variables|/Game/BP/BP_GameController.BP_GameController_C|GetUI (Variables|/Game/BP/BP_GameInstance.BP_GameInstance_C|GetGame%20Controller (Variables|Default|GetGame%20Instance))) false)
      (Default|Show/HideWavesText (Variables|/Game/BP/BP_GameController.BP_GameController_C|GetUI (Variables|/Game/BP/BP_GameInstance.BP_GameInstance_C|GetGame%20Controller (Variables|Default|GetGame%20Instance))) false)
      (if (== (Variables|/Game/BP/BP_GameSave.BP_GameSave_C|GetBattlefield%20Opening%20-%20Wizard%20Meet%20Choice%202%20%280-invald,%201-accept%20spell,%202-reject%20spell%29 (Variables|/Game/BP/BP_GameInstance.BP_GameInstance_C|GetSave%20Game%20Instance (Variables|Default|GetGame%20Instance))) 1)
        (Default|Show/HideAbilitiesPanel (Variables|/Game/BP/BP_GameController.BP_GameController_C|GetUI (Variables|/Game/BP/BP_GameInstance.BP_GameInstance_C|GetGame%20Controller (Variables|Default|GetGame%20Instance))) true))
      (Variables|Default|SetTop%20Down%20Character (Variables|/Game/TopDown/Blueprints/BP_TopDownController.BP_TopDownController_C|GetTop%20Down%20Character (Variables|/Game/BP/BP_GameInstance.BP_GameInstance_C|GetTop%20Down%20Controller (Variables|Default|GetGame%20Instance))))
      (Variables|/Script/Engine.CharacterMovementComponent|SetMaxWalkSpeed (Variables|/Script/Engine.Character|GetCharacterMovement (Variables|/Game/TopDown/Blueprints/BP_TopDownController.BP_TopDownController_C|GetTop%20Down%20Character (Variables|/Game/BP/BP_GameInstance.BP_GameInstance_C|GetTop%20Down%20Controller (Variables|Default|GetGame%20Instance)))) (* (Variables|/Script/Engine.CharacterMovementComponent|GetMaxWalkSpeed (Variables|/Script/Engine.Character|GetCharacterMovement (Variables|/Game/TopDown/Blueprints/BP_TopDownController.BP_TopDownController_C|GetTop%20Down%20Character (Variables|/Game/BP/BP_GameInstance.BP_GameInstance_C|GetTop%20Down%20Controller (Variables|Default|GetGame%20Instance))))) 2.0))
      (Default|ChangeInputType (Variables|/Game/BP/BP_GameInstance.BP_GameInstance_C|GetTop%20Down%20Controller (Variables|Default|GetGame%20Instance)) "NewEnumerator6")
      (Variables|/Script/Engine.SpringArmComponent|SetCameraLagSpeed (Variables|/Game/TopDown/Blueprints/BP_TopDownCharacter.BP_TopDownCharacter_C|GetSpringArm1%20Perspective%20Cam (Variables|/Game/TopDown/Blueprints/BP_TopDownController.BP_TopDownController_C|GetTop%20Down%20Character (Variables|/Game/BP/BP_GameInstance.BP_GameInstance_C|GetTop%20Down%20Controller (Variables|Default|GetGame%20Instance)))) 7.0))
    (:then_2
      (CallFunction|StartSpawningEnemies))
    (:then_3
      (Default|CreateScreenFade (Variables|Default|GetGame%20Instance) "(R=0.000000,G=0.000000,B=0.000000,A=1.000000)" 0.0 1.0 true 2.0))
    (:then_4
      ;[1 1 1] Midnight Mode Timer
      (Utilities|FlowControl|Delay 55.0)
      (CallFunction|EndMidnightMode))
    (:then_5
      ;[1 1 1] Messages
      (Utilities|FlowControl|Delay 3.0)
      (Default|StartMessage (Variables|/Game/BP/BP_GameInstance.BP_GameInstance_C|GetGame%20Controller (Variables|Default|GetGame%20Instance)) "\"Gotta Get out of here.\"" "NewEnumerator0" 3.0)
      (Utilities|FlowControl|Delay 3.0)
      (Audio|PlaySound2D "/Game/Sound/SoundFX/Cue_UndeadDragonRoar_Short.Cue_UndeadDragonRoar_Short" 1.1 0.7 0.0 0 0)
      (Utilities|FlowControl|Delay 9.0)
      (Default|StartMessage (Variables|/Game/BP/BP_GameInstance.BP_GameInstance_C|GetGame%20Controller (Variables|Default|GetGame%20Instance)) "\"That thing was following me!\"" "NewEnumerator0" 4.0)
      (Utilities|FlowControl|Delay 3e+01)
      (Default|StartMessage (Variables|/Game/BP/BP_GameInstance.BP_GameInstance_C|GetGame%20Controller (Variables|Default|GetGame%20Instance)) "\"Almost there.\"" "NewEnumerator0" 3.0))))

(event EventTick
  (params (DeltaSeconds :type Float%20%28single-precision%29))
  (CallFunction|MoveCharacterForward))

(fn ConstructionScript)