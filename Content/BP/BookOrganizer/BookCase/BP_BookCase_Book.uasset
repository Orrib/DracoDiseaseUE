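; Bookcase actor for a book-sorting puzzle, labeled with its shelf index as a Roman numeral.
; Construction randomly hides decorative books, shelves and scene components for variety and disables actor collision.
; BeginPlay links book slots to the bookcase; RegisterBook records books per slot and calls the order check.
; The order check has an empty loop, UnregisterBook is empty, and TryAcceptBookcase's contradictory condition blocks its GM-validated snapping.
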(event EventBeginPlay
  (for _array_element (Variables|Default|GetBookSlots)
    (Variables|/Game/BP/BookOrganizer/BookCase/BP_BookSlot.BP_BookSlot_C|SetOwningBookcase _array_element self)
    (bind _roman (CallFunction|IndextoRoman (Variables|Default|GetShelfIndex)))
    (Rendering|Components|TextRender|SetText (Variables|Default|GetLabel) _roman)))

(fn ConstructionScript
  (bind _returnvalue (Math|Random|RandomBool))
  (Utilities|FlowControl|Sequence
    (:then_0
      (Utilities|FlowControl|Sequence
        (:then_0
          (Utilities|FlowControl|Sequence
            (:then_0
              (Rendering|SetVisibility (Variables|Default|GetScene4) _returnvalue true))
            (:then_1
              (Rendering|SetVisibility (Variables|Default|GetBook7) _returnvalue false))
            (:then_2
              (Rendering|SetVisibility (Variables|Default|GetBook22) _returnvalue false))))
        (:then_1
          (Utilities|FlowControl|Sequence
            (:then_0
              (Rendering|SetVisibility (Variables|Default|GetShelf%202) _returnvalue true))
            (:then_1
              (Rendering|SetVisibility (Variables|Default|GetBook5) _returnvalue false))))
        (:then_2
          (Utilities|FlowControl|Sequence
            (:then_0
              (Rendering|SetVisibility (Variables|Default|GetBook10) _returnvalue false))
            (:then_1
              (Rendering|SetVisibility (Variables|Default|GetBook4) _returnvalue false))
            (:then_2
              (Rendering|SetVisibility (Variables|Default|GetScene) _returnvalue true))
            (:then_3
              (Rendering|SetVisibility (Variables|Default|GetScene2) _returnvalue true))))
        (:then_3
          (Utilities|FlowControl|Sequence
            (:then_0
              (Rendering|SetVisibility (Variables|Default|GetBook16) _returnvalue true))
            (:then_1
              (Rendering|SetVisibility (Variables|Default|GetBook15) _returnvalue true))
            (:then_2
              (Rendering|SetVisibility (Variables|Default|GetBook17) _returnvalue true))))))
    (:then_2
      (Collision|SetActorEnableCollision false))))

(fn TryAcceptBookcase
  (params (BookRef :type BP%20Book%20Base%20Object%20Reference))
  (Development|PrintString "HIT")
  (if (and (not (Variables|/Game/BP/BookOrganizer/Bookbase/BP_BookBase.BP_BookBase_C|GetbPlaced BookRef)) (Variables|/Game/BP/BookOrganizer/Bookbase/BP_BookBase.BP_BookBase_C|GetbPlaced BookRef))
    (Actor|GetActorOfClass (Utilities|GetClass (Variables|Default|GetGM)))
    (Utilities|Casting|CastToBP_Book_I BookRef)
    (if (Default|ValidatePlacement (Variables|Default|GetGM))
      (Transformation|AttachComponentToComponent BookRef 0 "None" "SnapToTarget" "SnapToTarget" "KeepRelative" true)
      (Variables|/Game/BP/BookOrganizer/Bookbase/BP_BookBase.BP_BookBase_C|SetbPlaced BookRef true)
      (Collision|SetActorEnableCollision BookRef false)
      (Default|RegisterBookPlacedCorrect() (Variables|Default|GetGM))
      (return)
      (else
        (Default|ReturntoOriginal BookRef)
        (return)))))

(fn IndextoRoman
  (params (Index :type Integer))
  ;[1 1 1] Converting Integer to Roman
  (switch int Index
    (:Default
      (return "?"))
    (:1
      (return "I"))
    (:2
      (return "II"))
    (:3
      (return "III"))
    (:4
      (return "IV"))
    (:5
      (return "V"))
    (:6
      (return "VI"))
    (:7
      (return "VII"))
    (:8
      (return "VIII"))))

(fn RegisterBook
  (params (Book :type BP%20Book%20Base%20Object%20Reference) (SlotIndex :type Integer))
  (bind _placedbooks (Variables|Default|GetPlacedBooks))
  (bind _placedbooks_2 (Variables|Default|GetPlacedBooks))
  (bind _returnvalue (Utilities|Array|FindItem _placedbooks_2 Book))
  (bind _returnvalue_2 (Utilities|Array|Length _placedbooks))
  (bind _returnvalue_3 (< SlotIndex _returnvalue_2))
  (if (Variables|Default|GetbPuzzleSolved)
    (return)
    (elif (and _returnvalue_3 (>= _returnvalue_3 0))
      (Utilities|FlowControl|Sequence
        (:then_0
          (if (and (!= _returnvalue -1) (!= _returnvalue SlotIndex))
            (Utilities|Array|SetArrayElem (Variables|Default|GetPlacedBooks) _returnvalue 0)))
        (:then_1
          (Utilities|Array|SetArrayElem (Variables|Default|GetPlacedBooks) SlotIndex Book)
          (CallFunction|CheckAllBooksCorrect :!label _label))
        (:then_2
          (goto _label)))
      (else
        (return)))))

(fn UnregisterBook)

(fn CheckAllBooksCorrect
  (bind _expectedorder (Variables|Default|GetExpectedOrder))
  (bind _placedbooks (Variables|Default|GetPlacedBooks))
  (bind _returnvalue (Utilities|Array|Length _placedbooks))
  (bind _returnvalue_2 (Utilities|Array|Length _expectedorder))
  (bind _returnvalue_3 (Class|KismetMathLibrary|AndIntInt _returnvalue _returnvalue_2))
  (LocalVariables|SetAllCorrect true)
  (if (Variables|Default|GetbPuzzleSolved)
    (return)
    (elif (== _returnvalue_3 _returnvalue_3)
      (for _index (range 0 (- (Utilities|Array|Length (Variables|Default|GetPlacedBooks)) -1))
        _)
      (else
        (return)))))