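; One-shot trigger volume that fires a numbered game event when an actor tagged "player" overlaps it.
; A DoOnce gets the GameController from BP_GameInstance and calls TriggerEvent with EventNum, delaying a tick first if the controller is invalid.
; The second Sequence pin destroys the volume right away, without waiting for that delay.
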(event EventBeginPlay)

(event Collision|EventActorBeginOverlap
  (params (OtherActor :type Actor%20Object%20Reference))
  (if (Actor|ActorHasTag OtherActor "player")
    (Utilities|FlowControl|Sequence
      (:then_0
        (Utilities|FlowControl|DoOnce false
          (:Completed
            (bind _asbp_game_instance (Utilities|Casting|CastToBP_GameInstance (Game|GetGameInstance)))
            (Utilities|IsValid (Variables|/Game/BP/BP_GameInstance.BP_GameInstance_C|GetGame%20Controller _asbp_game_instance)
              (:Is%20Valid
                _)
              (:Is%20Not%20Valid
                (Utilities|FlowControl|DelayUntilNextTick)))
            (Default|TriggerEvent (Variables|/Game/BP/BP_GameInstance.BP_GameInstance_C|GetGame%20Controller _asbp_game_instance) (Variables|Default|GetEvent%20Num)))))
      (:then_1
        (Actor|DestroyActor)))))

(event EventTick
  (params (DeltaSeconds :type Float%20%28single-precision%29)))

(fn ConstructionScript)