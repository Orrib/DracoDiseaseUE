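; BP_Altar is an altar actor that shows on-screen UI while something overlaps it.
; On overlap begin it adds an activation prompt, or an already-used widget if HasBeenUsed is set; this file never sets that flag.
; Overlap end removes the prompt and used widget, but the main altar widget only when the used widget is also valid.
; AddWidgetAltarToScreen offers that main widget or the used one, with no caller here.
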(event Collision|EventActorBeginOverlap
  (params (OtherActor :type Actor%20Object%20Reference))
  (CallFunction|AddWidgetActivateAltartoScreen))

(event Collision|EventActorEndOverlap
  (params (OtherActor :type Actor%20Object%20Reference))
  (CallFunction|RemoveWidgetfromScreen)
  (Widget|RemovefromParent (Variables|Default|GetWidget%20Activate%20Altar)))

(fn ConstructionScript)

(fn AddWidgetAltartoScreen
  (if (Variables|Default|GetHas%20Been%20Used)
    (bind _returnvalue (UserInterface|CreateWidget "/Game/UI/Widget_AltarUsed.Widget_AltarUsed_C"))
    (bind _output_get (Variables|Default|SetWidget%20Altar%20Used _returnvalue))
    (UserInterface|Viewport|AddtoViewport _output_get 0)
    (else
      (bind _returnvalue_2 (UserInterface|CreateWidget "/Game/UI/Widget_Altar.Widget_Altar_C"))
      (bind _output_get_2 (Variables|Default|SetWidget%20Altar _returnvalue_2))
      (UserInterface|Viewport|AddtoViewport _output_get_2 0))))

(fn RemoveWidgetfromScreen
  (bind _widget_altar (Variables|Default|GetWidget%20Altar))
  (bind _widget_altar_used (Variables|Default|GetWidget%20Altar%20Used))
  (Utilities|IsValid _widget_altar_used
    (:Is%20Valid
      (Widget|RemovefromParent _widget_altar_used)
      (Utilities|IsValid _widget_altar
        (:Is%20Valid
          (Widget|RemovefromParent _widget_altar))))))

(fn AddWidgetActivateAltartoScreen
  (if (Variables|Default|GetHas%20Been%20Used)
    (bind _returnvalue (UserInterface|CreateWidget "/Game/UI/Widget_AltarUsed.Widget_AltarUsed_C"))
    (bind _output_get (Variables|Default|SetWidget%20Altar%20Used _returnvalue))
    (UserInterface|Viewport|AddtoViewport _output_get 0)
    (else
      (bind _returnvalue_2 (UserInterface|CreateWidget "/Game/UI/Widget_ActivateAltar.Widget_ActivateAltar_C"))
      (bind _output_get_2 (Variables|Default|SetWidget%20Activate%20Altar _returnvalue_2))
      (UserInterface|Viewport|AddtoViewport _output_get_2 0))))