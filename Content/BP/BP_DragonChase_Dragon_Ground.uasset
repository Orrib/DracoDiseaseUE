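; Ground dragon actor for a dragon chase, with a Fire component that other logic can switch on and off.
; The construction script hides it and disables its collision, and BeginPlay turns the fire off.
; Show/Hide sets visibility and actor collision together.
; Enable/DisableFire activates or deactivates Fire and also toggles collision for the whole actor, so both events write the same collision state.
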(event Custom|Enable/Disable%20Fire
  (params (Enable? :type Boolean))
  (Collision|SetActorEnableCollision Enable?)
  (Components|Activation|SetActive (Variables|Default|GetFire) Enable? false))

(event Custom|Show/Hide
  (params (Show? :type Boolean))
  (Rendering|SetActorHiddenInGame (not Show?))
  (Collision|SetActorEnableCollision Show?))

(event EventBeginPlay
  (CallFunction|Enable/DisableFire false))

(event Collision|EventActorBeginOverlap
  (params (OtherActor :type Actor%20Object%20Reference)))

(event EventTick
  (params (DeltaSeconds :type Float%20%28single-precision%29)))

(fn ConstructionScript
  (CallFunction|Show/Hide false))