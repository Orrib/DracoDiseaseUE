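; BP_CastleDoor is the castle door actor that turns arriving NPCs of one allegiance into castle damage.
; On BeginPlay it finds and stores the BP_GameController in the level.
; When an actor tagged "npc" overlaps it and casts to BP_NPC with the matching allegiance, it destroys that NPC and calls DamageCastle on the controller with a fixed amount.
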(event EventBeginPlay
  (bind _returnvalue (Actor|GetActorOfClass "/Game/BP/BP_GameController.BP_GameController_C"))
  (Variables|Default|SetGame%20Controller _returnvalue))

(event Collision|EventActorBeginOverlap
  (params (OtherActor :type Actor%20Object%20Reference))
  (if (Actor|ActorHasTag OtherActor "npc")
    (bind _asbp_npc (Utilities|Casting|CastToBP_NPC OtherActor))
    (if (Utilities|Enum|Equal(Enum) (Variables|/Game/TopDown/Blueprints/BP_NPC.BP_NPC_C|GetAllegiance _asbp_npc) "NewEnumerator2")
      (Actor|DestroyActor _asbp_npc)
      (Default|DamageCastle (Variables|Default|GetGame%20Controller) 0.2))))

(event EventTick
  (params (DeltaSeconds :type Float%20%28single-precision%29)))

(fn ConstructionScript)