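; BP_CursedAltar is an altar actor that offers an activation prompt when something overlaps it.
; On overlap it shows either the activation widget, which receives a reference to the altar, or an already-used widget, depending on HasBeenUsed.
; An unused altar also plays its own sound and calls StopOtherMusic.
; Ending overlap removes the widgets, stops the sound and calls PlayOtherMusic.
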(event Collision|EventActorBeginOverlap
  (params (OtherActor :type Actor%20Object%20Reference))
  (CallFunction|AddWidgetstoScreen)
  (if (not (Variables|Default|GetHasBeenUsed))
    (Audio|Components|Audio|Play (Variables|Default|GetCursed%20Altar%20Sound) 0.0)
    (Default|CallStopOtherMusic)))

(event Collision|EventActorEndOverlap
  (params (OtherActor :type Actor%20Object%20Reference))
  (bind _widget_altar_used (Variables|Default|GetWidget%20Altar%20Used))
  (Widget|RemovefromParent (Variables|Default|GetWidget%20Activate%20Altar))
  (Audio|Components|Audio|Stop (Variables|Default|GetCursed%20Altar%20Sound))
  (Default|CallPlayOtherMusic)
  (Utilities|IsValid _widget_altar_used
    (:Is%20Valid
      (Widget|RemovefromParent _widget_altar_used))))

(fn ConstructionScript)

(fn AddWidgetstoScreen
  (if (Variables|Default|GetHasBeenUsed)
    (bind _returnvalue (UserInterface|CreateWidget "/Game/UI/Widget_AltarUsed.Widget_AltarUsed_C"))
    (bind _output_get (Variables|Default|SetWidget%20Altar%20Used _returnvalue))
    (UserInterface|Viewport|AddtoViewport _output_get 0)
    (else
      (bind _returnvalue_2 (UserInterface|CreateWidget "/Game/UI/Widget_ActivateCursedAltar.Widget_ActivateCursedAltar_C" 0 self))
      (bind _output_get_2 (Variables|Default|SetWidget%20Activate%20Altar _returnvalue_2))
      (UserInterface|Viewport|AddtoViewport _output_get_2 0))))