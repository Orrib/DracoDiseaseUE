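; BP_Treasure is a pickup treasure chest that awards coins to the player who collects it.
; On pickup it plays a sound, turns on a hidden RectLight and swings the lid hinge open with a timeline.
; When the timeline finishes it adds CoinReward coins, then calls the parent pickup logic after a short delay.
; On destruction in Map_Kingdom, the first chest sets and saves a persistent flag and shows a popup explaining coins.
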(event EventBeginPlay
  (|CallParentFunction)
  (Rendering|SetVisibility (Variables|Default|GetRectLight) false false))

(event EventDestroyed
  (bind _returnvalue (Game|GetCurrentLevelName true))
  (bind _asbp_game_instance (Utilities|Casting|CastToBP_GameInstance (Game|GetGameInstance)))
  (if (and (Utilities|Enum|Equal(Enum) _returnvalue "Map_Kingdom") (not (Variables|/Game/BP/BP_GameSave_Persistent.BP_GameSave_Persistent_C|GetFirst%20Treasure%20Chest%20Opened (Variables|/Game/BP/BP_GameInstance.BP_GameInstance_C|GetSave%20Game%20Instance%20-%20Persistent _asbp_game_instance))))
    (Variables|/Game/BP/BP_GameSave_Persistent.BP_GameSave_Persistent_C|SetFirst%20Treasure%20Chest%20Opened (Variables|/Game/BP/BP_GameInstance.BP_GameInstance_C|GetSave%20Game%20Instance%20-%20Persistent _asbp_game_instance) true)
    (Default|SaveGameAsync _asbp_game_instance "NewEnumerator0")
    (Default|CreatePopup (Variables|/Game/BP/BP_GameInstance.BP_GameInstance_C|GetGame%20Controller _asbp_game_instance) false false false "Treasure" "Coins can purchase troops and defenses." "Ok")))

(event EventOnPickup
  (params (Player%20Controller :type BP%20Top%20Down%20Controller%20Object%20Reference))
  (bind _hinge (Variables|Default|GetHinge))
  (Variables|Default|SetHinge%20Orig%20Relative%20Rotation (Variables|/Script/Engine.SceneComponent|GetRelativeRotation _hinge))
  (Audio|PlaySound2D "/Game/Sound/SoundFX/Cue_Pickup_Treasure.Cue_Pickup_Treasure" 1.0 0.7 0.0 0 0 false)
  (Rendering|SetVisibility (Variables|Default|GetRectLight) true false)
  (bind _newtrack_0 (Timeline|Open%20Chest PlayFromStart)
    (:Update
      (Transformation|SetRelativeRotation _hinge (Math|Rotator|Lerp(Rotator) (Variables|Default|GetHinge%20Orig%20Relative%20Rotation) "0.000000,0.000000,-120.000000" _newtrack_0) false false))
    (:Finished
      (Default|AddCoins Player%20Controller (Variables|Default|GetCoin%20Reward))
      (Audio|PlaySound2D "/Game/Sound/SoundFX/Cue_Pickup.Cue_Pickup" 1.0 (Variables|Default|GetPickup%20SoundPitch%20Multiplier) 0.0 0 0 false)
      (Utilities|FlowControl|Delay 0.8)
      (|CallParentFunction Player%20Controller))))

(fn ConstructionScript
  (|CallParentFunction))