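; Static NPC that displays a speech widget, optionally triggered when a player-tagged actor enters its Detector sphere and hidden when they leave.
; ShowSpeechUI caches the widget, then either runs a monologue that a timer hides, or loads a conversation and enables query collision on the widget.
; UpdateDetectorOverlap re-applies the sphere's radius to refresh overlaps.
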(event OnComponentBeginOverlap(Detector)
  (params (OverlappedComponent :type Primitive%20Component%20Object%20Reference) (OtherActor :type Actor%20Object%20Reference) (OtherComp :type Primitive%20Component%20Object%20Reference) (OtherBodyIndex :type Integer) (bFromSweep :type Boolean) (SweepResult :type Hit%20Result%20Structure%20%28by%20ref%29))
  (if (Actor|ActorHasTag OtherActor "player")
    (if (Variables|Default|GetProximity%20Speech%20NPC)
      (CallFunction|ShowSpeechUI))))

(event OnComponentEndOverlap(Detector)
  (params (OverlappedComponent :type Primitive%20Component%20Object%20Reference) (OtherActor :type Actor%20Object%20Reference) (OtherComp :type Primitive%20Component%20Object%20Reference) (OtherBodyIndex :type Integer))
  (if (and (Actor|ActorHasTag OtherActor "player") (Variables|Default|GetProximity%20Speech%20NPC))
    (CallFunction|HideSpeechUI)))

(event Custom|Hide%20Speech%20UI
  (bind _widget_speech (Variables|Default|GetWidget_Speech))
  (Development|SetHiddeninGame _widget_speech true false)
  (Collision|SetCollisionEnabled _widget_speech "NoCollision"))

(event Custom|CustomEvent_0
  (CallFunction|HideSpeechUI)
  (Collision|SetCollisionEnabled (Variables|Default|GetWidget_Speech) "NoCollision")
  (Utilities|Time|ClearandInvalidateTimerbyHandle (Variables|Default|GetMonoogue%20Timer)))

(event Custom|Update%20Detector%20Overlap
  (bind _detector (Variables|Default|GetDetector))
  (Components|Sphere|SetSphereRadius _detector (Variables|/Script/Engine.SphereComponent|GetSphereRadius _detector) true))

(event Custom|Show%20Speech%20UI
  (bind _speech_ui_time (Variables|Default|GetSpeech%20UI%20Time))
  (bind _widget_speech (Variables|Default|GetWidget_Speech))
  (Development|SetHiddeninGame _widget_speech false false)
  (Utilities|IsValid (Variables|Default|GetNPC%20Speech%20Widget)
    (:Is%20Valid
      _)
    (:Is%20Not%20Valid
      (bind _aswidget_npcspeech_static_npc (Utilities|Casting|CastToWidget_NPCSpeech_StaticNPC (UserInterface|GetWidget _widget_speech)))
      (Variables|Default|SetNPC%20Speech%20Widget _aswidget_npcspeech_static_npc)))
  (switch Utilities|FlowControl|Switch|SwitchonEnum_SpeechType (Variables|Default|GetSpeech%20Type)
    (:NewEnumerator1
      (Default|InitiateMonologue (Variables|Default|GetNPC%20Speech%20Widget) (Variables|Default|GetMonologue%20Text) _speech_ui_time)
      (bind _returnvalue (Utilities|Time|SetTimerbyEvent (delegate Custom|CustomEvent_0) _speech_ui_time))
      (Variables|Default|SetMonoogue%20Timer _returnvalue))
    (:NewEnumerator2
      (Variables|/Game/UI/Widget_NPCSpeech_StaticNPC.Widget_NPCSpeech_StaticNPC_C|SetConversation (Variables|Default|GetNPC%20Speech%20Widget) (Variables|Default|GetConversation))
      (Default|LoadConversationNPCSpeechWidget (Variables|Default|GetNPC%20Speech%20Widget) self)
      (Collision|SetCollisionEnabled (Variables|Default|GetWidget_Speech) "QueryOnly")
      (Utilities|Time|ClearandInvalidateTimerbyHandle (Variables|Default|GetMonoogue%20Timer)))))

(event EventBeginPlay
  (Rendering|SetVisibility (Variables|Default|GetWidget_Speech) true false))

(event Collision|EventActorBeginOverlap
  (params (OtherActor :type Actor%20Object%20Reference)))

(event EventTick
  (params (DeltaSeconds :type Float%20%28single-precision%29)))

(fn ConstructionScript
  (bind _widget_speech (Variables|Default|GetWidget_Speech))
  (Rendering|SetVisibility _widget_speech false false)
  (Rendering|SetCastShadow _widget_speech false)
  (Rendering|SetVisibility (Variables|Default|GetDetector) (Variables|Default|GetProximity%20Speech%20NPC) false))