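; Medium tent building actor with an inner door that can open and close and an optional dragon statue.
; An overlap on the indoor trigger by an "npc"-tagged actor opens the closed door once, if auto-open is enabled.
; Door state drives the inner wall door mesh's visibility and collision, hiding it rather than animating it.
; The construction script applies door state and statue visibility.
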(event OnComponentBeginOverlap(IndoorDoorTrigger)
  (params (OverlappedComponent :type Primitive%20Component%20Object%20Reference) (OtherActor :type Actor%20Object%20Reference) (OtherComp :type Primitive%20Component%20Object%20Reference) (OtherBodyIndex :type Integer) (bFromSweep :type Boolean) (SweepResult :type Hit%20Result%20Structure%20%28by%20ref%29))
  (if (Math|Boolean|ANDBoolean (Actor|ActorHasTag OtherActor "npc") (Variables|Default|GetAuto-Open%20Door%20For%20NPCs) (not (Variables|Default|GetDoor%20Open)))
    (Utilities|FlowControl|DoOnce false
      (:Completed
        (CallFunction|Open/CloseDoor true)))))

(event Custom|Update%20Appearance
  (bind _door_open (Variables|Default|GetDoor%20Open))
  (bind _inner_wall_door (Variables|Default|GetInner%20Wall%20Door))
  (Collision|SetCollisionEnabled _inner_wall_door (select _door_open "NoCollision" "QueryAndPhysics"))
  (Rendering|SetVisibility _inner_wall_door (not _door_open) false))

(event Custom|Open/Close%20Door
  (params (Open? :type Boolean))
  (Variables|Default|SetDoor%20Open Open?)
  (CallFunction|UpdateAppearance))

(event EventBeginPlay
  (|CallParentFunction) ; This node is disabled and will not be called.\nDrag off pins to build functionality.
)

(event Collision|EventActorBeginOverlap
  (params (OtherActor :type Actor%20Object%20Reference))
  (|CallParentFunction OtherActor) ; This node is disabled and will not be called.\nDrag off pins to build functionality.
)

(event EventTick
  (params (DeltaSeconds :type Float%20%28single-precision%29))
  (|CallParentFunction DeltaSeconds) ; This node is disabled and will not be called.\nDrag off pins to build functionality.
)

(fn ConstructionScript
  (|CallParentFunction)
  (CallFunction|UpdateAppearance)
  (Rendering|SetVisibility (Variables|Default|GetSM_tentLarge_SM_dragon_needswings) (Variables|Default|GetShow%20Dragon%20Statue) false))