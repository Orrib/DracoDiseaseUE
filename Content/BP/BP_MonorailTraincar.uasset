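; Monorail traincar that rides a spline, knocks away players and NPCs it overlaps, and destroys itself at the end of the track.
; A timeline scaled by TimeToCompleteSpline drives its transform, while a second, looping timeline rocks it in pitch with randomized speed and amplitude.
; On overlap it applies point damage and a horizontal, mass-scaled launch away from DamageImpulseSourcePos, playing a hit sound only for players.
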(event EventBeginPlay
  (Audio|Components|Audio|Play (Variables|Default|GetAudio) (Math|Random|RandomFloatinRange 0.0 12.0))
  (Components|Timeline|SetPlayRate (Variables|Default|GetFollow%20Track) (Math|Float|Power (Variables|Default|GetTime%20to%20Complete%20Spline) -1.0))
  (Utilities|FlowControl|Sequence
    (:then_0
      ;[1 1 1] Follow Track
      (bind _newtrack_0 (Timeline|Follow%20Track PlayFromStart)
        (:Update
          (Transformation|SetActorTransform (Spline|GetTransformatTime (Variables|Default|GetSpline) _newtrack_0 "World" (Variables|Default|GetUse%20Constant%20Velocity) false)))
        (:Finished
          (Actor|DestroyActor))))
    (:then_1
      ;[1 1 1] rotate train
      (Components|Timeline|SetPlayRate (Variables|Default|GetRotate) (Math|Float|Power (Math|Random|RandomFloatinRange 1.0 1.5) -1.0) :!label _label)
      (Variables|Default|SetRandom%20Rotation%20Factor (Math|Random|RandomFloatinRange 5.0 7.0))
      (bind _newtrack_0_2 (Timeline|Rotate PlayFromStart)
        (:Update
          (Transformation|SetRelativeRotation (Variables|Default|GetScene1) (Math|Rotator|MakeRotator 0.0 (* _newtrack_0_2 (Variables|Default|GetRandom%20Rotation%20Factor)) 0.0) false false))
        (:Finished
          (Utilities|FlowControl|Delay (Math|Random|RandomFloatinRange 0.0 0.0))
          (goto _label))))))

(event EventTick
  (params (DeltaSeconds :type Float%20%28single-precision%29)))

(event Collision|EventActorBeginOverlap
  (params (OtherActor :type Actor%20Object%20Reference))
  (bind _returnvalue (Transformation|GetActorLocation OtherActor))
  (bind _returnvalue_2 (Transformation|GetActorLocation OtherActor))
  (bind _damage_impulse_source_pos (Variables|Default|GetDamage%20Impulse%20Source%20Pos))
  (bind _returnvalue_3 (Transformation|GetWorldLocation _damage_impulse_source_pos))
  (bind _returnvalue_4 (Math|Vector|GetUnitDirection(Vector) (Math|Vector|MakeVector (.x _returnvalue_3) (.y _returnvalue_3) (.z _returnvalue_2)) _returnvalue))
  (if (Actor|ActorHasTag OtherActor "player")
    (Audio|PlaySound2D "/Game/Sound/SoundFX/Cue_Sword_Hit_Gore.Cue_Sword_Hit_Gore" 0.5 1.5 0.0 0 0)
    (Game|Damage|ApplyPointDamage OtherActor 0.1 _returnvalue_4 (Collision|MakeHitResult false false 0.0 0.0 "0, 0, 0" "0, 0, 0" "0,0,1" "0,0,1" 0 0) 0 self "/Engine/EngineDamageTypes/DmgTypeBP_Environmental.DmgTypeBP_Environmental_C" :!label _label)
    (bind _ascharacter (Utilities|Casting|CastToCharacter OtherActor))
    ;[1 1 1] Apply Impulse, accountinmg for mass
    (Character|LaunchCharacter _ascharacter (* _returnvalue_4 (/ 2e+05 (Variables|/Script/Engine.CharacterMovementComponent|GetMass (Variables|/Script/Engine.Character|GetCharacterMovement _ascharacter)))) true true)
    (elif (Actor|ActorHasTag OtherActor "npc")
      (goto _label))))

(fn ConstructionScript)