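; Air-to-ground dragon fire hazard for the Chapter 1 Part 1 dragon chase, switched on and off through a single enable/disable event.
; Enabling turns on the player collision and fades in the fire sound; disabling removes collision, fades out the sound and runs a timeline dimming the spotlight to zero.
; It calls disable on construction and BeginPlay, and nothing here restores the light on enable.
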(event Custom|Enable/Disable%20Dragon%20Fire%20Settings%20for%20Chap%201%20Part%201%20Dragon%20Chase
  (params (Enble? :type Boolean))
  (bind _fire_sound (Variables|Default|GetFire%20Sound))
  (Collision|SetCollisionEnabled (Variables|Default|GetPlayer%20Collision) (select Enble? "QueryAndPhysics" "NoCollision"))
  (if Enble?
    (Audio|Components|Audio|FadeIn _fire_sound 3.0 1.0 0.0 "Linear" :!class /Script/Engine.AudioComponent)
    (else
      (Audio|Components|Audio|FadeOut _fire_sound 2.0 0.0 "Linear" :!class /Script/Engine.AudioComponent)
      (bind _newtrack_0 (Timeline|Timeline PlayFromStart)
        (:Update
          (Rendering|Components|Light|SetIntensity (Variables|Default|GetSpotLight) (Math|Float|Lerp (Variables|Default|GetInitial%20Intensity) 0.0 _newtrack_0)))))))

(event EventBeginPlay
  (|CallParentFunction)
  (CallFunction|Enable/DisableDragonFireSettingsforChap1Part1DragonChase false))

(event Collision|EventActorBeginOverlap
  (params (OtherActor :type Actor%20Object%20Reference))
  (|CallParentFunction OtherActor) ; This node is disabled and will not be called.\nDrag off pins to build functionality.
)

(event EventTick
  (params (DeltaSeconds :type Float%20%28single-precision%29))
  (|CallParentFunction DeltaSeconds) ; This node is disabled and will not be called.\nDrag off pins to build functionality.
)

(fn ConstructionScript
  (|CallParentFunction)
  (CallFunction|Enable/DisableDragonFireSettingsforChap1Part1DragonChase false)
  (Variables|Default|SetInitial%20Intensity (Variables|/Script/Engine.LightComponentBase|GetIntensity (Variables|Default|GetSpotLight))))