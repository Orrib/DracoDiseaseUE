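; Necromancer sprite actor that stages the necromancer's appearance when MoveNecromancer is called.
; The event unhides the actor, then runs two slowed timelines together: one fades the sprite color from black to white, the other moves its parent component from StartPos to EndPos.
; When the move finishes, a Levitate timeline offsets it vertically around EndPos for a hovering effect.
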(event Custom|Move%20Necromancer
  (Rendering|SetActorHiddenInGame false)
  (Utilities|FlowControl|Sequence
    (:then_0
      (Components|Timeline|SetPlayRate (Variables|Default|GetTimeline_0) (Math|Float|Power 15.0 -1.0))
      (bind _newtrack_1 (Timeline|Timeline_0 PlayFromStart)
        (:Update
          (Sprite|SetSpriteColor (Variables|Default|GetNecro_Sprite) (Math|Color|Lerp(LinearColor) "(R=0.000000,G=0.000000,B=0.000000,A=1.000000)" "(R=1.000000,G=1.000000,B=1.000000,A=1.000000)" _newtrack_1)))))
    (:then_1
      (Components|Timeline|SetPlayRate (Variables|Default|GetTimeline) (Math|Float|Power 6.0 -1.0))
      (bind _newtrack_0 (Timeline|Timeline PlayFromStart)
        (:Update
          (Transformation|SetWorldLocation (Variables|Default|GetNecro%20Parent) (Math|Vector|Lerp(Vector) (Transformation|GetWorldLocation (Variables|Default|GetStart%20Pos)) (Transformation|GetWorldLocation (Variables|Default|GetEnd%20Pos)) _newtrack_0) false false))
        (:Finished
          (Components|Timeline|SetPlayRate (Variables|Default|GetLevitate) (Math|Float|Power 5.0 -1.0))
          (bind _newtrack_0_2 (Timeline|Levitate PlayFromStart)
            (:Update
              (Transformation|SetWorldLocation (Variables|Default|GetNecro%20Parent) (+ (Transformation|GetWorldLocation (Variables|Default|GetEnd%20Pos)) (Math|Vector|MakeVector 0.0 0.0 (* _newtrack_0_2 2e+01))) false false))))))))

(event EventBeginPlay)

(fn ConstructionScript)