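; Short-lived sword slash hitbox actor that grows, deals damage on overlap, then fades out and destroys itself.
; On BeginPlay a Slash timeline scales CubeOrigin, then fires a radial impulse and starts a Fade timeline that drives material opacity and disables collision partway.
; Timeline play rates derive from SlashTime and FadeTime.
; Overlaps apply point damage to actors tagged as wizard NPCs (with hit sound), boxes, dragons or wild.
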(event EventBeginPlay
  ;[1 1 1] convert slash time to play rate
  (Components|Timeline|SetPlayRate (Variables|Default|GetSlash) (Math|Float|Power (Variables|Default|GetSlash%20Time) -1.0))
  (bind _newtrack_1 (Timeline|Slash PlayFromStart)
    (:Update
      (Transformation|SetRelativeScale3D (Variables|Default|GetCube%20Origin) _newtrack_1))
    (:Finished
      ;[1 1 1] Physics Impulse
      (Class|RadialForceComponent|FireImpulse (Variables|Default|GetRadialForce))
      ;[1 1 1] convert slash time to play rate
      (Components|Timeline|SetPlayRate (Variables|Default|GetFade) (Math|Float|Power (Variables|Default|GetFade%20Time) -1.0))
      (bind _newtrack_0 (Timeline|Fade PlayFromStart)
        (:Update
          (Rendering|Material|SetScalarParameterValueonMaterials (Variables|Default|GetCube) "Opacity" _newtrack_0))
        (:Finished
          (Actor|DestroyActor))
        (:Collision%20Disabled
          (Collision|SetActorEnableCollision false))))))

(event Collision|EventActorBeginOverlap
  (params (OtherActor :type Actor%20Object%20Reference))
  (bind _returnvalue (Transformation|GetActorLocation OtherActor))
  (bind _cube_origin (Variables|Default|GetCube%20Origin))
  (bind _returnvalue_2 (Transformation|GetWorldLocation _cube_origin))
  (if (and (Actor|ActorHasTag OtherActor "npc") (Actor|ActorHasTag OtherActor "wizard"))
    ;[1 1 1] enemy
    (Audio|PlaySound2D "/Game/Sound/SoundFX/Cue_Sword_Hit.Cue_Sword_Hit" 1.0 1.0 0.0 0 0)
    (Game|Damage|ApplyPointDamage OtherActor (Variables|Default|GetDamage) (Math|Vector|GetUnitDirection(Vector) _returnvalue_2 _returnvalue) (Collision|MakeHitResult false false 0.0 0.0 _returnvalue_2 _returnvalue "0,0,1" "0,0,1" 0 0) 0 self)
    (else
      ;[1 1 1] box
      (if (Actor|ActorHasTag OtherActor "box")
        (Game|Damage|ApplyPointDamage OtherActor (Variables|Default|GetDamage) (Math|Vector|GetUnitDirection(Vector) (Transformation|GetWorldLocation (Variables|Default|GetDamage%20Origin)) (Transformation|GetActorLocation OtherActor)) (Collision|MakeHitResult false true 0.0 0.0 "0, 0, 0" "0, 0, 0" "0,0,1" "0,0,1" 0 0) 0 self)
        (else
          ;[1 1 1] dragon
          (if (Actor|ActorHasTag OtherActor "dragon")
            (Game|Damage|ApplyPointDamage OtherActor (Variables|Default|GetDamage) (Math|Vector|GetUnitDirection(Vector) (Transformation|GetWorldLocation (Variables|Default|GetDamage%20Origin)) (Transformation|GetActorLocation OtherActor)) (Collision|MakeHitResult false true 0.0 0.0 "0, 0, 0" "0, 0, 0" "0,0,1" "0,0,1" 0 0) 0 self)
            (else
              ;[1 1 1] wild
              (if (Actor|ActorHasTag OtherActor "wild")
                (Game|Damage|ApplyPointDamage OtherActor (Variables|Default|GetDamage) (Math|Vector|GetUnitDirection(Vector) (Transformation|GetWorldLocation (Variables|Default|GetDamage%20Origin)) (Transformation|GetActorLocation OtherActor)) (Collision|MakeHitResult false true 0.0 0.0 "0, 0, 0" "0, 0, 0" "0,0,1" "0,0,1" 0 0) 0 self)))))))))

(event EventTick
  (params (DeltaSeconds :type Float%20%28single-precision%29)))

(fn ConstructionScript)