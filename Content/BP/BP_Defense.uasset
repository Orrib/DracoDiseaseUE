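; BP_Defense is a base Blueprint for selectable defenses, with stub hooks for right-click actions and selection UI subtitle text.
; On BeginPlay it registers with the GameController's Defenses list and binds its selection icon widget, whose clicks route back to that controller.
; The icon is visible and clickable only in strategy mode, while selection changes update the icon and optionally play sounds.
; Right-clicks play an error sound unless CanRightClickSelectionUI, false by default, allows them.
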(event Custom|Initial%20UI%20Refresh
  (CallFunction|UpdateSelectionIconWidget))

(event Custom|Defense:%20On%20Right%20Click%20Selection%20UI)

(event Custom|On%20Clicked%20Icon_Event
  (Default|OnClickDefenseSelectionIcon (Variables|/Game/BP/BP_GameInstance.BP_GameInstance_C|GetGame%20Controller (Variables|Default|GetGame%20Instance)) self))

(event Custom|Update%20Selection%20Icon%20Widget
  (bind _game_instance (Variables|Default|GetGame%20Instance))
  (bind _selection_icon_component (Variables|Default|GetSelection%20Icon%20Component))
  (bind _top_down_controller (Variables|/Game/BP/BP_GameInstance.BP_GameInstance_C|GetTop%20Down%20Controller _game_instance))
  (bind _in_strategy_mode_ (Variables|/Game/TopDown/Blueprints/BP_TopDownController.BP_TopDownController_C|GetIn%20Strategy%20Mode? _top_down_controller))
  (Rendering|SetVisibility _selection_icon_component _in_strategy_mode_ false)
  (Collision|SetCollisionEnabled _selection_icon_component (select _in_strategy_mode_ "QueryOnly" "NoCollision")))

(event EventBeginPlay
  (bind _asbp_game_instance (Utilities|Casting|CastToBP_GameInstance (Game|GetGameInstance)))
  (Variables|Default|SetGame%20Instance _asbp_game_instance)
  (bind _aswidget_selection_icon (Utilities|Casting|CastToWidget_SelectionIcon (UserInterface|GetWidget (Variables|Default|GetSelection%20Icon%20Component))))
  (Variables|Default|SetWidget%20Selection%20Icon _aswidget_selection_icon)
  (Utilities|FlowControl|DelayUntilNextTick)
  (Utilities|Array|Add (Variables|/Game/BP/BP_GameController.BP_GameController_C|GetDefenses (Variables|/Game/BP/BP_GameInstance.BP_GameInstance_C|GetGame%20Controller (Variables|Default|GetGame%20Instance))) self)
  (CallFunction|InitialUIRefresh)
  (EventDispatchers|AssignOnClickedIcon (Variables|Default|GetWidget%20Selection%20Icon) (delegate Custom|On%20Clicked%20Icon_Event)))

(event EventOnSelect/UnselectDefense
  (params (Select? :type Boolean) (Play%20Sound? :type Boolean))
  (bind _output_get (Variables|Default|SetSelected Select?))
  (Default|Select/UnselectIcon (Variables|Default|GetWidget%20Selection%20Icon) _output_get)
  (if _output_get
    (if Play%20Sound?
      (Audio|PlaySound2D "/Game/Sound/SoundFX/Cue_Select.Cue_Select" 0.5 1.0 0.0 0 0))
    (elif Play%20Sound?
      (Audio|PlaySound2D "/Game/Sound/SoundFX/Cue_Unselect.Cue_Unselect" 0.5 1.0 0.0 0 0))))

(event EventOnEnter/ExitStrategyMode
  (params (Enter? :type Boolean))
  (CallFunction|UpdateSelectionIconWidget))

(event EventOnRightClickSelectionUI
  (if (CallFunction|CanRightClickSelectionUI?)
    (CallFunction|Defense:onRightClickSelectionUI)
    (else
      (Audio|PlaySound2D "/Game/Sound/SoundFX/Cue_Error.Cue_Error" 0.5 1.0 0.0 0 0))))

(fn ConstructionScript)

(fn CanRightClickSelectionUI?
  (return false))

(fn Defense:GetSelectionUISubtitleText
  (return ""))