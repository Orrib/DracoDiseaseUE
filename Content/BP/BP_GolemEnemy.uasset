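; Paper2D golem enemy character that detects player and NPC actors, attacks them, and drops treasure and a potion on death.
; Detector overlaps maintain a target list and drive alert or timed de-alert through BP_GolemController's state.
; Attacks randomly alternate between an arced leap that spawns a shockwave on landing and repeated AIMoveTo charges, falling back to leaping when pathfinding fails.
; Low health tints the sprite and lengthens charge chains; Tick flips the sprite by velocity.
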(event OnComponentBeginOverlap(Detector)
  (params (OverlappedComponent :type Primitive%20Component%20Object%20Reference) (OtherActor :type Actor%20Object%20Reference) (OtherComp :type Primitive%20Component%20Object%20Reference) (OtherBodyIndex :type Integer) (bFromSweep :type Boolean) (SweepResult :type Hit%20Result%20Structure%20%28by%20ref%29))
  (if (Utilities|ActorIsEnemy? OtherActor)
    (Utilities|Array|Add (Variables|Default|GetDetected%20Enemies) OtherActor)
    (Game|BindEventtoOnDestroyed OtherActor (delegate Custom|On%20Detected%20Actor%20Destroyed))
    (Variables|Default|SetTarget%20Enemy%20Actor OtherActor)
    (if (Actor|ActorHasTag OtherActor "player")
      (Default|OnPlayerAlertsEnemy (Variables|/Game/BP/BP_GameInstance.BP_GameInstance_C|GetTop%20Down%20Controller (Variables|Default|GetGame%20Instance)) self))
    (Utilities|Time|ClearandInvalidateTimerbyHandle (Variables|Default|GetDe-Alert%20Timer%20Handle))
    (if (not (Utilities|Enum|Equal(Enum) (Variables|/Game/BP/BP_GolemController.BP_GolemController_C|GetCurrent%20State (Variables|Default|GetGolem%20Controller)) "NewEnumerator2"))
      (CallFunction|Alert/De-Alert true))))

(event OnComponentEndOverlap(Detector)
  (params (OverlappedComponent :type Primitive%20Component%20Object%20Reference) (OtherActor :type Actor%20Object%20Reference) (OtherComp :type Primitive%20Component%20Object%20Reference) (OtherBodyIndex :type Integer))
  (if (Utilities|ActorIsEnemy? OtherActor)
    (Utilities|Array|RemoveItem (Variables|Default|GetDetected%20Enemies) OtherActor)
    (Utilities|GolemDying?
      (:false
        (Utilities|IsValid (Variables|Default|GetGolem%20Controller)
          (:Is%20Valid
            (if (Utilities|Enum|Equal(Enum) (Variables|/Game/BP/BP_GolemController.BP_GolemController_C|GetCurrent%20State (Variables|Default|GetGolem%20Controller)) "NewEnumerator0")
              (CallFunction|UpdateDe-alertTimer :!label _label)))
          (:Is%20Not%20Valid
            (goto _label)))))))

(event Custom|Damage%20Flash
  (bind _paperflipbook (Variables|Default|GetPaperFlipbook))
  ;[1 1 1] Damage
  (Sprite|SetSpriteColor _paperflipbook "(R=0.392157,G=0.000000,B=0.000000,A=0.635294)")
  (Utilities|FlowControl|RetriggerableDelay 0.2)
  (Sprite|SetSpriteColor _paperflipbook (Variables|Default|GetOrig%20Color)))

(event Custom|Attack%20Target
  (bind _returnvalue (Transformation|GetActorLocation))
  (bind _charactermovement (Variables|Character|GetCharacterMovement))
  (bind _target_enemy_actor (Variables|Default|GetTarget%20Enemy%20Actor))
  (bind _returnvalue_2 (Transformation|GetActorLocation _target_enemy_actor))
  ;[1 1 1] Attack
  (if (Utilities|Enum|Equal(Enum) (Variables|/Game/BP/BP_GolemController.BP_GolemController_C|GetCurrent%20State (Variables|Default|GetGolem%20Controller)) "NewEnumerator2")
    (Utilities|Array|Clear (Variables|Default|GetHit%20Enemies))
    (Components|Movement|StopMovementImmediately _charactermovement)
    (Utilities|IsValid _target_enemy_actor
      (:Is%20Valid
        (switch int (Math|Random|RandomIntegerinRange 0 1)
          (:0
            ;;[0 0 0] Leap to player
            ;;;[1 1 1] animation
            (Class|PaperZDAnimInstance|JumptoNode (Variables|Default|GetABP%20Golem) "Attack_Leap" "None" :!label _label)
            (bind (_outlaunchvelocity _returnvalue_3) (Game|SuggestProjectileVelocityCustomArc _returnvalue _returnvalue_2 0.0 0.4))
            (Character|LaunchCharacter (select _returnvalue_3 (Math|Vector|VectorClampSizeMax _outlaunchvelocity 1.4e+03) (* (Math|Vector|GetUnitDirection(Vector) _returnvalue _returnvalue_2) (* (Variables|Default|GetCharge%20Walk%20Speed) 5.0))) true true)
            (Variables|Default|SetLeap%20Attacking true)
            (Class|PrimitiveComponent|SetCastHiddenShadow (Variables|Default|GetFake%20Shadow) true)
            ;;;[1 1 1] rest
            (Utilities|FlowControl|RetriggerableDelay (select (Variables|Default|GetLeap%20Attacking) 7.0 (Math|Random|RandomFloatinRange 1.0 2.5)))
            ;;;;[1 1 1] reset leap attack check
            (Variables|Default|SetLeap%20Attacking false)
            (Class|PrimitiveComponent|SetCastHiddenShadow (Variables|Default|GetFake%20Shadow) false)
            ;;[1 1 1] attack again
            (Utilities|GolemDying? :!label _label_2
              (:false
                (CallFunction|AttackTarget))))
          (:1
            ;;[0 0 0] Charge to target
            ;;;[1 1 1] animation
            (Class|PaperZDAnimInstance|JumptoNode (Variables|Default|GetABP%20Golem) "Attack_Roll" "None")
            ;;;[1 1 1] Set to charge speed
            (Variables|/Script/Engine.CharacterMovementComponent|SetMaxWalkSpeed _charactermovement (Variables|Default|GetCharge%20Walk%20Speed))
            (Variables|Default|SetCharge%20Count 0)
            (Variables|Default|SetCharge%20Attacking true)
            (Utilities|IsValid (Variables|Default|GetTarget%20Enemy%20Actor) :!label _label_3
              (:Is%20Valid
                (bind _movementresult (AI|AIMoveTo self _returnvalue_2 0 -1.0 false)
                  (:OnSuccess
                    _)
                  (:OnFail
                    _))
                ;;;[1 1 1] Pathfinding Fail?
                (Utilities|GolemDying?
                  (:false
                    (if (Math|Boolean|ORBoolean (Utilities|Enum|Equal(Enum) _movementresult "OffPath") (Utilities|Enum|Equal(Enum) _movementresult "Aborted") (Utilities|Enum|Equal(Enum) _movementresult "Invalid"))
                      (CallFunction|ResetWalkingSpeed)
                      (Variables|Default|SetCharge%20Attacking false)
                      (Utilities|IsValid (Variables|Default|GetTarget%20Enemy%20Actor)
                        (:Is%20Valid
                          (goto _label))
                        (:Is%20Not%20Valid
                          (CallFunction|RevaluateTargets)))
                      (else
                        ;;;[1 1 1] Charge 1x-2x normally, Charge 3x-5x if low health (agro mode)
                        (bind _result (Math|Integer|IncrementInt (Variables|Default|GetCharge%20Count))
                          (:%20%20
                            (if (>= _result (select (Utilities|IsLowHealth) (Math|Random|RandomIntegerinRange 5 7) (Math|Random|RandomIntegerinRange 1 2)))
                              (CallFunction|ResetWalkingSpeed)
                              (Variables|Default|SetCharge%20Attacking false)
                              ;;;[1 1 1] rest
                              (Utilities|FlowControl|Delay (Math|Random|RandomFloatinRange 0.7 2.5))
                              (goto _label_2)
                              (else
                                (Utilities|Array|Clear (Variables|Default|GetHit%20Enemies))
                                (goto _label_3))))))))))
              (:Is%20Not%20Valid
                (CallFunction|ResetWalkingSpeed)
                (Variables|Default|SetCharge%20Attacking false)
                (CallFunction|RevaluateTargets))))))
      (:Is%20Not%20Valid
        (CallFunction|RevaluateTargets)))))

(event Custom|On%20Death%20Anim%20COmplete
  ;[1 1 1] Damage
  (Game|SpawnActorfromClass "/Game/BP/BP_Treasure_Special.BP_Treasure_Special_C" (Math|Transform|MakeTransform (Transformation|GetWorldLocation (Variables|Default|GetTreasure%20Spawn%20Point)) "0, 0, 0" "1.000000,1.000000,1.000000") "AdjustIfPossibleButAlwaysSpawn" "MultiplyWithRoot" 0 true 1.0 0)
  (Game|SpawnActorfromClass "/Game/BP/BP_Potion.BP_Potion_C" (Math|Transform|MakeTransform (Transformation|GetWorldLocation (Variables|Default|GetHealthSpawn%20Point)) "0, 0, 0" "1.000000,1.000000,1.000000") "AdjustIfPossibleButAlwaysSpawn" "MultiplyWithRoot" 0 true 1.0 0)
  (Actor|DestroyActor))

(event Custom|Invoke%20Stop%20Charge%20Attack
  ;[1 1 1] Attack
  ;;[0 0 0] Charge to target
  (CallFunction|ResetWalkingSpeed)
  (Variables|Default|SetCharge%20Attacking false)
  ;;;[1 1 1] rest
  (Utilities|FlowControl|Delay (Math|Random|RandomFloatinRange 0.7 2.5))
  ;;[1 1 1] attack again
  (Utilities|GolemDying?
    (:false
      (CallFunction|AttackTarget))))

(event Custom|Die
  ;[1 1 1] Damage
  (Audio|PlaySound2D "/Game/Sound/SoundFX/Cue_Death.Cue_Death" 2.0 0.3 0.0 0 0 false)
  (Actor|DestroyActor (Variables|/Game/BP/BP_GolemController.BP_GolemController_C|GetRock%20Actor (Variables|Default|GetGolem%20Controller)))
  (Class|PaperZDAnimInstance|JumptoNode (Variables|Default|GetABP%20Golem) "Die" "None"))

(event Custom|Alert/De-Alert
  (params (Alert? :type Boolean))
  (Default|ChangeGolemState (Variables|Default|GetGolem%20Controller) (select Alert? "NewEnumerator2" "NewEnumerator5"))
  (Rendering|SetVisibility (Variables|Default|GetAlert%20Marker) Alert? true)
  (if Alert?
    (Audio|PlaySound2D "/Game/Sound/SoundFX/Cue_Alert.Cue_Alert" 1.0 1.0 0.0 0 0)
    (Utilities|FlowControl|Delay 0.7)
    (CallFunction|AttackTarget)
    (else
      ;[1 1 1] Updated player's alerted actors list
      (Utilities|Array|RemoveItem (Variables|/Game/TopDown/Blueprints/BP_TopDownController.BP_TopDownController_C|GetAlerted%20Enemies (Variables|/Game/BP/BP_GameInstance.BP_GameInstance_C|GetTop%20Down%20Controller (Variables|Default|GetGame%20Instance))) self)
      (Variables|Default|SetTarget%20Enemy%20Actor 0)
      (Default|Patrol (Variables|Default|GetGolem%20Controller))
      (Variables|Default|SetCharge%20Attacking false)
      (Variables|Default|SetLeap%20Attacking false))))

(event Custom|Update%20De-alert%20Timer
  (if (and (Utilities|Array|IsEmpty (Variables|Default|GetDetected%20Enemies)) (not (Utilities|Time|IsValidTimerHandle (Variables|Default|GetDe-Alert%20Timer%20Handle))))
    ;[1 1 1] De-Alert Timer
    (bind _returnvalue (Utilities|Time|SetTimerbyEvent (delegate Custom|CustomEvent) (Variables|Default|GetTime%20until%20De-Alert)))
    (Variables|Default|SetDe-Alert%20Timer%20Handle _returnvalue)))

(event Custom|On%20Leap%20Attack%20Land
  (bind _self self)
  ;[1 1 1] Attack
  ;;[0 0 0] Leap to player
  (Variables|Default|SetLeap%20Attacking false)
  (Game|SpawnActorfromClass "/Game/BP/BP_Shockwave_Golem.BP_Shockwave_Golem_C" (Math|Transform|MakeTransform (Transformation|GetWorldLocation (Variables|Default|GetShockwave%20Spawn))) "AlwaysSpawn" "MultiplyWithRoot" _self (Variables|Default|GetShockwave%20Damage) _self)
  (CallFunction|GolemShockwaveFlash)
  ;;;[1 1 1] rest
  (Utilities|FlowControl|RetriggerableDelay (select (Variables|Default|GetLeap%20Attacking) 7.0 (Math|Random|RandomFloatinRange 1.0 2.5)))
  ;;;;[1 1 1] reset leap attack check
  (Variables|Default|SetLeap%20Attacking false)
  (Class|PrimitiveComponent|SetCastHiddenShadow (Variables|Default|GetFake%20Shadow) false)
  ;;[1 1 1] attack again
  (Utilities|GolemDying?
    (:false
      (CallFunction|AttackTarget))))

(event Custom|Golem%20Shockwave%20Flash
  (bind _paperflipbook (Variables|Default|GetPaperFlipbook))
  ;[1 1 1] Attack
  (Sprite|SetSpriteColor _paperflipbook "(R=0.447917,G=1.000000,B=0.490513,A=0.635294)")
  (Utilities|FlowControl|RetriggerableDelay 0.2)
  (Sprite|SetSpriteColor _paperflipbook (Variables|Default|GetOrig%20Color)))

(event Custom|CustomEvent
  ;[1 1 1] De-Alert Timer
  (CallFunction|Alert/De-Alert false)
  (Utilities|Time|ClearandInvalidateTimerbyHandle (Variables|Default|GetDe-Alert%20Timer%20Handle)))

(event Custom|Reset%20Walking%20Speed
  ;[1 1 1] Attack
  ;;[1 1 1] reset walk speed
  (Variables|/Script/Engine.CharacterMovementComponent|SetMaxWalkSpeed (Variables|Character|GetCharacterMovement) (Variables|Default|GetNormal%20Walk%20Speed)))

(event Custom|Revaluate%20Targets
  (bind _detected_enemies (Variables|Default|GetDetected%20Enemies))
  (bind _output (Utilities|Array|Get(acopy) _detected_enemies))
  (Utilities|IsValid (Variables|Default|GetTarget%20Enemy%20Actor)
    (:Is%20Valid
      (if (not (Utilities|Array|ContainsItem _detected_enemies (Variables|Default|GetTarget%20Enemy%20Actor)))
        (Utilities|IsValid _output :!label _label
          (:Is%20Valid
            (Variables|Default|SetTarget%20Enemy%20Actor _output))
          (:Is%20Not%20Valid
            (Utilities|Array|RemoveIndex _detected_enemies)
            (if (Utilities|Array|IsEmpty _detected_enemies)
              (CallFunction|UpdateDe-alertTimer)
              (else
                (goto _label)))))))
    (:Is%20Not%20Valid
      (goto _label))))

(event Custom|On%20Detected%20Actor%20Destroyed
  (params (DestroyedActor :type Actor%20Object%20Reference))
  (Utilities|Array|RemoveItem (Variables|Default|GetDetected%20Enemies) DestroyedActor)
  (CallFunction|RevaluateTargets))

(event EventBeginPlay
  (Utilities|FlowControl|Sequence
    (:then_0
      (bind _asabp_golem_e (Utilities|Casting|CastToABP_GolemE (Variables|/Script/PaperZD.PaperZDAnimationComponent|GetAnimInstance (Variables|Components|GetPaperZDAnimation))))
      (bind _output_get (Variables|Default|SetABP%20Golem _asabp_golem_e))
      (Variables|/Game/Animation/ABP_GolemE.ABP_GolemE_C|SetCharacter%20Movement _output_get (Variables|Character|GetCharacterMovement))
      (bind _asbp_game_instance (Utilities|Casting|CastToBP_GameInstance (Game|GetGameInstance)))
      (Variables|Default|SetGame%20Instance _asbp_game_instance)
      (Variables|Default|SetOrig%20Color (Class|PaperFlipbookComponent|GetSpriteColor (Variables|Default|GetPaperFlipbook))))
    (:then_1
      (bind _asbp_golem_controller (Utilities|Casting|CastToBP_GolemController (Pawn|GetController)))
      (bind _output_get_2 (Variables|Default|SetGolem%20Controller _asbp_golem_controller))
      (bind _output_get_3 (Variables|/Game/Animation/ABP_GolemE.ABP_GolemE_C|SetGolem%20Controller (Variables|Default|GetABP%20Golem) _output_get_2))
      (Variables|/Game/BP/BP_GolemController.BP_GolemController_C|SetGolm%20Character _output_get_3 self))
    (:then_2
      (Variables|Default|SetHealth (Variables|Default|GetMax%20Health)))))

(event EventTick
  (params (DeltaSeconds :type Float%20%28single-precision%29))
  (bind _charactermovement (Variables|Character|GetCharacterMovement))
  (bind _sprite_parnet (Variables|Default|GetSprite%20Parnet))
  (bind _returnvalue (Pawn|Components|CharacterMovement|GetLastUpdateVelocity _charactermovement))
  (bind _relativescale3d (Variables|/Script/Engine.SceneComponent|GetRelativeScale3D _sprite_parnet))
  (Transformation|SetWorldRotation (Variables|Default|GetParent%20No%20Rotation) "0, 0, 0" false false)
  ;[1 1 1] Sprite Flip
  (Transformation|SetRelativeScale3D _sprite_parnet (Math|Vector|MakeVector 1.0 (Math|Float|SelectFloat (* (.y _relativescale3d) -1.0) (.y _relativescale3d) (or (and (> (.y _relativescale3d) 0.0) (< (.y _returnvalue) 0.0)) (and (< (.y _relativescale3d) 0.0) (> (.y _returnvalue) 0.0)))) 1.0)))

(event EventOnLanded
  (params (Hit :type Hit%20Result%20Structure%20%28by%20ref%29))
  (if (and (Variables|Default|GetLeap%20Attacking) (Utilities|Enum|Equal(Enum) (Variables|/Game/BP/BP_GolemController.BP_GolemController_C|GetCurrent%20State (Variables|Default|GetGolem%20Controller)) "NewEnumerator2"))
    (CallFunction|OnLeapAttackLand)))

(event Game|Damage|EventAnyDamage
  (params (Damage :type Float%20%28single-precision%29) (DamageType :type Damage%20Type%20Object%20Reference) (InstigatedBy :type Controller%20Object%20Reference) (DamageCauser :type Actor%20Object%20Reference))
  ;[1 1 1] Damage
  (Utilities|GolemDying?
    (:false
      (bind _output_get (Variables|Default|SetHealth (- (Variables|Default|GetHealth) Damage)))
      (if (<= _output_get 0.0)
        (CallFunction|DamageFlash)
        (Default|ChangeGolemState (Variables|Default|GetGolem%20Controller) "NewEnumerator6")
        (else
          (Utilities|FlowControl|Sequence
            (:then_0
              (if (Utilities|IsLowHealth)
                (Utilities|FlowControl|DoOnce false
                  (:Completed
                    (Variables|Default|SetOrig%20Color "(R=1.000000,G=0.385417,B=0.385417,A=1.000000)")))))
            (:then_1
              (CallFunction|DamageFlash))))))))

(event Collision|EventHit
  (params (MyComp :type Primitive%20Component%20Object%20Reference) (Other :type Actor%20Object%20Reference) (OtherComp :type Primitive%20Component%20Object%20Reference) (bSelfMoved :type Boolean) (HitLocation :type Vector :default "0, 0, 0") (HitNormal :type Vector :default "0, 0, 0") (NormalImpulse :type Vector :default "0, 0, 0") (Hit :type Hit%20Result%20Structure%20%28by%20ref%29))
  (bind _hit_enemies (Variables|Default|GetHit%20Enemies))
  ;[1 1 1] Enemy who has not been hit yet?
  (if (and (Utilities|ActorIsEnemy? Other) (not (Utilities|Array|ContainsItem _hit_enemies Other)))
    (Utilities|GolemDying?
      (:false
        (Utilities|Array|Add _hit_enemies Other)
        (Game|Damage|ApplyPointDamage Other (Variables|Default|GetDamage) (Math|Vector|GetUnitDirection(Vector) (Transformation|GetActorLocation) (Transformation|GetActorLocation Other)) (Collision|MakeHitResult true false 0.0 0.0 HitLocation "0, 0, 0" "0,0,1" "0,0,1" 0 Other))
        (if (Variables|Default|GetCharge%20Attacking)
          (CallFunction|InvokeStopChargeAttack))))))

(fn ConstructionScript
  (Rendering|SetVisibility (Variables|Default|GetDetector) (Variables|Default|GetDebug%20Detector%20Volume?) false)
  (Rendering|SetVisibility (Variables|Default|GetAlert%20Marker) false true)
  (Class|PrimitiveComponent|SetCastHiddenShadow (Variables|Default|GetFake%20Shadow) false)
  (Collision|SetCollisionEnabled (Variables|Default|GetDetector) "NoCollision"))