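; BP_GroundFire is a blue ground fire hazard that ignites when it takes any damage.
; An optional retriggerable delay with random extra time then puts the FireBlue effect out.
; When player collision is enabled, the box overlap deals blue-fire point damage to player-tagged actors and launches characters away, scaled inversely by mass.
; The overlap does not check whether the fire is active.
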(event OnComponentBeginOverlap(Box)
  (params (OverlappedComponent :type Primitive%20Component%20Object%20Reference) (OtherActor :type Actor%20Object%20Reference) (OtherComp :type Primitive%20Component%20Object%20Reference) (OtherBodyIndex :type Integer) (bFromSweep :type Boolean) (SweepResult :type Hit%20Result%20Structure%20%28by%20ref%29))
  (bind _returnvalue (Transformation|GetActorLocation OtherActor))
  (bind _defaultsceneroot (Variables|Default|GetDefaultSceneRoot))
  (bind _returnvalue_2 (Transformation|GetWorldLocation _defaultsceneroot))
  (bind _returnvalue_3 (Math|Vector|GetUnitDirection(Vector) _returnvalue_2 _returnvalue))
  (if (Variables|Default|GetPlayer%20Collision)
    (if (Actor|ActorHasTag OtherActor "player")
      (Game|Damage|ApplyPointDamage OtherActor (Variables|Default|GetDamage) _returnvalue_3 (Collision|MakeHitResult false false 0.0 0.0 "0, 0, 0" "0, 0, 0" "0,0,1" "0,0,1" 0 0) 0 self "/Game/BP/DamageType_Fire_Blue.DamageType_Fire_Blue_C")
      (bind _ascharacter (Utilities|Casting|CastToCharacter OtherActor))
      ;[1 1 1] Apply Impulse, accountinmg for mass
      (Character|LaunchCharacter _ascharacter (* _returnvalue_3 (/ 3e+04 (Variables|/Script/Engine.CharacterMovementComponent|GetMass (Variables|/Script/Engine.Character|GetCharacterMovement _ascharacter)))) true true))))

(event EventBeginPlay)

(event Collision|EventActorBeginOverlap
  (params (OtherActor :type Actor%20Object%20Reference)))

(event EventTick
  (params (DeltaSeconds :type Float%20%28single-precision%29)))

(event Game|Damage|EventAnyDamage
  (params (Damage :type Float%20%28single-precision%29) (DamageType :type Damage%20Type%20Object%20Reference) (InstigatedBy :type Controller%20Object%20Reference) (DamageCauser :type Actor%20Object%20Reference))
  (bind _fire_blue (Variables|Default|GetFire_blue))
  (Components|Activation|Activate _fire_blue false)
  (if (Variables|Default|GetDactivate%20after%20delay)
    (Utilities|FlowControl|RetriggerableDelay (+ (Variables|Default|GetDeactivation%20Delay) (Math|Random|RandomFloatinRange 0.0 3.0)))
    (Components|Activation|Deactivate _fire_blue)))

(fn ConstructionScript)