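; BP_RisingIcon is an actor that floats an icon component from the actor's location up to an end-point component, then removes itself.
; On BeginPlay it plays the Rise timeline at a rate of one over RiseTime, lerping the icon parent's world position along the track.
; A halfway event calls an empty RiseHalfway hook, and two seconds after the timeline finishes, RiseFinished destroys the actor.
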(event Custom|Rise%20Halfway)

(event Custom|Rise%20Finished
  (Actor|DestroyActor))

(event EventBeginPlay
  (Components|Timeline|SetPlayRate (Variables|Default|GetRise) (Math|Float|Power (Variables|Default|GetRise%20Time) -1.0))
  (bind _newtrack_0 (Timeline|Rise PlayFromStart)
    (:Update
      (Transformation|SetWorldLocation (Variables|Default|GetIcon%20Parent) (Math|Vector|Lerp(Vector) (Transformation|GetActorLocation) (Transformation|GetWorldLocation (Variables|Default|GetEnd%20Pos)) _newtrack_0) false false))
    (:Finished
      (Utilities|FlowControl|Delay 2.0)
      (CallFunction|RiseFinished))
    (:halfway
      (CallFunction|RiseHalfway))))

(fn ConstructionScript)