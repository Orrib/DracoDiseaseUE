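; Dragon fire hazard, named for a window, that burns and knocks back the top-down player; it starts disabled and is toggled through the Box collision.
; Box overlaps count player-tagged contacts and deal one-off damage to bush-tagged actors.
; While the count is above zero, Tick applies fire damage every frame and calls the knockback.
; Knockback launches only a grounded player away from an origin component, with clamped distance falloff.
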(event OnComponentBeginOverlap(Box)
  (params (OverlappedComponent :type Primitive%20Component%20Object%20Reference) (OtherActor :type Actor%20Object%20Reference) (OtherComp :type Primitive%20Component%20Object%20Reference) (OtherBodyIndex :type Integer) (bFromSweep :type Boolean) (SweepResult :type Hit%20Result%20Structure%20%28by%20ref%29))
  (if (Actor|ActorHasTag OtherActor "player")
    (Math|Integer|IncrementInt (Variables|Default|GetColliders%20that%20detect%20player))
    (elif (Actor|ActorHasTag OtherActor "bush")
      (Game|Damage|ApplyDamage OtherActor 1.0 0 0))))

(event OnComponentEndOverlap(Box)
  (params (OverlappedComponent :type Primitive%20Component%20Object%20Reference) (OtherActor :type Actor%20Object%20Reference) (OtherComp :type Primitive%20Component%20Object%20Reference) (OtherBodyIndex :type Integer))
  (if (Actor|ActorHasTag OtherActor "player")
    (Math|Integer|DecrementInt (Variables|Default|GetColliders%20that%20detect%20player))))

(event Custom|Enable/Disable%20Fire
  (params (Enable? :type Boolean))
  (Collision|SetCollisionEnabled (Variables|Default|GetBox) (select Enable? "QueryOnly" "NoCollision"))
  (Variables|/Script/Engine.PrimitiveComponent|SetbGenerateOverlapEvents (Variables|Default|GetBox) Enable?))

(event EventBeginPlay
  (bind _asbp_top_down_character (Utilities|Casting|CastToBP_TopDownCharacter (Game|GetPlayerCharacter 0)))
  (Variables|Default|SetPlayer _asbp_top_down_character)
  (CallFunction|Enable/DisableFire false))

(event Collision|EventActorBeginOverlap
  (params (OtherActor :type Actor%20Object%20Reference)))

(event EventTick
  (params (DeltaSeconds :type Float%20%28single-precision%29))
  (if (> (Variables|Default|GetColliders%20that%20detect%20player) 0)
    (Game|Damage|ApplyDamage (Variables|Default|GetPlayer) (Variables|Default|GetDamage) 0 0 "/Game/BP/DamageType_Fire.DamageType_Fire_C")
    (Utilities|KnockbackCharacter (Variables|Default|GetPlayer) 1.0)))

(fn ConstructionScript)