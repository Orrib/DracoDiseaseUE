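; Monorail actor that sends randomly composed trains of empty, villager, guard or crystal cars along its spline while the player is inside its overlap area.
; A gate and random delay pace spawn attempts.
; Each train type rolls its length through nested weighted chances and picks cars from weighted lists.
; Cars are queued and spawned at the spline start on a looping buffer timer, which triggers another attempt once the queue empties.
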(event Custom|Spawn%20Train
  (params (Train%20Type :type Enum_MonorailTrainType%20Enum :default "NewEnumerator0"))
  (bind _returnvalue (Math|Random|RandomBoolwithWeight 0.3))
  (bind _array (Utilities|Array|MakeArray "NewEnumerator0" "NewEnumerator1" "NewEnumerator1"))
  (bind _array_2 (Utilities|Array|MakeArray "NewEnumerator2" "NewEnumerator2" "NewEnumerator2" "NewEnumerator0"))
  (bind _returnvalue_2 (select _returnvalue "NewEnumerator4" "NewEnumerator0"))
  (bind _array_3 (Utilities|Array|MakeArray "NewEnumerator3" _returnvalue_2))
  (switch Utilities|FlowControl|Switch|SwitchonEnum_MonorailTrainType Train%20Type
    (:NewEnumerator0
      ;[1 1 1] Empty
      (CallFunction|SpawnTrainCar "NewEnumerator0")
      (CallFunction|SpawnTrainCar "NewEnumerator0")
      (if (Math|Random|RandomBoolwithWeight 0.3)
        (CallFunction|SpawnTrainCar "NewEnumerator0")))
    (:NewEnumerator1
      ;[1 1 1] Vllager
      (CallFunction|SpawnTrainCar "NewEnumerator1")
      (CallFunction|SpawnRandomTrainCarfromList _array)
      (if (Math|Random|RandomBoolwithWeight 0.8)
        (CallFunction|SpawnRandomTrainCarfromList _array)
        (if (Math|Random|RandomBoolwithWeight 0.6)
          (CallFunction|SpawnRandomTrainCarfromList _array)
          (if (Math|Random|RandomBoolwithWeight 0.5)
            (CallFunction|SpawnRandomTrainCarfromList _array)
            (if (Math|Random|RandomBoolwithWeight 0.3)
              (CallFunction|SpawnRandomTrainCarfromList _array))))))
    (:NewEnumerator2
      ;[1 1 1] Guard
      (CallFunction|SpawnTrainCar "NewEnumerator2")
      (CallFunction|SpawnRandomTrainCarfromList _array_2)
      (if (Math|Random|RandomBoolwithWeight 0.8)
        (CallFunction|SpawnRandomTrainCarfromList _array_2)
        (if (Math|Random|RandomBoolwithWeight 0.6)
          (CallFunction|SpawnRandomTrainCarfromList _array_2)
          (if (Math|Random|RandomBoolwithWeight 0.5)
            (CallFunction|SpawnRandomTrainCarfromList _array_2)
            (if (Math|Random|RandomBoolwithWeight 0.3)
              (CallFunction|SpawnRandomTrainCarfromList _array_2))))))
    (:NewEnumerator3
      ;[1 1 1] Crystal
      (CallFunction|SpawnTrainCar "NewEnumerator3")
      (CallFunction|SpawnRandomTrainCarfromList _array_3)
      (if (Math|Random|RandomBoolwithWeight 0.8)
        (CallFunction|SpawnRandomTrainCarfromList _array_3)
        (if (Math|Random|RandomBoolwithWeight 0.6)
          (CallFunction|SpawnRandomTrainCarfromList _array_3)
          (if (Math|Random|RandomBoolwithWeight 0.5)
            (CallFunction|SpawnRandomTrainCarfromList _array_3)
            (if (Math|Random|RandomBoolwithWeight 0.3)
              (CallFunction|SpawnRandomTrainCarfromList _array_3))))))))

(event Custom|Spawn%20TrainCar
  (params (Traincar%20Type :type Enum_MonorailTraincarType%20Enum :default "NewEnumerator0"))
  (bind _spline (Variables|Default|GetSpline))
  (bind _train_car_queue (Variables|Default|GetTrain%20Car%20Queue))
  (bind _returnvalue (Spline|GetTransformatSplinePoint _spline 0 "World" false))
  (bind _output (Utilities|Array|Get(acopy) _train_car_queue))
  (Utilities|Array|Add (Variables|Default|GetTrain%20Car%20Queue) Traincar%20Type)
  (if (not (Utilities|Time|IsValidTimerHandle (Variables|Default|GetTrain%20Car%20Queue%20Timer)))
    (Utilities|FlowControl|Sequence
      (:then_0
        (bind _output_get (Variables|Default|SetTrain%20Car%20Class (Utilities|Select :Index _output :NewEnumerator0 "/Game/BP/BP_MonorailTraincar.BP_MonorailTraincar_C" :NewEnumerator1 "/Game/BP/BP_MonorailTraincar_Villager.BP_MonorailTraincar_Villager_C" :NewEnumerator2 "/Game/BP/BP_MonorailTraincar_Guard.BP_MonorailTraincar_Guard_C" :NewEnumerator3 "/Game/BP/BP_MonorailTraincar_Crystal.BP_MonorailTraincar_Crystal_C" :NewEnumerator4 "/Game/BP/BP_MonorailTraincar_Crystal_Red.BP_MonorailTraincar_Crystal_Red_C")))
        (Game|SpawnActorfromClass _output_get (Math|Transform|MakeTransform (.location _returnvalue) (Math|Rotator|MakeRotator (.roll (.rotation _returnvalue)) (.pitch (.rotation _returnvalue)) (+ (.yaw (.rotation _returnvalue)) (select (Variables|Default|GetTrain%20Faces%20Right?) 0.0 1.8e+02))) (.scale _returnvalue)) "AlwaysSpawn" "MultiplyWithRoot" 0 (Variables|Default|GetSpline) (Variables|Default|GetTrain%20Time%20to%20Complete%20Spline) _output 0)
        (Utilities|Array|RemoveIndex _train_car_queue))
      (:then_1
        (bind _returnvalue_2 (Utilities|Time|SetTimerbyEvent (delegate Custom|CustomEvent) (Variables|Default|GetTrain%20Car%20Spawn%20Buffer%20Time) true))
        (Variables|Default|SetTrain%20Car%20Queue%20Timer _returnvalue_2)))))

(event Custom|Spawn%20Random%20Train%20Car%20From%20List
  (params (List%20of%20Possible%20Types :type Array%20of%20Enum_MonorailTraincarType%20Enums :default "NewEnumerator0"))
  (CallFunction|SpawnTrainCar (.OutItem (Utilities|Array|Random List%20of%20Possible%20Types))))

(event Custom|CustomEvent
  (bind _spline (Variables|Default|GetSpline))
  (bind _train_car_queue (Variables|Default|GetTrain%20Car%20Queue))
  (bind _returnvalue (Spline|GetTransformatSplinePoint _spline 0 "World" false))
  (bind _output (Utilities|Array|Get(acopy) _train_car_queue))
  (if (Utilities|Array|IsEmpty _train_car_queue)
    (Utilities|Time|ClearandInvalidateTimerbyHandle (Variables|Default|GetTrain%20Car%20Queue%20Timer))
    (CallFunction|AttemptSpawnRandomTrain)
    (else
      (bind _output_get (Variables|Default|SetTrain%20Car%20Class (Utilities|Select :Index _output :NewEnumerator0 "/Game/BP/BP_MonorailTraincar.BP_MonorailTraincar_C" :NewEnumerator1 "/Game/BP/BP_MonorailTraincar_Villager.BP_MonorailTraincar_Villager_C" :NewEnumerator2 "/Game/BP/BP_MonorailTraincar_Guard.BP_MonorailTraincar_Guard_C" :NewEnumerator3 "/Game/BP/BP_MonorailTraincar_Crystal.BP_MonorailTraincar_Crystal_C" :NewEnumerator4 "/Game/BP/BP_MonorailTraincar_Crystal_Red.BP_MonorailTraincar_Crystal_Red_C")))
      (Game|SpawnActorfromClass _output_get (Math|Transform|MakeTransform (.location _returnvalue) (Math|Rotator|MakeRotator (.roll (.rotation _returnvalue)) (.pitch (.rotation _returnvalue)) (+ (.yaw (.rotation _returnvalue)) (select (Variables|Default|GetTrain%20Faces%20Right?) 0.0 1.8e+02))) (.scale _returnvalue)) "AlwaysSpawn" "MultiplyWithRoot" 0 (Variables|Default|GetSpline) (Variables|Default|GetTrain%20Time%20to%20Complete%20Spline) _output 0)
      (Utilities|Array|RemoveIndex _train_car_queue))))

(event Custom|Spawn%20Random%20Train
  (CallFunction|SpawnTrain (.OutItem (Utilities|Array|Random (Variables|Default|GetPossible%20Train%20Types)))))

(event Custom|Attempt%20Spawn%20Random%20Train
  (Utilities|FlowControl|Sequence
    (:then_0
      _)
    (:then_1
      (Utilities|FlowControl|Delay (Math|Random|RandomFloatinRange (Variables|Default|GetMin%20Time%20Between%20Trains) (Variables|Default|GetMax%20Time%20Between%20Trains)))
      (Utilities|FlowControl|Sequence
        (:then_0
          (goto _label Open))
        (:then_1
          _))))
  (Utilities|FlowControl|Gate false :!label _label
    (:Exit
      (if (Variables|Default|GetPlayer%20Near)
        (CallFunction|SpawnRandomTrain)
        (goto _label Close)))))

(event Collision|EventActorBeginOverlap
  (params (OtherActor :type Actor%20Object%20Reference))
  (if (Actor|ActorHasTag OtherActor "player")
    (Variables|Default|SetPlayer%20Near true)
    (CallFunction|AttemptSpawnRandomTrain)))

(event Collision|EventActorEndOverlap
  (params (OtherActor :type Actor%20Object%20Reference))
  (if (Actor|ActorHasTag OtherActor "player")
    (Variables|Default|SetPlayer%20Near false)))

(fn ConstructionScript)