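; BP_Trigger_MidscreenMessage is a trigger actor that shows or hides a mid-screen text message when an actor tagged "player" overlaps it.
; On BeginPlay it caches BP_GameInstance, then on overlap calls its GameController's SetMidscreenMessageUninteractable.
; The message text, show/hide flag and auto-hide delay come from the trigger's variables, and a once-only option destroys the trigger after it fires.
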(event EventBeginPlay
  (bind _asbp_game_instance (Utilities|Casting|CastToBP_GameInstance (Game|GetGameInstance)))
  (Variables|Default|SetBP%20Game%20Instance _asbp_game_instance))

(event Collision|EventActorBeginOverlap
  (params (OtherActor :type Actor%20Object%20Reference))
  (if (Actor|ActorHasTag OtherActor "player")
    (Default|SetMidscreenMessage-Uninteractable (Variables|/Game/BP/BP_GameInstance.BP_GameInstance_C|GetGame%20Controller (Variables|Default|GetBP%20Game%20Instance)) (Variables|Default|GetShow/%20Hide%20Midscreen%20Message%20%28T/f%29) (Variables|Default|GetMessage%20Text) (Variables|Default|GetHide%20After%20Seconds%20%280%20to%20prevent%20hiding%29))
    (if (Variables|Default|GetOnly%20Show%20Once)
      (Actor|DestroyActor))))

(event EventTick
  (params (DeltaSeconds :type Float%20%28single-precision%29)))

(fn ConstructionScript)