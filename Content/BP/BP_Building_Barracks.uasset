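; Barracks building Blueprint that lets the player buy kingdom ally NPCs with coins.
; It extends a parent building, using a clickable plane that is hidden at construction and shown only in strategy mode, with a material swap on cursor hover.
; Clicking the plane deducts coins through the top-down controller and spawns an ally at the Spawn point, or plays an error sound with a popup when funds are short.
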(event OnBeginCursorOver(Plane)
  (params (TouchedComponent :type Primitive%20Component%20Object%20Reference))
  (Rendering|Material|SetMaterial (Variables|Default|GetPlane) 0 "/Game/Materials/M_Emissive.M_Emissive"))

(event OnEndCursorOver(Plane)
  (params (TouchedComponent :type Primitive%20Component%20Object%20Reference))
  (Rendering|Material|SetMaterial (Variables|Default|GetPlane) 0 "/Engine/BasicShapes/BasicShapeMaterial.BasicShapeMaterial"))

(event OnClicked(Plane)
  (params (TouchedComponent :type Primitive%20Component%20Object%20Reference) (ButtonPressed :type Key%20Structure :default "None"))
  (bind _game_instance (Variables|Default|GetGame%20Instance))
  (bind _top_down_controller (Variables|/Game/BP/BP_GameInstance.BP_GameInstance_C|GetTop%20Down%20Controller _game_instance))
  (if (>= (Variables|/Game/TopDown/Blueprints/BP_TopDownController.BP_TopDownController_C|GetCoins _top_down_controller) 3)
    (Audio|PlaySound2D "/Game/Sound/SoundFX/Cue_Pickup.Cue_Pickup" 1.0 0.7 0.0 0 0)
    (Default|AddCoins _top_down_controller -3)
    (Game|SpawnActorfromClass "/Game/TopDown/Blueprints/BP_NPC_KingdomAlly.BP_NPC_KingdomAlly_C" (Math|Transform|MakeTransform (.location (Transformation|GetWorldTransform (Variables|Default|GetSpawn))) "0, 0, 0" "1.000000,1.000000,1.000000") "AdjustIfPossibleButAlwaysSpawn" "MultiplyWithRoot" 0 0)
    (else
      (Audio|PlaySound2D "/Game/Sound/SoundFX/Cue_Error.Cue_Error" 1.0 1.0 0.0 0 0)
      (Default|CreatePopup (Variables|/Game/TopDown/Blueprints/BP_TopDownController.BP_TopDownController_C|GetGame%20Controller _top_down_controller) false false false "Need more coins!" "You're broke! Get more coins first." "Ok"))))

(event Custom|On%20Enter/Exit%20Strategy%20Mode
  (params (Enter/Exit :type Boolean))
  (|CallParentFunction Enter/Exit)
  (Rendering|SetVisibility (Variables|Default|GetPlane) Enter/Exit true))

(event EventBeginPlay
  (|CallParentFunction))

(event Collision|EventActorBeginOverlap
  (params (OtherActor :type Actor%20Object%20Reference)))

(event EventTick
  (params (DeltaSeconds :type Float%20%28single-precision%29)))

(fn ConstructionScript
  (|CallParentFunction)
  (CallFunction|OnEnter/ExitStrategyMode false))