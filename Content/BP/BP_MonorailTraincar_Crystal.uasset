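; Monorail traincar Blueprint that carries a randomized arrangement of crystals.
; The construction script loops over the direct children of the Crystals component, hiding each at random or adding a world-space delta transform.
; That transform has a slight random roll and pitch, any yaw, and a random unit vector as scale.
; The event graph holds only disabled default events, so the Blueprint adds no runtime logic.
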(event EventBeginPlay
  (|CallParentFunction) ; This node is disabled and will not be called.\nDrag off pins to build functionality.
)

(event Collision|EventActorBeginOverlap
  (params (OtherActor :type Actor%20Object%20Reference))
  (|CallParentFunction OtherActor) ; This node is disabled and will not be called.\nDrag off pins to build functionality.
)

(event EventTick
  (params (DeltaSeconds :type Float%20%28single-precision%29))
  (|CallParentFunction DeltaSeconds) ; This node is disabled and will not be called.\nDrag off pins to build functionality.
)

(fn ConstructionScript
  (|CallParentFunction)
  (for _array_element (Components|GetChildrenComponents (Variables|Default|GetCrystals) false)
    (if (Math|Random|RandomBool)
      (Class|SceneComponent|AddWorldTransform _array_element (Math|Transform|MakeTransform "0, 0, 0" (Math|Rotator|MakeRotator (Math|Random|RandomFloatinRange 5.0 1e+01) (Math|Random|RandomFloatinRange 0.0 1e+01) (Math|Random|RandomFloatinRange 0.0 3.6e+02)) (Math|Random|RandomUnitVector)) false false)
      (else
        (Rendering|SetVisibility _array_element false false)))))