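; BP_CommanderDragonFireFromAbove is a timed blue fire effect actor, named as a commander dragon's fire attack from above.
; On BeginPlay, a sequence runs two delay chains: one switches FireBlue off after a short time.
; The other holds two larger blue fire components off, activates them shortly before FireBlue stops, deactivates them after a longer burn, then destroys the actor following a final delay.
; The file contains no damage or movement logic.
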(event EventBeginPlay
  (bind _fire_blue_larger (Variables|Default|GetFire_blue_larger))
  (Utilities|FlowControl|Sequence
    (:then_0
      (Utilities|FlowControl|Delay 3.0)
      (Components|Activation|SetActive (Variables|Default|GetFire_blue) false false))
    (:then_1
      (Components|Activation|SetActive _fire_blue_larger false false)
      (Utilities|FlowControl|Delay 2.0)
      (Components|Activation|SetActive (Variables|Default|GetFire_blue_larger1) true false)
      (Utilities|FlowControl|Delay 1e+01)
      (Components|Activation|SetActive _fire_blue_larger false false)
      (Utilities|FlowControl|Delay 4.0)
      (Actor|DestroyActor))))

(fn ConstructionScript)