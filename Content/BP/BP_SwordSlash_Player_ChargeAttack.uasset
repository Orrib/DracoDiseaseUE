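; Player charge-attack sword slash whose strength depends on how long the attack was charged and on acquired upgrades.
; The construction script normalizes ChargeTime, with a higher cap under Steel Tide, to drive sprite darkening, damage, scale and duration, with Focus Strike boosting damage.
; On BeginPlay, a long enough charge with Steel Tide fires four staggered kinetic wave actors from separate spawn points, mirrored according to the player's yaw.
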(event Custom|Spawn%20Kinetic%20Wave
  (params (Spawn%20Point :type Scene%20Component%20Object%20Reference))
  (bind _player_flipped_ (Variables|Default|GetPlayer%20Flipped?))
  (bind _returnvalue (Game|SpawnActorfromClass "/Game/BP/BP_SwordSlash_Player_ChargeAttackWave.BP_SwordSlash_Player_ChargeAttackWave_C" (Math|Transform|MakeTransform (Transformation|GetWorldLocation Spawn%20Point) (Transformation|GetActorRotation) (Math|Vector|MakeVector 1.0 1.0 (select _player_flipped_ 1.0 -1.0))) "AlwaysSpawn" "MultiplyWithRoot" 0 0))
  (if (not _player_flipped_)
    (Transformation|SetRelativeScale3D (Variables|/Game/BP/BP_SwordSlash.BP_SwordSlash_C|GetSwordSlash _returnvalue) (Math|Vector|MakeVector (.x (Variables|/Script/Engine.SceneComponent|GetRelativeScale3D (Variables|/Game/BP/BP_SwordSlash.BP_SwordSlash_C|GetSwordSlash _returnvalue))) (.y (Variables|/Script/Engine.SceneComponent|GetRelativeScale3D (Variables|/Game/BP/BP_SwordSlash.BP_SwordSlash_C|GetSwordSlash _returnvalue))) (* (.z (Variables|/Script/Engine.SceneComponent|GetRelativeScale3D (Variables|/Game/BP/BP_SwordSlash.BP_SwordSlash_C|GetSwordSlash _returnvalue))) -1.0)))))

(event EventBeginPlay
  (bind _orig_rotation (Variables|Default|GetOrig%20Rotation))
  (bind _yaw (Math|Rotator|BreakRotator _orig_rotation))
  (|CallParentFunction)
  (if (and (> (Variables|Default|GetCharge%20Time) 3.0) (Variables|Default|GetSteel%20Tide%20Acquired))
    (Variables|Default|SetPlayer%20Flipped? (not (and (< _yaw 9e+01) (> _yaw -9e+01))))
    (CallFunction|SpawnKineticWave (Variables|Default|GetKinetic%20Wave%20Spawn%20Point_1))
    (Utilities|FlowControl|Delay 0.12)
    (CallFunction|SpawnKineticWave (Variables|Default|GetKinetic%20Wave%20Spawn%20Point_2))
    (Utilities|FlowControl|Delay 0.12)
    (CallFunction|SpawnKineticWave (Variables|Default|GetKinetic%20Wave%20Spawn%20Point_3))
    (Utilities|FlowControl|Delay 0.2)
    (CallFunction|SpawnKineticWave (Variables|Default|GetKinetic%20Wave%20Spawn%20Point_4))))

(event Collision|EventActorBeginOverlap
  (params (OtherActor :type Actor%20Object%20Reference))
  (|CallParentFunction OtherActor) ; This node is disabled and will not be called.\nDrag off pins to build functionality.
)

(event EventTick
  (params (DeltaSeconds :type Float%20%28single-precision%29))
  (|CallParentFunction DeltaSeconds) ; This node is disabled and will not be called.\nDrag off pins to build functionality.
)

(fn ConstructionScript
  (bind _charge_time (Variables|Default|GetCharge%20Time))
  (bind _slash_origin (Variables|Default|GetSlash%20Origin))
  (bind _steel_tide_acquired (Variables|Default|GetSteel%20Tide%20Acquired))
  (bind _returnvalue (select _steel_tide_acquired 3.0 2.0))
  (bind _returnvalue_2 (Math|Float|Clamp(Float) _charge_time 0.0 _returnvalue))
  (bind _returnvalue_3 (Math|Float|NormalizetoRange _returnvalue_2 0.0 _returnvalue))
  (bind _returnvalue_4 (+ _returnvalue_3 1.0))
  (|CallParentFunction)
  (Sprite|SetSpriteColor (Variables|Default|GetSwordSlash) (Math|Color|Lerp(LinearColor) "(R=0.494792,G=0.494792,B=0.494792,A=1.000000)" (select _steel_tide_acquired "(R=0.000000,G=0.000000,B=0.000000,A=1.000000)" "(R=0.125000,G=0.125000,B=0.125000,A=1.000000)") _returnvalue_3))
  (Variables|Default|SetDamage (* (Math|Float|Clamp(Float) (* (* (Variables|Default|GetDamage) (select _steel_tide_acquired 1.0 0.8)) _returnvalue_3) (Variables|Default|GetMin%20Damage) 5e+01) (select (Variables|Default|GetFocus%20Strike%20Acquired) 1.5 1.0)))
  (Transformation|SetRelativeScale3D _slash_origin (* (Variables|/Script/Engine.SceneComponent|GetRelativeScale3D _slash_origin) (Math|Float|Clamp(Float) _returnvalue_4 1.0 1.5)))
  (Variables|Default|SetSlash%20Duration (select (> (Variables|Default|GetCharge%20Time) 3.0) 1.2 (* (Variables|Default|GetSlash%20Duration) _returnvalue_4))))