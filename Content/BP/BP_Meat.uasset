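; BP_Meat is a health pickup that rewards the player when collected, built on a parent pickup class.
; On pickup it grants XP through the game controller and applies its HealthReward to the player controller.
; It then triggers a meat flash on the lighting controller, notifies the UI and plays a pitched-down 2D sound.
; The parent's pickup logic runs last, and BeginPlay and construction only call the parent.
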(event EventBeginPlay
  (|CallParentFunction))

(event EventOnPickup
  (params (Player%20Controller :type BP%20Top%20Down%20Controller%20Object%20Reference))
  (bind _game_instance (Variables|/Game/TopDown/Blueprints/BP_TopDownController.BP_TopDownController_C|GetGame%20Instance Player%20Controller))
  (Utilities|FlowControl|Sequence
    (:then_0
      (Default|AddXP (Variables|/Game/TopDown/Blueprints/BP_TopDownController.BP_TopDownController_C|GetGame%20Controller Player%20Controller) 10)
      (Default|ApplyHealth Player%20Controller (Variables|Default|GetHealth%20Reward))
      (Default|FlashMeatPickupEffect (Variables|/Game/BP/BP_GameInstance.BP_GameInstance_C|GetLighting%20Controller _game_instance))
      (Default|OnHealthPickup (Variables|/Game/BP/BP_GameController.BP_GameController_C|GetUI (Variables|/Game/BP/BP_GameInstance.BP_GameInstance_C|GetGame%20Controller _game_instance)))
      (Audio|PlaySound2D "/Game/Sound/SoundFX/Cue_Pickup.Cue_Pickup" 1.2 0.8 0.0 0 0))
    (:then_1
      (|CallParentFunction Player%20Controller))))

(fn ConstructionScript
  (|CallParentFunction))