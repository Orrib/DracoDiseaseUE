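; A physics-driven projectile actor that deals point damage to enemies and "box"-tagged actors it overlaps.
; Launch sets the mesh's linear velocity directly.
; On overlap, a HitActors list ensures each actor is handled once, then an allegiance macro filters enemies before applying damage and playing a sword-hit sound.
; An older tag-based damage chain remains in the graph but is disconnected.
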(event Custom|Launch
  (params (Velocity :type Vector))
  ;[1 1 1] Launch
  (Physics|SetPhysicsLinearVelocity (Variables|Default|GetProjectile%20Mesh) Velocity false "None"))

(event Collision|EventActorBeginOverlap
  (params (OtherActor :type Actor%20Object%20Reference))
  (bind _hit_actors (Variables|Default|GetHit%20Actors))
  (if (not (Utilities|Array|ContainsItem _hit_actors OtherActor))
    (Utilities|Array|Add _hit_actors OtherActor)
    ;[1 1 1] enemy
    (Utilities|IsActorAnEnemy?(Macro) (Variables|Default|GetAllegiance) OtherActor
      (:Is%20Enemy
        ;[1 1 1] damage
        (Game|Damage|ApplyPointDamage OtherActor (Variables|Default|GetDamage) (Math|Vector|GetUnitDirection(Vector) (Transformation|GetActorLocation) (Transformation|GetActorLocation OtherActor)) (Collision|MakeHitResult false true 0.0 0.0 "0, 0, 0" "0, 0, 0" "0,0,1" "0,0,1" 0 0) (Pawn|GetController (Variables|Actor|GetInstigator)) self :!label _label)
        (Audio|PlaySound2D "/Game/Sound/SoundFX/Cue_Sword_Hit.Cue_Sword_Hit" 1.0 1.0 0.0 0 0 false))
      (:Not%20Enemy
        ;[1 1 1] box
        (if (Actor|ActorHasTag OtherActor "box")
          (goto _label))))))

(event EventTick
  (params (DeltaSeconds :type Float%20%28single-precision%29)))

(fn ConstructionScript)