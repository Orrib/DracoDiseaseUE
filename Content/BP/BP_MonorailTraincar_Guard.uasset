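; Monorail traincar variant that carries up to two guard NPCs, randomized at construction.
; The construction script loops over Spine skeleton renderers, randomly hiding them or picking a Kingsguard or basic soldier PaperZD anim class.
; A FlipFlop on the hide branch turns every second hide into a guard, so at least one appears.
; Tick calls the parent, then zeroes both guards' world rotation so they ignore the car's rotation.
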(event EventBeginPlay
  (|CallParentFunction) ; This node is disabled and will not be called.\nDrag off pins to build functionality.
)

(event Collision|EventActorBeginOverlap
  (params (OtherActor :type Actor%20Object%20Reference))
  (|CallParentFunction OtherActor) ; This node is disabled and will not be called.\nDrag off pins to build functionality.
)

(event EventTick
  (params (DeltaSeconds :type Float%20%28single-precision%29))
  (|CallParentFunction DeltaSeconds)
  (Transformation|SetWorldRotation (Variables|Default|GetGuard1) "0, 0, 0" false false))

(fn ConstructionScript
  (|CallParentFunction)
  (for _array_element (Actor|GetComponentsByClass "/Script/SpinePlugin.SpineSkeletonRendererComponent")
    (if (Math|Random|RandomBool)
      (Class|PaperZDAnimationComponent|SetAnimInstanceClass (Variables|Default|GetPaperZDAnimation) (select (Math|Random|RandomBool) "/Game/Animation/ABP_StaticNPC_Kingsguard.ABP_StaticNPC_Kingsguard_C" "/Game/Animation/ABP_StaticNPC_BasicSoldier.ABP_StaticNPC_BasicSoldier_C") :!label _label)
      (else
        ;[1 1 1] ensure at least one guard will appear
        (Utilities|FlowControl|FlipFlop
          (:A
            (Rendering|SetVisibility _array_element false false))
          (:B
            (goto _label)))))))