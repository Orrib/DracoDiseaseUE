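; Interactable actor that shows a widget UI when a player-tagged actor enters its Detector volume and hides it on exit.
; BeginPlay links the widget to the actor and binds its lore button to a handler, which is empty here.
; Show/HideWidgetUI toggles widget collision and calls RevealHide.
; InstantHideWidgetUI can close a gate that skips the next RevealHide hide, then reopens, avoiding a hiding bug.
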(event OnComponentBeginOverlap(Detector)
  (params (OverlappedComponent :type Primitive%20Component%20Object%20Reference) (OtherActor :type Actor%20Object%20Reference) (OtherComp :type Primitive%20Component%20Object%20Reference) (OtherBodyIndex :type Integer) (bFromSweep :type Boolean) (SweepResult :type Hit%20Result%20Structure%20%28by%20ref%29))
  (if (Actor|ActorHasTag OtherActor "player")
    (CallFunction|Show/HideWidgetUI true)))

(event OnComponentEndOverlap(Detector)
  (params (OverlappedComponent :type Primitive%20Component%20Object%20Reference) (OtherActor :type Actor%20Object%20Reference) (OtherComp :type Primitive%20Component%20Object%20Reference) (OtherBodyIndex :type Integer))
  (if (Actor|ActorHasTag OtherActor "player")
    (CallFunction|Show/HideWidgetUI false)))

(event Custom|Show/Hide%20Widget%20UI
  (params (Show? :type Boolean))
  (bind _widget_interactable_ui (Variables|Default|GetWidget%20Interactable%20UI))
  (bind _widget (Variables|Default|GetWidget))
  (if Show?
    (Collision|SetCollisionEnabled _widget "QueryOnly")
    (Default|Reveal/Hide _widget_interactable_ui true)
    (else
      (Collision|SetCollisionEnabled _widget "NoCollision")
      (Utilities|FlowControl|Sequence
        (:then_0
          ;[1 1 1] Instant Hide Gate prevents hiding bug
          (Utilities|FlowControl|Gate false :!label _label
            (:Exit
              (Default|Reveal/Hide _widget_interactable_ui false))))
        (:then_1
          (goto _label Open))))))

(event Custom|Instant%20Hide%20Widget%20UI
  (params (Prevent%20Next%20"Hide%20Widget%20UI" :type Boolean))
  (bind _widget_interactable_ui (Variables|Default|GetWidget%20Interactable%20UI))
  (Default|InstantHide _widget_interactable_ui)
  (Collision|SetCollisionEnabled (Variables|Default|GetWidget) "NoCollision")
  (if Prevent%20Next%20"Hide%20Widget%20UI"
    ;[1 1 1] Instant Hide Gate prevents hiding bug
    (Utilities|FlowControl|Gate false) ; enters at Close
  ))

(event Custom|On%20Clicked%20Lore%20Button)

(event EventBeginPlay
  (bind _widget (Variables|Default|GetWidget))
  (Development|SetHiddeninGame _widget false false)
  (bind _aswidget_interactable_ui (Utilities|Casting|CastToWidget_InteractableUI (UserInterface|GetWidget _widget)))
  (bind _output_get (Variables|Default|SetWidget%20Interactable%20UI _aswidget_interactable_ui))
  (Variables|/Game/UI/Widget_InteractableUI.Widget_InteractableUI_C|SetBP%20Interactable _output_get self)
  (EventDispatchers|BindEventtoOnClickedLoreButton _output_get (delegate Custom|On%20Clicked%20Lore%20Button))
  (CallFunction|InstantHideWidgetUI false))

(event Collision|EventActorBeginOverlap
  (params (OtherActor :type Actor%20Object%20Reference)))

(event EventTick
  (params (DeltaSeconds :type Float%20%28single-precision%29)))

(fn ConstructionScript
  (Rendering|SetCastShadow (Variables|Default|GetWidget) false))