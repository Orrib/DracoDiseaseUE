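; A monorail traincar variant carrying four crystal cluster meshes with red-tinted emissive variation.
; After running the parent construction script, it independently gives each cluster either the standard or the red emissive material at random.
; The event graph holds only disabled stubs, so all of its own logic runs at construction.
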(event EventBeginPlay
  (|CallParentFunction) ; This node is disabled and will not be called.\nDrag off pins to build functionality.
)

(event Collision|EventActorBeginOverlap
  (params (OtherActor :type Actor%20Object%20Reference))
  (|CallParentFunction OtherActor) ; This node is disabled and will not be called.\nDrag off pins to build functionality.
)

(event EventTick
  (params (DeltaSeconds :type Float%20%28single-precision%29))
  (|CallParentFunction DeltaSeconds) ; This node is disabled and will not be called.\nDrag off pins to build functionality.
)

(fn ConstructionScript
  (bind _returnvalue (Math|Random|RandomBool))
  (bind _returnvalue_2 (select _returnvalue "/Game/Lighting/BlockoutAssets_City/BlockoutMaterials/M_ttrubenk_emissive_dramatic_Inst.M_ttrubenk_emissive_dramatic_Inst" "/Game/Lighting/BlockoutAssets_City/BlockoutMaterials/M_ttrubenk_emissive_dramatic_Inst_Red.M_ttrubenk_emissive_dramatic_Inst_Red"))
  (|CallParentFunction)
  (Rendering|Material|SetMaterial (Variables|Default|GetSM_PillarStructure_CityAsset_Crystal_Cluster1) 0 _returnvalue_2)
  (Rendering|Material|SetMaterial (Variables|Default|GetSM_PillarStructure_CityAsset_Crystal_Cluster2) 0 _returnvalue_2)
  (Rendering|Material|SetMaterial (Variables|Default|GetSM_PillarStructure_CityAsset_Crystal_Cluster3) 0 _returnvalue_2)
  (Rendering|Material|SetMaterial (Variables|Default|GetSM_PillarStructure_CityAsset_Crystal_Cluster4) 0 _returnvalue_2))