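; Trigger volume Blueprint that fades a referenced post process volume in while an actor tagged "player" overlaps it and out when that actor leaves.
; An optional BeginPlay setup makes the volume unbound, disables it, and scales the timeline play rate to the inverse of the transition time.
; Overlaps play or reverse the timeline, which drives blend weight and disables the volume once the weight returns to zero.
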(event EventBeginPlay
  (bind _post_process_volume (Variables|Default|GetPost%20Process%20Volume))
  (if (Variables|Default|GetMake%20Post%20Process%20Unbound%20on%20Start)
    (Variables|/Script/Engine.PostProcessVolume|SetbUnbound _post_process_volume true)
    (Variables|/Script/Engine.PostProcessVolume|SetbEnabled _post_process_volume false)
    (Components|Timeline|SetPlayRate (Variables|Default|GetTimeline) (Math|Float|Power (Variables|Default|GetPost%20Process%20Transition%20Time) -1.0))))

(event Collision|EventActorBeginOverlap
  (params (OtherActor :type Actor%20Object%20Reference))
  (bind _post_process_volume (Variables|Default|GetPost%20Process%20Volume))
  (if (Actor|ActorHasTag OtherActor "player")
    (Variables|/Script/Engine.PostProcessVolume|SetbEnabled (Variables|Default|GetPost%20Process%20Volume) true)
    (bind _newtrack_0 (Timeline|Timeline Play)
      (:Update
        (Variables|/Script/Engine.PostProcessVolume|SetBlendWeight _post_process_volume _newtrack_0))
      (:Finished
        (Variables|/Script/Engine.PostProcessVolume|SetbEnabled _post_process_volume (not (== _newtrack_0 0.0)))))))

(event Collision|EventActorEndOverlap
  (params (OtherActor :type Actor%20Object%20Reference))
  (bind _post_process_volume (Variables|Default|GetPost%20Process%20Volume))
  (if (Actor|ActorHasTag OtherActor "player")
    (Variables|/Script/Engine.PostProcessVolume|SetbEnabled (Variables|Default|GetPost%20Process%20Volume) true)
    (bind _newtrack_0 (Timeline|Timeline Reverse)
      (:Update
        (Variables|/Script/Engine.PostProcessVolume|SetBlendWeight _post_process_volume _newtrack_0))
      (:Finished
        (Variables|/Script/Engine.PostProcessVolume|SetbEnabled _post_process_volume (not (== _newtrack_0 0.0)))))))

(fn ConstructionScript)