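; A torch stand variant for a special torch in Chapter 1 Part 1, built as a child Blueprint that extends its parent's torch toggle.
; Its Activate/DeactivateTorch override runs the parent logic, then passes through a DoOnce, so only the first call triggers the special behavior, whether activating or deactivating.
; That call reaches the GameController through BP_GameInstance and runs ActivateSpecialTorchChap1Part1 with this stand as the argument.
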(event EventBeginPlay
  (|CallParentFunction) ; This node is disabled and will not be called.\nDrag off pins to build functionality.
)

(event Collision|EventActorBeginOverlap
  (params (OtherActor :type Actor%20Object%20Reference))
  (|CallParentFunction OtherActor) ; This node is disabled and will not be called.\nDrag off pins to build functionality.
)

(event EventTick
  (params (DeltaSeconds :type Float%20%28single-precision%29))
  (|CallParentFunction DeltaSeconds) ; This node is disabled and will not be called.\nDrag off pins to build functionality.
)

(event EventActivate/DeactivateTorch
  (params (Torch%20Activated :type Boolean))
  (|CallParentFunction Torch%20Activated)
  (Utilities|FlowControl|DoOnce false
    (:Completed
      (bind _asbp_game_instance (Utilities|Casting|CastToBP_GameInstance (Game|GetGameInstance)))
      (Default|ActivateSpecialTorchChap1Part1 (Variables|/Game/BP/BP_GameInstance.BP_GameInstance_C|GetGame%20Controller _asbp_game_instance) self))))

(fn ConstructionScript
  (|CallParentFunction))