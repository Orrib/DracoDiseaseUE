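; Trigger volume for the dragon chase that notifies the game controller when the player enters or leaves it.
; On BeginPlay it caches the BP_GameInstance to reach its GameController.
; Overlap begin and end by actors tagged "player" each fire a separate hard-coded numeric event through TriggerEvent, leaving the response to the controller.
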(event EventBeginPlay
  (bind _asbp_game_instance (Utilities|Casting|CastToBP_GameInstance (Game|GetGameInstance)))
  (Variables|Default|SetGame%20Instance _asbp_game_instance))

(event Collision|EventActorBeginOverlap
  (params (OtherActor :type Actor%20Object%20Reference))
  (if (Actor|ActorHasTag OtherActor "player")
    (Default|TriggerEvent (Variables|/Game/BP/BP_GameInstance.BP_GameInstance_C|GetGame%20Controller (Variables|Default|GetGame%20Instance)) 10)))

(event EventTick
  (params (DeltaSeconds :type Float%20%28single-precision%29)))

(event Collision|EventActorEndOverlap
  (params (OtherActor :type Actor%20Object%20Reference))
  (if (Actor|ActorHasTag OtherActor "player")
    (Default|TriggerEvent (Variables|/Game/BP/BP_GameInstance.BP_GameInstance_C|GetGame%20Controller (Variables|Default|GetGame%20Instance)) 11)))

(fn ConstructionScript)