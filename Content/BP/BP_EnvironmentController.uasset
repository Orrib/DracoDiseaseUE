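; BP_EnvironmentController is an actor that tracks the current time of day and drives the level's lighting to match.
; On BeginPlay it registers itself with BP_GameInstance, waits a tick to fetch the LightingController from it, then applies the initial TimeOfDay instantly.
; SetTimeOfDay forwards the scenario and transition time to that controller and stores the new value.
; Debug bracket keys step through the four times of day with wraparound.
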(event Custom|Set%20Time%20of%20Day%20Instantly
  (params (New%20Time%20of%20Day :type Enum_TimeOfDay%20Enum :default "NewEnumerator0"))
  (CallFunction|SetTimeOfDay New%20Time%20of%20Day 0.0))

(event Custom|Set%20Time%20of%20Day
  (params (New%20Time%20of%20Day :type Enum_TimeOfDay%20Enum :default "NewEnumerator0") (Transition%20Time :type Float%20%28double-precision%29))
  (Default|SetLightingScenario (Variables|Default|GetLighting%20Controller) New%20Time%20of%20Day Transition%20Time)
  (Variables|Default|SetTime%20of%20Day New%20Time%20of%20Day))

(event EventBeginPlay
  (bind _asbp_game_instance (Utilities|Casting|CastToBP_GameInstance (Game|GetGameInstance)))
  (bind _output_get (Variables|Default|SetGame%20Instance _asbp_game_instance))
  (Variables|/Game/BP/BP_GameInstance.BP_GameInstance_C|SetEnvironment%20Controller _output_get self)
  (Utilities|FlowControl|DelayUntilNextTick)
  (Variables|Default|SetLighting%20Controller (Variables|/Game/BP/BP_GameInstance.BP_GameInstance_C|GetLighting%20Controller (Variables|Default|GetGame%20Instance)))
  (CallFunction|SetTimeOfDayInstantly (Variables|Default|GetTime%20of%20Day))
  (Input|EnableInput (Game|GetPlayerController 0)))

(event Input|KeyboardEvents|DebugKeyLeftBracket
  (params (Key :type Key%20Structure :default "None") (ActionValue :type Input%20Action%20Value%20Structure))
  (bind _time_of_day (Variables|Default|GetTime%20of%20Day))
  (bind _returnvalue (Math|Conversions|ToInteger(Byte) _time_of_day))
  (bind _returnvalue_2 (- _returnvalue 1))
  ;[1 0.01848 0] (debug) Lighting Test
  (:Pressed
    (CallFunction|SetTimeOfDay (Utilities|Enum|ByteToEnumEnum_TimeOfDay (Math|Conversions|ToByte(Integer) (select (< _returnvalue_2 0) 3 _returnvalue_2))) 1.0)))

(event Input|KeyboardEvents|DebugKeyRightBracket
  (params (Key :type Key%20Structure :default "None") (ActionValue :type Input%20Action%20Value%20Structure))
  (bind _time_of_day (Variables|Default|GetTime%20of%20Day))
  (bind _returnvalue (Math|Conversions|ToInteger(Byte) _time_of_day))
  (bind _returnvalue_2 (+ _returnvalue 1))
  ;[1 0.01848 0] (debug) Lighting Test
  (:Pressed
    (CallFunction|SetTimeOfDay (Utilities|Enum|ByteToEnumEnum_TimeOfDay (Math|Conversions|ToByte(Integer) (select (> _returnvalue_2 3) 0 _returnvalue_2))) 1.0)))

(fn ConstructionScript)