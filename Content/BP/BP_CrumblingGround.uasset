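; A platform that crumbles after the player touches it, then respawns as a fresh copy of itself.
; The first hit flashes the crack meshes emissive and plays audio, then after a delay swaps the intact collision and visuals for a simulated Chaos geometry collection, crumbled and pushed downward.
; Later it spawns a replacement that scales in and keeps any attach parent, while the debris shrinks away and the old actor is destroyed.
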(event Custom|Collision%20Flash
  (Utilities|FlowControl|Sequence
    (:then_0
      (Utilities|FlowControl|RetriggerableDelay 0.15)
      (for _array_element (Components|GetChildrenComponents (Variables|Default|GetCracks) false)
        (bind _asstatic_mesh_component (Utilities|Casting|CastToStaticMeshComponent _array_element))
        (Rendering|Material|SetMaterial _asstatic_mesh_component 0 (Variables|Default|GetOrig%20Material))))
    (:then_1
      (for _array_element_2 (Components|GetChildrenComponents (Variables|Default|GetCracks) false)
        (bind _asstatic_mesh_component_2 (Utilities|Casting|CastToStaticMeshComponent _array_element_2))
        (Rendering|Material|SetMaterial _asstatic_mesh_component_2 0 "/Game/Materials/M_Emissive_PlatformGlow.M_Emissive_PlatformGlow")))))

(event Custom|Enable/Disable%20Destructible
  (params (Enable? :type Boolean))
  (bind _bp_box_geometrycollection (Variables|Default|GetBP_Box_GeometryCollection))
  (Collision|SetCollisionEnabled (Variables|Default|GetCollision) (select Enable? "NoCollision" "QueryAndPhysics"))
  (Rendering|SetVisibility (Variables|Default|GetCracks) (not Enable?) true)
  (Variables|/Script/GeometryCollectionEngine.GeometryCollectionComponent|SetObjectType _bp_box_geometrycollection (select Enable? "Chaos_Object_Dynamic" "Chaos_Object_Kinematic"))
  (Physics|SetSimulatePhysics _bp_box_geometrycollection Enable?)
  (Collision|SetCollisionEnabled _bp_box_geometrycollection (select Enable? "QueryAndPhysics" "NoCollision"))
  (Rendering|SetVisibility _bp_box_geometrycollection Enable? false))

(event EventBeginPlay
  (Variables|Default|SetOrig%20Material (Rendering|Material|GetMaterial (Variables|Default|GetBP_Box_GeometryCollection) 0))
  (CallFunction|Enable/DisableDestructible false)
  (bind _newtrack_0 (Timeline|Appear PlayFromStart)
    (:Update
      (Transformation|SetRelativeScale3D (Variables|Default|GetParent) (Math|Conversions|ToVector(Float) _newtrack_0)))))

(event Collision|EventHit
  (params (MyComp :type Primitive%20Component%20Object%20Reference) (Other :type Actor%20Object%20Reference) (OtherComp :type Primitive%20Component%20Object%20Reference) (bSelfMoved :type Boolean) (HitLocation :type Vector :default "0, 0, 0") (HitNormal :type Vector :default "0, 0, 0") (NormalImpulse :type Vector :default "0, 0, 0") (Hit :type Hit%20Result%20Structure%20%28by%20ref%29))
  (bind _returnvalue (Actor|GetAttachParentActor))
  (bind _bp_box_geometrycollection (Variables|Default|GetBP_Box_GeometryCollection))
  (bind _bp_box_geometrycollection_2 (Variables|Default|GetBP_Box_GeometryCollection))
  (if (Actor|ActorHasTag Other "player")
    (Utilities|FlowControl|DoOnce false
      (:Completed
        (CallFunction|CollisionFlash)
        (Audio|PlaySound2D "/Game/Sound/SoundFX/Footstep_Stone_1.Footstep_Stone_1" 1.0 0.2 (Math|Random|RandomFloatinRange 0.0 5e+01) 0 0)
        (Audio|Components|Audio|FadeOut (Variables|Default|GetMain%20Audio) 2.0 0.0 "SCurve" :!class /Script/Engine.AudioComponent)
        (Utilities|FlowControl|Delay (Variables|Default|GetCrumble%20Delay%20Time))
        (Utilities|FlowControl|Delay (Math|Random|RandomFloatinRange 0.4 0.8))
        (CallFunction|Enable/DisableDestructible true)
        (Audio|Components|Audio|Play (Variables|Default|GetBreak%20Audio) 0.0)
        (Class|GeometryCollectionComponent|CrumbleCluster _bp_box_geometrycollection)
        (Utilities|FlowControl|DelayUntilNextTick)
        (Physics|AddImpulseatLocation _bp_box_geometrycollection "0.000000,0.000000,-300000.000000" (Transformation|GetWorldLocation (Variables|Default|GetImpulse%20Point)) "None")
        (Physics|AddImpulseatLocation _bp_box_geometrycollection "0.000000,0.000000,-300000.000000" (Transformation|GetWorldLocation (Variables|Default|GetImpulse%20Point1)) "None")
        (Utilities|FlowControl|Delay 4.0)
        (Utilities|FlowControl|Sequence
          (:then_0
            (bind _returnvalue_2 (Game|SpawnActorfromClass "BP_CrumblingGround_C" (Transformation|GetActorTransform) "Undefined" "MultiplyWithRoot" 0 0))
            (Utilities|IsValid _returnvalue
              (:Is%20Valid
                (Transformation|AttachActorToActor _returnvalue_2 _returnvalue "None" "KeepWorld" "KeepWorld" "KeepWorld" false))))
          (:then_1
            (Utilities|FlowControl|Delay 1.0)
            (Variables|Default|SetOrig%20SCale (Variables|/Script/Engine.SceneComponent|GetRelativeScale3D _bp_box_geometrycollection_2))
            (bind _newtrack_0 (Timeline|Fade%20Destructable PlayFromStart)
              (:Update
                (Transformation|SetRelativeScale3D _bp_box_geometrycollection_2 (Math|Vector|Lerp(Vector) (Variables|Default|GetOrig%20SCale) "0, 0, 0" _newtrack_0)))
              (:Finished
                (Actor|DestroyActor)))))))))

(fn ConstructionScript)