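; Coin pickup Blueprint that grants the player coins when collected.
; On pickup it adds its coin reward to the player controller, plays a 2D coin sound, then runs the parent pickup logic.
; A Spin event drives a timeline that lerps the Paper2D sprite's yaw through a half turn to animate the coin.
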(event EventBeginPlay
  (|CallParentFunction) ; This node is disabled and will not be called.\nDrag off pins to build functionality.
)

(event Collision|EventActorBeginOverlap
  (params (OtherActor :type Actor%20Object%20Reference))
  (|CallParentFunction OtherActor) ; This node is disabled and will not be called.\nDrag off pins to build functionality.
)

(event EventTick
  (params (DeltaSeconds :type Float%20%28single-precision%29))
  (|CallParentFunction DeltaSeconds) ; This node is disabled and will not be called.\nDrag off pins to build functionality.
)

(event EventOnPickup
  (params (Player%20Controller :type BP%20Top%20Down%20Controller%20Object%20Reference))
  (Utilities|FlowControl|Sequence
    (:then_0
      (Default|AddCoins Player%20Controller (Variables|Default|GetCoin%20reward))
      (Audio|PlaySound2D "/Game/Sound/SoundFX/Cue_Pickup_Coin.Cue_Pickup_Coin" 1.0 1.0 0.0 0 0))
    (:then_1
      (|CallParentFunction Player%20Controller))))

(event EventSpin
  (bind _newtrack_0 (Timeline|Timeline_0 PlayFromStart)
    (:Update
      (Transformation|SetRelativeRotation (Variables|Default|GetPaperSprite) (Math|Rotator|MakeRotator 0.0 0.0 (Math|Float|Lerp 9e+01 2.7e+02 _newtrack_0)) false false))))

(fn ConstructionScript
  (|CallParentFunction))