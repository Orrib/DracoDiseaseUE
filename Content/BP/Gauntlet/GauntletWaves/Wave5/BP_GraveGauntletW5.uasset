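; Tombstone spawner for wave 5 of the Gauntlet mode, spawning temporary wizard-enemy zombies at its own transform.
; StartSpawning uses a DoOnce to set a single, non-looping timer that calls Spawn Zombie 5 after SpawnInterval.
; Below MaxZombies, the spawned zombie gets a primary objective and the Gauntlet manager's AppendZombie is called; otherwise it just spawns.
; Wave registration, SpawnCount updates and the SpawnerFinished hand-off are disconnected and never run.
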(event Custom|Start%20Spawning
  ;[1 1 1] Calling for SpawnZombie Function
  (Utilities|FlowControl|DoOnce false
    (:Completed
      (Utilities|Time|SetTimerbyFunctionName 0 "Spawn Zombie 5" (Variables|Default|GetSpawnInterval)))))

(fn ConstructionScript)

(fn SpawnZombie5
  ;[1 1 1] If spawn count is greater then or equal to max zombies then..
  (if (>= (Variables|Default|GetSpawnCount) (Variables|Default|GetMaxZombies))
    ;[1 1 1] after the final zombie of the wave has been spawned move on to the next spawner
    (bind _returnvalue (Game|SpawnActorfromClass "/Game/TopDown/Blueprints/BP_NPC_WizardEnemy_TempZombie.BP_NPC_WizardEnemy_TempZombie_C" (Transformation|GetActorTransform) "Undefined" "MultiplyWithRoot" 0 false "NewEnumerator0" 0 4.5e+02 false 0))
    (else
      ;[1 1 1] Spawn Zombie at location of tombstone
      (bind _returnvalue_2 (Game|SpawnActorfromClass "/Game/TopDown/Blueprints/BP_NPC_WizardEnemy_TempZombie.BP_NPC_WizardEnemy_TempZombie_C" (Transformation|GetActorTransform) "Undefined" "MultiplyWithRoot" 0 false "NewEnumerator7" 0 4.5e+02 false 0))
      (Default|AppendZombie (Variables|Default|GetGautletManagerRef)))))