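; BP_Volume_InputLimitter is a trigger volume that switches the player's input type on entering and leaving it.
; Overlaps by actors tagged "player" apply configurable enter and exit types to the TopDownController, reached through the GameController on the cached BP_GameInstance.
; For two of the enter types, it also unselects everything through the GameController and calls EnterExitStrategyMode with false.
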(event EventBeginPlay
  (bind _asbp_game_instance (Utilities|Casting|CastToBP_GameInstance (Game|GetGameInstance)))
  (Variables|Default|SetBP%20Game%20Instance _asbp_game_instance))

(event Collision|EventActorBeginOverlap
  (params (OtherActor :type Actor%20Object%20Reference))
  (bind _bp_game_instance (Variables|Default|GetBP%20Game%20Instance))
  (bind _input_type_enter (Variables|Default|GetInput%20Type%20Enter))
  (bind _game_controller (Variables|/Game/BP/BP_GameInstance.BP_GameInstance_C|GetGame%20Controller _bp_game_instance))
  (bind _top_down_character (Variables|/Game/BP/BP_GameController.BP_GameController_C|GetTop%20Down%20Character _game_controller))
  (bind _top_down_controller (Variables|/Game/TopDown/Blueprints/BP_TopDownCharacter.BP_TopDownCharacter_C|GetTop%20Down%20Controller _top_down_character))
  (if (Actor|ActorHasTag OtherActor "player")
    (Default|ChangeInputType _top_down_controller _input_type_enter)
    (if (or (Utilities|Enum|Equal(Enum) _input_type_enter "NewEnumerator1") (Utilities|Enum|Equal(Enum) _input_type_enter "NewEnumerator3"))
      (Default|UnselectAll _game_controller)
      (Default|Enter/ExitStrategyMode _top_down_controller false))))

(event EventTick
  (params (DeltaSeconds :type Float%20%28single-precision%29)))

(event Collision|EventActorEndOverlap
  (params (OtherActor :type Actor%20Object%20Reference))
  (if (Actor|ActorHasTag OtherActor "player")
    (Default|ChangeInputType (Variables|/Game/TopDown/Blueprints/BP_TopDownCharacter.BP_TopDownCharacter_C|GetTop%20Down%20Controller (Variables|/Game/BP/BP_GameController.BP_GameController_C|GetTop%20Down%20Character (Variables|/Game/BP/BP_GameInstance.BP_GameInstance_C|GetGame%20Controller (Variables|Default|GetBP%20Game%20Instance)))) (Variables|Default|GetInput%20Type%20Exit))))

(fn ConstructionScript)