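; Lighting controller that blends between day, sunset, night and sunrise scenarios and registers itself with BP_GameInstance.
; A timeline, rate-scaled to the transition time or skipped for instant changes, lerps sun, skylight and fog values from previous to new scenario onto a visible master scenario.
; Post process volumes instead crossfade directly through blend weights.
; In the construction script, dev mode hides the master and shows the chosen scenario's actors for direct editing.
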(event Custom|Set%20Lighting%20Scenario
  (params (New%20Time%20of%20Day :type Enum_TimeOfDay%20Enum :default "NewEnumerator0") (Transition%20Time :type Float%20%28double-precision%29))
  (Variables|Default|SetPrev%20Time%20Of%20Day (Variables|Default|GetTime%20Of%20Day))
  (Variables|Default|SetTime%20Of%20Day New%20Time%20of%20Day)
  (if (Variables|Default|GetEnable%20Lighting%20Scenarios)
    (if (> Transition%20Time 0.0)
      (Components|Timeline|SetPlayRate (Variables|Default|GetLerp) (Math|Float|Power Transition%20Time -1.0))
      (bind _newtrack_0 (Timeline|Lerp PlayFromStart)
        (:Update
          (CallFunction|CopyScenario _newtrack_0)))
      (else
        (CallFunction|CopyScenario 1.0)))))

(event Custom|Hide%20Scenarios
  (CallFunction|Show/HideScenarioComponents (Variables|Default|GetDay%20%20Scenario) false)
  (CallFunction|Show/HideScenarioComponents (Variables|Default|GetSunset%20Scenario) false)
  (CallFunction|Show/HideScenarioComponents (Variables|Default|GetSunrise%20Scenario) false)
  (CallFunction|Show/HideScenarioComponents (Variables|Default|GetNight%20Scenario) false))

(event Custom|Copy%20Skylight
  (params (Source :type Sky%20Light%20Object%20Reference%20%28by%20ref%29) (Target :type Sky%20Light%20Object%20Reference%20%28by%20ref%29) (Lerp%20Percentage%20%280-1%29 :type Float%20%28double-precision%29))
  (bind _lightcomponent (Variables|/Script/Engine.SkyLight|GetLightComponent Target))
  (bind _lightcomponent_2 (Variables|/Script/Engine.SkyLight|GetLightComponent Source))
  (bind _master_scenario (Variables|Default|GetMaster%20Scenario))
  (bind _skylight (Utilities|Struct|BreakStruct_EnvironmentScenario _master_scenario))
  (bind _lightcomponent_3 (Variables|/Script/Engine.SkyLight|GetLightComponent _skylight))
  ;[0 0 0] Copy Scenario
  ;;[1 1 1] Skylight
  (Rendering|Components|Light|SetIntensity _lightcomponent_3 (Math|Float|Lerp (Variables|/Script/Engine.LightComponentBase|GetIntensity _lightcomponent_2) (Variables|/Script/Engine.LightComponentBase|GetIntensity _lightcomponent) Lerp%20Percentage%20%280-1%29))
  (Rendering|Components|Light|SetLightColor _lightcomponent_3 (Math|Color|Lerp(LinearColor) (Rendering|Components|Light|GetLightColor _lightcomponent_2) (Rendering|Components|Light|GetLightColor _lightcomponent) Lerp%20Percentage%20%280-1%29)))

(event Custom|Enable%20Post%20Processes
  (params (Original :type Post%20Process%20Volume%20Object%20Reference%20%28by%20ref%29) (New :type Post%20Process%20Volume%20Object%20Reference%20%28by%20ref%29))
  ;[0 0 0] Copy Scenario
  ;;[1 1 1] Post Process
  (Rendering|SetVisibility (Variables|/Script/Engine.Actor|GetRootComponent Original) true true))

(event Custom|Set%20Lighting%20Scenario%20Instantly
  (params (New%20Time%20of%20Day :type Enum_TimeOfDay%20Enum :default "NewEnumerator0"))
  (CallFunction|SetLightingScenario New%20Time%20of%20Day 0.0))

(event Custom|Copy%20Fog
  (params (Source :type Exponential%20Height%20Fog%20Object%20Reference%20%28by%20ref%29) (Target :type Exponential%20Height%20Fog%20Object%20Reference%20%28by%20ref%29) (Lerp%20Percentage%20%280-1%29 :type Float%20%28double-precision%29))
  (bind _master_scenario (Variables|Default|GetMaster%20Scenario))
  (bind _component (Variables|/Script/Engine.ExponentialHeightFog|GetComponent Target))
  (bind _component_2 (Variables|/Script/Engine.ExponentialHeightFog|GetComponent Source))
  (bind _fog (Utilities|Struct|BreakStruct_EnvironmentScenario _master_scenario))
  (bind _component_3 (Variables|/Script/Engine.ExponentialHeightFog|GetComponent _fog))
  ;[0 0 0] Copy Scenario
  ;;[1 1 1] Fog
  (Class|ExponentialHeightFogComponent|SetFogDensity _component_3 (Math|Float|Lerp (Variables|/Script/Engine.ExponentialHeightFogComponent|GetFogDensity _component_2) (Variables|/Script/Engine.ExponentialHeightFogComponent|GetFogDensity _component) Lerp%20Percentage%20%280-1%29))
  (Class|ExponentialHeightFogComponent|SetSecondFogDensity _component_3 (Math|Float|Lerp (.fogdensity (Variables|/Script/Engine.ExponentialHeightFogComponent|GetSecondFogData _component_2)) (.fogdensity (Variables|/Script/Engine.ExponentialHeightFogComponent|GetSecondFogData _component)) Lerp%20Percentage%20%280-1%29))
  (Class|ExponentialHeightFogComponent|SetStartDistance _component_3 (Math|Float|Lerp (Variables|/Script/Engine.ExponentialHeightFogComponent|GetStartDistance _component_2) (Variables|/Script/Engine.ExponentialHeightFogComponent|GetStartDistance _component) Lerp%20Percentage%20%280-1%29)))

(event Custom|Show/Hide%20Scenario%20Components
  (params (Scenario :type Struct%20Environment%20Scenario%20Structure%20%28by%20ref%29) (bNewVisibility :type Boolean))
  (Rendering|SetVisibility (Variables|/Script/Engine.Light|GetLightComponent (.sun Scenario)) bNewVisibility true))

(event Custom|Crossfade%20Post%20Process
  (params (Original :type Post%20Process%20Volume%20Object%20Reference%20%28by%20ref%29) (New :type Post%20Process%20Volume%20Object%20Reference%20%28by%20ref%29) (Crossfade%20Percentage%20%280-1%29 :type Float%20%28double-precision%29))
  ;[0 0 0] Copy Scenario
  ;;[1 1 1] Post Process
  (Variables|/Script/Engine.PostProcessVolume|SetBlendWeight Original (- 1.0 Crossfade%20Percentage%20%280-1%29))
  (Variables|/Script/Engine.PostProcessVolume|SetBlendWeight New Crossfade%20Percentage%20%280-1%29))

(event Custom|Copy%20Scenario
  (params (Lerp%20Percentage%20%280-1%29 :type Float%20%28double-precision%29))
  (bind _time_of_day (Variables|Default|GetTime%20Of%20Day))
  (bind _prev_time_of_day (Variables|Default|GetPrev%20Time%20Of%20Day))
  (bind _returnvalue (Utilities|GetScenariofromTimeOfDay _time_of_day))
  (bind _returnvalue_2 (Utilities|GetScenariofromTimeOfDay _prev_time_of_day))
  (bind (_sun _skylight _fog _postprocessvolume) (Utilities|Struct|BreakStruct_EnvironmentScenario _returnvalue))
  (bind (_sun_2 _skylight_2 _fog_2 _postprocessvolume_2) (Utilities|Struct|BreakStruct_EnvironmentScenario _returnvalue_2))
  ;[0 0 0] Copy Scenario
  (CallFunction|CopySun _sun_2 _sun Lerp%20Percentage%20%280-1%29)
  (CallFunction|CopySkylight _skylight_2 _skylight Lerp%20Percentage%20%280-1%29)
  (CallFunction|EnablePostProcesses _postprocessvolume_2 _postprocessvolume)
  (CallFunction|CrossfadePostProcess _postprocessvolume_2 _postprocessvolume Lerp%20Percentage%20%280-1%29)
  (CallFunction|CopyFog _fog_2 _fog Lerp%20Percentage%20%280-1%29))

(event Custom|Set%20Up%20%28Dev%20Mode%29
  (CallFunction|HideScenarios)
  (CallFunction|Show/HideScenarioComponents (Variables|Default|GetMaster%20Scenario) false)
  (CallFunction|Show/HideScenarioComponents (Utilities|GetScenariofromTimeOfDay (Variables|Default|GetTime%20Of%20Day)) true))

(event Custom|Copy%20Sun
  (params (Source :type Directional%20Light%20Object%20Reference%20%28by%20ref%29) (Target :type Directional%20Light%20Object%20Reference%20%28by%20ref%29) (Lerp%20Percentage%20%280-1%29 :type Float%20%28double-precision%29))
  (bind _lightcomponent (Variables|/Script/Engine.Light|GetLightComponent Source))
  (bind _lightcomponent_2 (Variables|/Script/Engine.Light|GetLightComponent Target))
  (bind _master_scenario (Variables|Default|GetMaster%20Scenario))
  (bind _sun (Utilities|Struct|BreakStruct_EnvironmentScenario _master_scenario))
  (bind _lightcomponent_3 (Variables|/Script/Engine.Light|GetLightComponent _sun))
  ;[0 0 0] Copy Scenario
  ;;[1 1 1] Sun
  (Rendering|Components|Light|SetIntensity _lightcomponent_3 (Math|Float|Lerp (Variables|/Script/Engine.LightComponentBase|GetIntensity _lightcomponent) (Variables|/Script/Engine.LightComponentBase|GetIntensity _lightcomponent_2) Lerp%20Percentage%20%280-1%29))
  (Transformation|SetActorRotation _sun (Math|Rotator|Lerp(Rotator) (Transformation|GetActorRotation Source) (Transformation|GetActorRotation Target) Lerp%20Percentage%20%280-1%29 true))
  (Class|LightComponent|SetTemperature _lightcomponent_3 (Math|Float|Lerp (Variables|/Script/Engine.LightComponent|GetTemperature _lightcomponent) (Variables|/Script/Engine.LightComponent|GetTemperature _lightcomponent_2) Lerp%20Percentage%20%280-1%29))
  (Rendering|Components|Light|SetLightColor _lightcomponent_3 (Math|Color|Lerp(LinearColor) (Rendering|Components|Light|GetLightColor _lightcomponent) (Rendering|Components|Light|GetLightColor _lightcomponent_2) Lerp%20Percentage%20%280-1%29) true))

(event Custom|Set%20Up
  (CallFunction|HideScenarios)
  (CallFunction|Show/HideScenarioComponents (Variables|Default|GetMaster%20Scenario) true))

(event EventBeginPlay
  (bind _asbp_game_instance (Utilities|Casting|CastToBP_GameInstance (Game|GetGameInstance)))
  (Variables|/Game/BP/BP_GameInstance.BP_GameInstance_C|SetLighting%20Controller _asbp_game_instance self)
  (if (Variables|Default|GetEnable%20Lighting%20Scenarios)
    (CallFunction|SetUp)))

(fn ConstructionScript
  (if (Variables|Default|GetEnable%20Lighting%20Scenarios)
    (if (Variables|Default|GetDev%20Mode%20-%20Allows%20you%20to%20work%20Directly%20on%20the%20actors%20in%20the%20chosen%20Lighting%20Scenario)
      (CallFunction|SetUp(DevMode))
      (CallFunction|SetLightingScenarioInstantly (Variables|Default|GetTime%20Of%20Day))
      (else
        (CallFunction|SetUp)))))